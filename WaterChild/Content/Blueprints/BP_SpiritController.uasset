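; Player controller for the Spirit character, turning input into movement, look, jump, climb and revive calls on the possessed BP_Spirit.
; Each overridden input event calls its parent, then forwards to the cached Spirit only while its CanTakeInput flag is set.
; Pause toggles that flag along with game pause, the UI_Pause widget and input mode, but requires CanPauseGame, which BeginPlay sets to false.
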(event EventBeginPlay
  (Variables|Default|SetCanPauseGame false)
  (bind _asbp_spirit (Utilities|Casting|CastToBP_Spirit (Pawn|GetControlledPawn)))
  (Variables|Default|SetSpirit _asbp_spirit)
  (Class|SpiritController|SetIsUsingGamepad false))

(event EventGamepadRightAxis
  (params (Value :type Float%20%28single-precision%29))
  (bind _spirit (Variables|Default|GetSpirit))
  (|CallParentFunction Value)
  (bind _returnvalue (Class|Spirit|GetCanTakeInput _spirit))
  (if _returnvalue
    (Class|Spirit|MoveRight _spirit Value)))

(event EventMouseLookUpAxis
  (params (Value :type Float%20%28single-precision%29))
  (bind _spirit (Variables|Default|GetSpirit))
  (|CallParentFunction Value)
  (bind _returnvalue (Class|Spirit|GetCanTakeInput _spirit))
  (if _returnvalue
    (Class|Spirit|LookUpat _spirit Value)))

(event EventMouseTurnAxis
  (params (Value :type Float%20%28single-precision%29))
  (bind _spirit (Variables|Default|GetSpirit))
  (|CallParentFunction Value)
  (bind _returnvalue (Class|Spirit|GetCanTakeInput _spirit))
  (if _returnvalue
    (Class|Spirit|Turnat _spirit Value)))

(event EventGamepadLookUpAxis
  (params (Value :type Float%20%28single-precision%29))
  (bind _spirit (Variables|Default|GetSpirit))
  (|CallParentFunction Value)
  (bind _returnvalue (Class|Spirit|GetCanTakeInput _spirit))
  (if _returnvalue
    (Class|Spirit|LookUpatRate _spirit Value)))

(event EventGamepadTurnAxis
  (params (Value :type Float%20%28single-precision%29))
  (bind _spirit (Variables|Default|GetSpirit))
  (|CallParentFunction Value)
  (bind _returnvalue (Class|Spirit|GetCanTakeInput _spirit))
  (if _returnvalue
    (Class|Spirit|TurnatRate _spirit Value)))

(event EventPauseAction
  (bind _self self)
  (bind _spirit (Variables|Default|GetSpirit))
  (|CallParentFunction)
  (if (Variables|Default|GetCanPauseGame)
    (bind _returnvalue (Class|Spirit|GetCanTakeInput _spirit))
    (Class|Spirit|SetCanTakeInput _spirit (not _returnvalue))
    (if _returnvalue
      (Game|SetGamePaused true)
      (bind _returnvalue_2 (UserInterface|CreateWidget "/Game/Blueprints/UI/UI_Pause.UI_Pause_C" _self))
      (UserInterface|Viewport|AddtoViewport _returnvalue_2 0)
      (Input|SetInputModeGameandUI _self _returnvalue_2 "DoNotLock" true)
      (else
        (Game|SetGamePaused false)
        (Widget|RemovefromParent _returnvalue_2)
        (Input|SetInputModeGameOnly _self)
        (Variables|Default|SetbShowMouseCursor false)))))

(event EventReviveAction
  (bind _spirit (Variables|Default|GetSpirit))
  (|CallParentFunction)
  (bind _returnvalue (Class|Spirit|GetCanTakeInput _spirit))
  (if _returnvalue
    (Class|Spirit|Revive _spirit)))

(event EventStopReviveAction
  (bind _spirit (Variables|Default|GetSpirit))
  (|CallParentFunction)
  (bind _returnvalue (Class|Spirit|GetCanTakeInput _spirit))
  (if _returnvalue
    (Class|Spirit|StopRevive _spirit)))

(event EventClimbAction
  (bind _spirit (Variables|Default|GetSpirit))
  (|CallParentFunction)
  (bind _returnvalue (Class|Spirit|GetCanTakeInput _spirit))
  (if _returnvalue
    (Class|Spirit|Climb _spirit)))

(event EventStopClimbAction
  (bind _spirit (Variables|Default|GetSpirit))
  (|CallParentFunction)
  (bind _returnvalue (Class|Spirit|GetCanTakeInput _spirit))
  (if _returnvalue
    (Class|Spirit|StopClimb _spirit)))

(event EventJumpAction
  (bind _spirit (Variables|Default|GetSpirit))
  (|CallParentFunction)
  (bind _returnvalue (Class|Spirit|GetCanTakeInput _spirit))
  (if _returnvalue
    (Class|Spirit|JumpAction _spirit)))

(event EventKeyboardForwardAxis
  (params (Value :type Float%20%28single-precision%29))
  (bind _spirit (Variables|Default|GetSpirit))
  (|CallParentFunction Value)
  (bind _returnvalue (Class|Spirit|GetCanTakeInput _spirit))
  (if _returnvalue
    (Class|Spirit|MoveForward _spirit Value)))

(event EventKeyboardRightAxis
  (params (Value :type Float%20%28single-precision%29))
  (bind _spirit (Variables|Default|GetSpirit))
  (|CallParentFunction Value)
  (bind _returnvalue (Class|Spirit|GetCanTakeInput _spirit))
  (if _returnvalue
    (Class|Spirit|MoveRight _spirit Value)))

(event EventGamepadForwardAxis
  (params (Value :type Float%20%28single-precision%29))
  (bind _spirit (Variables|Default|GetSpirit))
  (|CallParentFunction Value)
  (bind _returnvalue (Class|Spirit|GetCanTakeInput _spirit))
  (if _returnvalue
    (Class|Spirit|MoveForward _spirit Value)))

(fn ConstructionScript)