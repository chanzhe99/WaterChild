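; External follow camera for the player's BP_Spirit, set as the view target at BeginPlay.
; Each Tick, a tracker eases toward the spirit, scaled by distance and pitch, teleporting if too far and reparenting to a yaw tracker during turn input.
; Yaw auto-rotates behind sideways movement after a delay without look input.
; Revive reparents the camera to the spirit's spring arm, while sandstorms and timed LookAts steer rotation, adjust framing and lower sensitivity.
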(event Custom|UseCamera
  ;[1 1 1] Sets the camera to this, called by spirit as the middleman
  (Game|Player|SetViewTargetwithBlend (Game|GetPlayerController 0) (Components|GetOwner (Variables|Default|GetCamera)) 0.0 "VTBlend_Linear" 0.0 false))

(event Custom|RotateTick
  (params (DeltaTime :type Float%20%28single-precision%29))
  (bind _returnvalue (Game|GetPlayerController 0))
  (bind _returnvalue_2 (Pawn|GetControlRotation _returnvalue :!class /Script/Engine.Controller))
  (bind (_roll _pitch _yaw) (Math|Rotator|BreakRotator _returnvalue_2))
  ;[1 1 1] Keep Rotation tracker consistent with player controller and spirit position
  (Transformation|SetWorldLocation (Variables|Default|GetRotation%20Yaw%20Tracker) (Transformation|GetActorLocation (Variables|Default|GetSpirit)) false false)
  (Transformation|SetWorldRotation (Variables|Default|GetRotation%20Yaw%20Tracker) (Math|Rotator|MakeRotator 0.0 0.0 (.Yaw (Math|Rotator|BreakRotator (Pawn|GetControlRotation (Game|GetPlayerController 0) :!class /Script/Engine.Controller)))) false false)
  ;[1 1 1] Update Pitch Tracker
  (Transformation|SetWorldRotation (Variables|Default|GetLocation%20And%20Pitch%20Tracker) (Math|Rotator|MakeRotator 0.0 _pitch _yaw) false false))

(event Custom|Teleport%20Camera%20Tracker%20to%20Spirit
  ;[1 1 1] For crack movement
  (Transformation|SetWorldLocation (Variables|Default|GetLocation%20And%20Pitch%20Tracker) (Transformation|GetActorLocation (Variables|Default|GetSpirit)) false false))

(event Custom|RotateToMovement
  (bind _returnvalue (Game|GetPlayerController 0))
  (bind _spirit (Variables|Default|GetSpirit))
  (bind _returnvalue_2 (Pawn|GetControlRotation _returnvalue :!class /Script/Engine.Controller))
  (bind _spiritanimbp (Variables|/Game/Blueprints/BP_Spirit.BP_Spirit_C|GetSpiritAnimBP _spirit))
  (bind (_roll _pitch) (Math|Rotator|BreakRotator _returnvalue_2))
  (if (Utilities|Enum|NotEqual(Enum) (Variables|/Script/WaterChild.Spirit|GetSpiritState (Variables|Default|GetSpirit)) "Reviving")
    (if (not (and (Variables|/Game/Art/Spirit/Animations/AnimBP_Spirit.AnimBP_Spirit_C|GetIsInSandstorm _spiritanimbp) (Variables|/Game/Art/Spirit/Animations/AnimBP_Spirit.AnimBP_Spirit_C|GetIsSandstormOn _spiritanimbp)))
      (if (not (Variables|LookAt(calculation)|GetLookAtActive)) ; If look at is active, don't do anything
        (if (and (== (Input|AxisValues|GetGamepadTurnAxis) 0.0) (== (Input|AxisValues|GetMouseTurnAxis) 0.0)) ; If player is moving forward
          ;[1 1 1] Delay before active
          (bind _output_get (Variables|Default|SetDelayCounter (+ (Variables|Default|GetDelayCounter) (Variables|Default|GetDelta%20Time))))
          (if (>= _output_get (Variables|Default|GetKickInDelay)) ; If player is moving forward
            (if (not (and (== (Input|AxisValues|GetKeyboardRightAxis) 0.0) (== (Input|AxisValues|GetGamepadRightAxis) 0.0))) ; if player is moving sideways
              ;[1 1 1] Autorotate Calculation
              (Pawn|SetControlRotation _returnvalue (Math|Rotator|MakeRotator _roll _pitch (.Yaw (Math|Rotator|BreakRotator (Math|Interpolation|RInterpTo _returnvalue_2 (Transformation|GetActorRotation (Variables|Default|GetSpirit)) (Variables|Default|GetDelta%20Time) (Math|Interpolation|Ease "EaseIn" (Variables|AutorotateTweak|GetAutorotate%20Ease%20In%20speed) (Variables|AutorotateTweak|GetAutorotate%20Min%20Sensitivity) (Variables|AutorotateTweak|GetAutorotateMaxSensitivity) 2.0))))))))
          (else
            (Variables|Default|SetDelayCounter 0.0)))))))

(event Custom|ReviveCam
  (bind _spirit (Variables|Default|GetSpirit))
  (bind _spirit_2 (Variables|Default|GetSpirit))
  (bind _camera (Variables|Default|GetCamera))
  (bind _camera_2 (Variables|Default|GetCamera))
  (bind _delta_time (Variables|Default|GetDelta%20Time))
  (bind _revive_zoom_out_time (Variables|ReviveCamTweak|GetRevive%20Zoom%20Out%20time))
  (bind _spirit_3 (Variables|Default|GetSpirit))
  (bind _spirit_4 (Variables|Default|GetSpirit))
  (bind _camera_3 (Variables|Default|GetCamera))
  (bind _revive_zoom_in_time (Variables|ReviveCamTweak|GetRevive%20Zoom%20In%20time))
  (bind _delta_time_2 (Variables|Default|GetDelta%20Time))
  (bind _camera_4 (Variables|Default|GetCamera))
  (bind _result (Math|Interpolation|Ease "EaseIn" _revive_zoom_out_time 0.0 1.0 2.0))
  (bind _result_2 (Math|Interpolation|Ease "EaseIn" _revive_zoom_in_time 0.0 1.0 2.0))
  (bind _relativelocation (Variables|/Script/Engine.SceneComponent|GetRelativeLocation _camera))
  (bind _relativerotation (Variables|/Script/Engine.SceneComponent|GetRelativeRotation _camera))
  (bind _camera_5 (Variables|/Script/WaterChild.Spirit|GetCamera _spirit_3))
  (bind _camera_6 (Variables|/Script/WaterChild.Spirit|GetCamera _spirit_4))
  (bind _camera_7 (Variables|/Script/WaterChild.Spirit|GetCamera _spirit_2))
  (bind _relativelocation_2 (Variables|/Script/Engine.SceneComponent|GetRelativeLocation _camera_3))
  (bind _relativerotation_2 (Variables|/Script/Engine.SceneComponent|GetRelativeRotation _camera_3))
  (bind _relativelocation_3 (Variables|/Script/Engine.SceneComponent|GetRelativeLocation _camera_7))
  (bind _relativerotation_3 (Variables|/Script/Engine.SceneComponent|GetRelativeRotation _camera_7))
  (if (not (Variables|LookAt(calculation)|GetLookAtActive))
    (if (and (not (<= (Math|Vector|Distance(Vector) (Transformation|GetWorldLocation (Variables|/Script/WaterChild.Spirit|GetCamera _spirit)) (Transformation|GetActorLocation (Pawn|GetControlledPawn (Game|GetPlayerController 0)))) 5e+01)) (Utilities|Enum|Equal(Enum) (Variables|/Script/WaterChild.Spirit|GetSpiritState _spirit) "Reviving"))
      (if (Variables|Default|GetcameraDisconnectedFromArm)
        _
        (else
          (Transformation|AttachComponentToComponent (Variables|Default|GetCamera) (Variables|/Script/WaterChild.Spirit|GetSpringArm (Variables|Default|GetSpirit)) "None" "KeepWorld" "KeepWorld" "KeepWorld" false)
          (Variables|Default|SetcameraDisconnectedFromArm true)))
      (if (or (not (Math|Vector|Equal(Vector) _relativelocation_2 (Variables|/Script/Engine.SceneComponent|GetRelativeLocation _camera_6) 0.001)) (not (Math|Rotator|Equal(Rotator) _relativerotation_2 (Variables|/Script/Engine.SceneComponent|GetRelativeRotation _camera_6) 0.001)))
        ;[1 1 1] sync Local position
        (Transformation|SetRelativeLocationAndRotation _camera_4 (Math|Interpolation|VInterpTo (Variables|/Script/Engine.SceneComponent|GetRelativeLocation _camera_4) (Variables|/Script/Engine.SceneComponent|GetRelativeLocation _camera_5) _delta_time_2 _result_2) (Math|Interpolation|RInterpTo (Variables|/Script/Engine.SceneComponent|GetRelativeRotation _camera_4) (Variables|/Script/Engine.SceneComponent|GetRelativeRotation _camera_5) _delta_time_2 _result_2) false false)
        (else
          ;[1 1 1] Final Push as interp does not hit the exact values
          (if (not (or (Class|KismetMathLibrary|EqualExactlyVectorVector _relativelocation_2 _relativelocation_3) (Math|Rotator|Equal(Rotator) _relativerotation_2 _relativerotation_3 0.0)))
            (Transformation|SetRelativeLocationAndRotation (Variables|Default|GetCamera) _relativelocation_3 _relativerotation_3 false false))))
      (else
        (if (Variables|Default|GetcameraDisconnectedFromArm)
          (Transformation|AttachComponentToComponent (Variables|Default|GetCamera) (Variables|Default|GetSpringArm) "None" "KeepWorld" "KeepWorld" "KeepWorld" false)
          (Variables|Default|SetcameraDisconnectedFromArm false))
        ;[1 1 1] Final push as interp dosen't reach the exact value
        (if (or (not (Math|Vector|Equal(Vector) _relativelocation "0, 0, 0" 0.001)) (not (Math|Rotator|Equal(Rotator) _relativerotation "0, 0, 0" 0.001)))
          ;[1 1 1] Reset Local position
          (Transformation|SetRelativeLocationAndRotation _camera_2 (Math|Interpolation|VInterpTo (Variables|/Script/Engine.SceneComponent|GetRelativeLocation _camera_2) "0, 0, 0" _delta_time _result) (Math|Interpolation|RInterpTo (Variables|/Script/Engine.SceneComponent|GetRelativeRotation _camera_2) "0, 0, 0" _delta_time _result) false false)
          (elif (not (or (Class|KismetMathLibrary|EqualExactlyVectorVector _relativelocation "0, 0, 0") (Math|Rotator|Equal(Rotator) _relativerotation "0, 0, 0" 0.0)))
            (Transformation|SetRelativeLocationAndRotation _camera_2 "0, 0, 0" "0, 0, 0" false false)))))))

(event Custom|Sandstorm
  (bind _returnvalue (Game|GetPlayerController 0))
  (bind _returnvalue_2 (Game|GetPlayerController 0))
  (bind _returnvalue_3 (Game|GetPlayerController 0))
  (bind _spirit (Variables|Default|GetSpirit))
  (bind _springarm (Variables|Default|GetSpringArm))
  (bind _springarm_2 (Variables|Default|GetSpringArm))
  (bind _spiritanimbp (Variables|/Game/Blueprints/BP_Spirit.BP_Spirit_C|GetSpiritAnimBP _spirit))
  ;[1 1 1] Check if player is in sandstorm
  (if (and (Variables|/Game/Art/Spirit/Animations/AnimBP_Spirit.AnimBP_Spirit_C|GetIsInSandstorm _spiritanimbp) (Variables|/Game/Art/Spirit/Animations/AnimBP_Spirit.AnimBP_Spirit_C|GetIsSandstormOn _spiritanimbp))
    ;[1 1 1] Sync Springarm
    (Variables|/Script/Engine.SpringArmComponent|SetTargetArmLength (Variables|Default|GetSpringArm) (Variables|/Script/Engine.SpringArmComponent|GetTargetArmLength (Variables|/Script/WaterChild.Spirit|GetSpringArm (Variables|Default|GetSpirit))))
    ;[1 1 1] Camera offset stuff
    (Variables|/Script/Engine.SpringArmComponent|SetSocketOffset _springarm_2 (Math|Interpolation|VInterpTo (Variables|/Script/Engine.SpringArmComponent|GetSocketOffset _springarm_2) (Variables|Default|GetExCamSandstormCameraOffset) (Variables|Default|GetDelta%20Time) (Math|Interpolation|Ease "EaseIn" (Variables|LookAt(calculation)|GetLookAt%20Zoom%20in%20Acceleration) 0.0 1.0 2.0)))
    (Variables|Default|SetisSandstormOffsetDefault false)
    (Pawn|SetControlRotation _returnvalue_2 (Math|Interpolation|RInterpTo (Pawn|GetControlRotation _returnvalue_2 :!class /Script/Engine.Controller) (Math|Rotator|FindLookatRotation (Transformation|GetActorLocation (Pawn|GetControlledPawn _returnvalue_2)) (Variables|Default|GetSandstormLookatVector)) (Variables|Default|GetDelta%20Time) (Variables|SensitivityTweak|GetSandstorm%20Interp%20Speed)))
    (if (Variables|Default|GetSensitivity%20is%20default)
      ;[1 1 1] Lower Sensitivity to preset
      (Variables|/Script/Engine.PlayerController|SetInputPitchScale _returnvalue_3 (Variables|SensitivityTweak|GetPitch%20Locked%20Sensitivity))
      (Variables|/Script/Engine.PlayerController|SetInputYawScale _returnvalue_3 (Variables|SensitivityTweak|GetYaw%20Locked%20Sensitivity))
      (Variables|Default|SetSensitivity%20is%20default false))
    (else
      ;[1 1 1] Reset
      (if (Variables|Default|GetisSandstormOffsetDefault)
        _
        (else
          (bind _output_get (Variables|/Script/Engine.SpringArmComponent|SetSocketOffset _springarm (Math|Interpolation|VInterpTo (Variables|/Script/Engine.SpringArmComponent|GetSocketOffset _springarm) (Variables|LookAt(calculation)|GetDefaultLookatOffset) (Variables|Default|GetDelta%20Time) (Math|Interpolation|Ease "EaseIn" (Variables|LookAt(calculation)|GetLookAt%20Zoom%20in%20Acceleration) 0.0 1.0 2.0))))
          (if (Math|Vector|Equal(Vector) _output_get (Variables|LookAt(calculation)|GetDefaultLookatOffset) 0.01)
            (Variables|/Script/Engine.SpringArmComponent|SetSocketOffset (Variables|Default|GetSpringArm) (Variables|LookAt(calculation)|GetDefaultLookatOffset))
            (Variables|Default|SetisSandstormOffsetDefault true))))
      ;[1 1 1] Reset Sensitivity
      (if (not (Variables|Default|GetSensitivity%20is%20default))
        (Variables|/Script/Engine.PlayerController|SetInputPitchScale _returnvalue (Variables|Default|GetDefaultPitchScale))
        (Variables|/Script/Engine.PlayerController|SetInputYawScale _returnvalue (Variables|Default|GetDefaultYawScale))
        (Variables|Default|SetSensitivity%20is%20default true)))))

(event Custom|LookAt
  (bind _currentlookatbp (Variables|LookAt(calculation)|GetCurrentLookAtBP))
  ;[1 1 1] Grab Varibles and Cache and reset varibles
  (Utilities|IsValid _currentlookatbp
    (:Is%20Valid
      (if (not (Variables|/Game/Blueprints/GameTriggers/BP_LookAtArea.BP_LookAtArea_C|GetHasBeenTriggered _currentlookatbp))
        (Variables|LookAt(calculation)|SetLookAtActive true)
        (Variables|LookAt(calculation)|SetLookAtTimer 0.0)
        (Variables|LookAt(calculation)|SetLookAt%20Duration (Variables|/Game/Blueprints/GameTriggers/BP_LookAtArea.BP_LookAtArea_C|GetLookAtDuration _currentlookatbp))
        (Variables|LookAt(calculation)|SetLookAtVector (Transformation|GetWorldLocation (Variables|/Game/Blueprints/GameTriggers/BP_LookAtArea.BP_LookAtArea_C|GetLookAtTarget _currentlookatbp)))
        (Variables|LookAt(calculation)|SetLookAtSpringarm (Variables|/Game/Blueprints/GameTriggers/BP_LookAtArea.BP_LookAtArea_C|GetSpringArmLength%28zoom%29 _currentlookatbp))
        (Variables|LookAt(calculation)|SetLookAt%20Zoom%20in%20Acceleration (Variables|/Game/Blueprints/GameTriggers/BP_LookAtArea.BP_LookAtArea_C|GetZoomInAcceleration _currentlookatbp))
        (Variables|LookAt(calculation)|SetLookAt%20Zoom%20out%20Acceleration (Variables|/Game/Blueprints/GameTriggers/BP_LookAtArea.BP_LookAtArea_C|GetZoomOutAcceleration _currentlookatbp))
        (Variables|LookAt(calculation)|SetLookAt%20Zoom%20in%20Top%20Speed (Variables|/Game/Blueprints/GameTriggers/BP_LookAtArea.BP_LookAtArea_C|GetZoomInTopSpeed _currentlookatbp))
        (Variables|LookAt(calculation)|SetLookAt%20Zoom%20out%20Top%20Speed (Variables|/Game/Blueprints/GameTriggers/BP_LookAtArea.BP_LookAtArea_C|GetZoomOutTopSpeed _currentlookatbp))
        (Variables|LookAt(calculation)|SetLookatoffset (Variables|/Game/Blueprints/GameTriggers/BP_LookAtArea.BP_LookAtArea_C|GetCamera%20Offset _currentlookatbp))
        (Default|PressedLookatPrompt _currentlookatbp)))))

(event Custom|LookAtCalculation
  (bind _returnvalue (Game|GetPlayerController 0))
  (bind _returnvalue_2 (Game|GetPlayerController 0))
  (bind _returnvalue_3 (Game|GetPlayerController 0))
  (bind _springarm (Variables|Default|GetSpringArm))
  (bind _springarm_2 (Variables|Default|GetSpringArm))
  (bind _springarm_3 (Variables|Default|GetSpringArm))
  (bind _springarm_4 (Variables|Default|GetSpringArm))
  (bind _springarm_5 (Variables|Default|GetSpringArm))
  (if (Variables|LookAt(calculation)|GetLookAtActive)
    ;[1 1 1] Set Springarm Length and offset
    (Variables|/Script/Engine.SpringArmComponent|SetTargetArmLength _springarm_2 (Math|Interpolation|FInterpTo (Variables|/Script/Engine.SpringArmComponent|GetTargetArmLength _springarm_2) (Variables|LookAt(calculation)|GetLookAtSpringarm) (Variables|Default|GetDelta%20Time) (Math|Interpolation|Ease "EaseIn" (Variables|LookAt(calculation)|GetLookAt%20Zoom%20in%20Acceleration) 0.0 (Variables|LookAt(calculation)|GetLookAt%20Zoom%20in%20Top%20Speed) 2.0)))
    (Variables|/Script/Engine.SpringArmComponent|SetSocketOffset _springarm (Math|Interpolation|VInterpTo (Variables|/Script/Engine.SpringArmComponent|GetSocketOffset _springarm) (Variables|LookAt(calculation)|GetLookatoffset) (Variables|Default|GetDelta%20Time) (Math|Interpolation|Ease "EaseIn" (Variables|LookAt(calculation)|GetLookAt%20Zoom%20in%20Acceleration) 0.0 (Variables|LookAt(calculation)|GetLookAt%20Zoom%20in%20Top%20Speed) 2.0)))
    (Variables|LookAt(calculation)|SetLookAtBackToDefault false)
    (Pawn|SetControlRotation _returnvalue (Math|Interpolation|RInterpTo (Pawn|GetControlRotation _returnvalue :!class /Script/Engine.Controller) (Math|Rotator|FindLookatRotation (Transformation|GetActorLocation (Pawn|GetControlledPawn _returnvalue)) (Variables|LookAt(calculation)|GetLookAtVector)) (Variables|Default|GetDelta%20Time) (Variables|SensitivityTweak|GetLookAt%20Interp%20Speed)))
    (bind _output_get (Variables|LookAt(calculation)|SetLookAtTimer (+ (Variables|Default|GetDelta%20Time) (Variables|LookAt(calculation)|GetLookAtTimer))))
    (if (>= _output_get (Variables|LookAt(calculation)|GetLookAt%20Duration))
      (Variables|LookAt(calculation)|SetLookAtActive false)
      (else
        ;[1 1 1] Lower Sensitivity to preset
        (if (Variables|Default|GetLookat%20Sensitivity%20is%20default)
          (Variables|/Script/Engine.PlayerController|SetInputPitchScale _returnvalue_2 (Variables|SensitivityTweak|GetPitch%20Locked%20Sensitivity))
          (Variables|/Script/Engine.PlayerController|SetInputYawScale _returnvalue_2 (Variables|SensitivityTweak|GetYaw%20Locked%20Sensitivity))
          (Variables|Default|SetLookat%20Sensitivity%20is%20default false))))
    (elif (not (Variables|LookAt(calculation)|GetLookAtBackToDefault))
      ;[1 1 1] Reset springarm and offset
      (Variables|/Script/Engine.SpringArmComponent|SetTargetArmLength _springarm_4 (Math|Interpolation|FInterpTo (Variables|/Script/Engine.SpringArmComponent|GetTargetArmLength _springarm_4) (Variables|LookAt(calculation)|GetDefault%20Springarm%20Length) (Variables|Default|GetDelta%20Time) (Math|Interpolation|Ease "EaseIn" (Variables|LookAt(calculation)|GetLookAt%20Zoom%20out%20Acceleration) 0.0 (Variables|LookAt(calculation)|GetLookAt%20Zoom%20out%20Top%20Speed) 2.0)))
      (bind _output_get_2 (Variables|/Script/Engine.SpringArmComponent|SetSocketOffset _springarm_3 (Math|Interpolation|VInterpTo (Variables|/Script/Engine.SpringArmComponent|GetSocketOffset _springarm_3) (Variables|LookAt(calculation)|GetDefaultLookatOffset) (Variables|Default|GetDelta%20Time) (Math|Interpolation|Ease "EaseIn" (Variables|LookAt(calculation)|GetLookAt%20Zoom%20out%20Acceleration) 0.0 (Variables|LookAt(calculation)|GetLookAt%20Zoom%20out%20Top%20Speed) 2.0))))
      ;[1 1 1] Reset Completion
      (if (and (Math|Vector|Equal(Vector) _output_get_2 (Variables|LookAt(calculation)|GetDefaultLookatOffset) 0.01) (Math|Float|NearlyEqual(Float) (Variables|/Script/Engine.SpringArmComponent|GetTargetArmLength (Variables|Default|GetSpringArm)) (Variables|LookAt(calculation)|GetDefault%20Springarm%20Length) 0.01))
        (Variables|LookAt(calculation)|SetLookAtBackToDefault true)
        (Variables|LookAt(calculation)|SetCurrentLookAtBP 0)
        (Variables|/Script/Engine.SpringArmComponent|SetTargetArmLength _springarm_5 (Variables|LookAt(calculation)|GetDefault%20Springarm%20Length))
        (Variables|/Script/Engine.SpringArmComponent|SetSocketOffset _springarm_5 (Variables|LookAt(calculation)|GetDefaultLookatOffset)))
      ;[1 1 1] Reset Sensitivity
      (if (not (Variables|Default|GetLookat%20Sensitivity%20is%20default))
        (Variables|/Script/Engine.PlayerController|SetInputPitchScale _returnvalue_3 (Variables|Default|GetDefaultPitchScale))
        (Variables|/Script/Engine.PlayerController|SetInputYawScale _returnvalue_3 (Variables|Default|GetDefaultYawScale))
        (Variables|Default|SetLookat%20Sensitivity%20is%20default true)))))

(event EventBeginPlay
  (bind _returnvalue (Game|GetPlayerController 0))
  ;[1 1 1] Set up, get spirit reference, and triggering start camera
  (Input|EnableInput (Game|GetPlayerController 0))
  (bind _asbp_spirit (Utilities|Casting|CastToBP_Spirit (Game|GetPlayerCharacter 0)))
  (Variables|Default|SetSpirit _asbp_spirit)
  (CallFunction|UseCamera)
  (bind _returnvalue_2 (Actor|GetActorOfClass "/Game/Blueprints/GameTriggers/StartCamera.StartCamera_C"))
  (Utilities|IsValid _returnvalue_2
    (:Is%20Valid
      (Default|CallStart _returnvalue_2))
    (:Is%20Not%20Valid
      (Development|PrintString "Start Camera not found")))
  ;[1 1 1] calculate defeault distance from camera to player
  (Variables|Default|SetDefault%20Camera%20Distance (Math|Float|Truncate (Math|Vector|Distance(Vector) (Transformation|GetWorldLocation (Variables|Default|GetCamera)) (Transformation|GetWorldLocation (Variables|Default|GetLocation%20And%20Pitch%20Tracker)))))
  (Variables|Default|SetDefaultYawScale (Variables|/Script/Engine.PlayerController|GetInputYawScale _returnvalue))
  (Variables|Default|SetDefaultPitchScale (Variables|/Script/Engine.PlayerController|GetInputPitchScale _returnvalue))
  (Variables|LookAt(calculation)|SetDefault%20Springarm%20Length (Variables|/Script/Engine.SpringArmComponent|GetTargetArmLength (Variables|Default|GetSpringArm)))
  (Variables|LookAt(calculation)|SetDefaultLookatOffset (Variables|/Script/Engine.SpringArmComponent|GetSocketOffset (Variables|Default|GetSpringArm))))

(event EventTick
  (params (DeltaSeconds :type Float%20%28single-precision%29))
  (bind _spirit (Variables|Default|GetSpirit))
  (bind _location_and_pitch_tracker (Variables|Default|GetLocation%20And%20Pitch%20Tracker))
  (bind _location_and_pitch_tracker_2 (Variables|Default|GetLocation%20And%20Pitch%20Tracker))
  (bind _spirit_2 (Variables|Default|GetSpirit))
  (bind _returnvalue (Transformation|GetActorLocation _spirit))
  (bind _returnvalue_2 (Transformation|GetWorldLocation _location_and_pitch_tracker_2))
  (bind _returnvalue_3 (Transformation|GetActorLocation _spirit_2))
  (CallFunction|ReviveCam)
  (CallFunction|LookatCalculation)
  (CallFunction|Sandstorm)
  (CallFunction|RotateTick DeltaSeconds) ; To split the rotation calculation
  (bind _output_get (Variables|Default|SetDelta%20Time DeltaSeconds))
  ;[1 1 1] Calculation for post rotation easing of follow
  (Variables|Default|SetRotateMultiplier (Class|KismetMathLibrary|FInterpEaseinOut (Variables|Default|GetRotateMultiplier) 1.0 _output_get (Variables|PostRotationVariables(calculation)|GetPostRotationTrackingEaseOutExponent)))
  (CallFunction|RotatetoMovement) ; Calls rotate To player direction if player is not turning camera
  ;[1 1 1] Parent Location and Pitch to Rotation Yaw if input is detected
  (if (== (Input|AxisValues|GetTurn) 0.0)
    (if (Variables|Default|GetIs%20attached%20to%20Root)
      _
      (else
        (Transformation|AttachComponentToComponent _location_and_pitch_tracker (Variables|Default|GetDefaultSceneRoot) "None" "KeepWorld" "KeepWorld" "KeepRelative" false)
        (Variables|Default|SetIs%20attached%20to%20Root true)
        (Variables|Default|SetIs%20attached%20to%20Rotator false)))
    (elif (Variables|Default|GetIs%20attached%20to%20Rotator)
      ;;[1 1 1] calculation for post rotation ease to follow
      (Variables|Default|SetRotateMultiplier (Class|KismetMathLibrary|FInterpEaseinOut (Variables|Default|GetRotateMultiplier) 0.0 (Variables|Default|GetDelta%20Time) (Variables|PostRotationVariables(calculation)|GetPostRotationTrackingEaseInExponent)))
      (else
        (Transformation|AttachComponentToComponent _location_and_pitch_tracker (Variables|Default|GetRotation%20Yaw%20Tracker) "None" "KeepWorld" "KeepWorld" "KeepRelative" false)
        (Variables|Default|SetIs%20attached%20to%20Rotator true)
        (Variables|Default|SetIs%20attached%20to%20Root false))))
  (if (> (Math|Vector|Distance(Vector) (Transformation|GetWorldLocation (Variables|Default|GetLocation%20And%20Pitch%20Tracker)) _returnvalue) (Variables|Default|GetTeleport%20Trigger%20Distance))
    ;[1 1 1] Teleport Location Tracker if player is too far
    (Transformation|SetWorldLocation (Variables|Default|GetLocation%20And%20Pitch%20Tracker) _returnvalue false false)
    (else
      ;[1 1 1] Ease Location Tracker towards spirit, strength depends on distance
      (Transformation|SetWorldLocation (Variables|Default|GetLocation%20And%20Pitch%20Tracker) (Math|Interpolation|Ease "EaseInOut" (Variables|Default|GetDelta%20Time) _returnvalue_2 _returnvalue_3 (* (* (- (Variables|Default|GetCamera%20follow%20Sensitivity) (* (Math|Vector|Distance(Vector) _returnvalue_2 _returnvalue_3) 0.01)) (- 1.0 (/ (Math|Float|Absolute(Float) (.Pitch (Math|Rotator|BreakRotator (Transformation|GetWorldRotation (Variables|Default|GetLocation%20And%20Pitch%20Tracker))))) 9e+01)) (/ (Math|Vector|Distance(Vector) (Transformation|GetWorldLocation (Variables|Default|GetCamera)) (Transformation|GetWorldLocation (Variables|Default|GetLocation%20And%20Pitch%20Tracker))) (Math|Conversions|ToFloat(Integer) (Variables|Default|GetDefault%20Camera%20Distance)))) (Variables|Default|GetRotateMultiplier))) false false))))

(fn ConstructionScript)