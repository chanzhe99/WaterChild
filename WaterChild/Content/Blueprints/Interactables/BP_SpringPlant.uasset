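; Spring plant interactable that is revived by watering and then plays a bounce animation and sound on the parent's bounce event.
; While interaction lasts, a pre-grow animation advances at a rate scaled to the required water, with reviving Niagara, and freezes when interaction ends early.
; The grow event fires a burst, disables blocking collision and tick, then loops idle.
; An FMOD Status parameter follows the idle, reviving and grown stages.
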(event Collision|EventActorBeginOverlap
  (params (OtherActor :type Actor%20Object%20Reference)))

(event EventBeginPlay
  (bind _flowermesh (Variables|Default|GetFlowerMesh))
  (Components|Animation|PlayAnimation _flowermesh "/Game/Art/Interactables/SpringPlant/Anim_SpringPlant_PreGrow.Anim_SpringPlant_PreGrow" false)
  (Components|Timeline|SetPlayRate _flowermesh 0.0)
  (bind _returnvalue (Class|FMODBlueprintStatics|PlayEventatLocation "/Game/FMOD/Events/SFX/Plants/SpringPlant.SpringPlant" (Transformation|GetActorTransform)))
  (Variables|Default|SetfmodSpringPlant _returnvalue))

(event EventTick
  (params (DeltaSeconds :type Float%20%28single-precision%29)))

(event EventPlayPlantAnimation
  (bind _flowermesh (Variables|Default|GetFlowerMesh))
  (Components|Timeline|SetPlayRate _flowermesh 1.0)
  (Components|Activation|Activate (Variables|Default|GetNiagaraReviveBurst) false)
  (Components|Animation|PlayAnimation _flowermesh "/Game/Art/Interactables/SpringPlant/Anim_SpringPlant_Grow.Anim_SpringPlant_Grow" false)
  (Class|FMODBlueprintStatics|EventInstanceSetParameter (Variables|Default|GetfmodSpringPlant) "Status" 2.0)
  (Collision|SetCollisionEnabled (Variables|Default|Getprevent%20player%20going%20inside) "NoCollision")
  (Utilities|FlowControl|Delay 1.33)
  (Components|Activation|Deactivate (Variables|Default|GetNiagaraReviving))
  (Actor|Tick|SetActorTickEnabled false)
  (Components|Animation|PlayAnimation _flowermesh "/Game/Art/Interactables/SpringPlant/Anim_SpringPlant_Idle.Anim_SpringPlant_Idle" true))

(event EventBounceAnimation
  (params (Caller :type Spirit%20Object%20Reference))
  (bind _flowermesh (Variables|Default|GetFlowerMesh))
  (|CallParentFunction Caller)
  (Components|Animation|PlayAnimation _flowermesh "/Game/Art/Interactables/SpringPlant/Anim_SpringPlant_Bounce.Anim_SpringPlant_Bounce" false)
  (Class|FMODBlueprintStatics|PlayEventatLocation "/Game/FMOD/Events/SFX/Plants/SpringBounce.SpringBounce" (Transformation|GetActorTransform))
  (Utilities|FlowControl|Delay 1.0)
  (Components|Animation|PlayAnimation _flowermesh "/Game/Art/Interactables/SpringPlant/Anim_SpringPlant_Idle.Anim_SpringPlant_Idle" true))

(event EventOnInteract
  (params (Caller :type Spirit%20Object%20Reference))
  (bind _maxwatervalue (Variables|Default|GetMaxWaterValue))
  (bind _flowermesh (Variables|Default|GetFlowerMesh))
  (bind _currentwatervalue (Variables|Default|GetCurrentWaterValue))
  (bind _returnvalue (/ 0.67 _maxwatervalue))
  (|CallParentFunction Caller)
  (Utilities|FlowControl|Sequence
    (:then_0
      (switch Utilities|FlowControl|Switch|SwitchonEPlantState (Variables|Default|GetPlantState)
        (:Growing
          (Components|Activation|Activate (Variables|Default|GetNiagaraReviving) false)
          (Class|FMODBlueprintStatics|EventInstanceSetParameter (Variables|Default|GetfmodSpringPlant) "Status" 1.0))))
    (:then_1
      (if (not (>= _currentwatervalue (Variables|Default|GetMaxWaterValue)))
        (if (Variables|Default|GetbSetPreGrow)
          (Components|Timeline|SetPlayRate _flowermesh _returnvalue)
          (else
            (Components|Timeline|SetPlayRate _flowermesh _returnvalue)
            (Components|Animation|PlayAnimation _flowermesh "/Game/Art/Interactables/SpringPlant/Anim_SpringPlant_PreGrow.Anim_SpringPlant_PreGrow" false)
            (Variables|Default|SetbSetPreGrow true)))))
    (:then_2
      (Development|PrintString (Utilities|String|ToString(Float) _currentwatervalue)))))

(event EventOnInteractEnd
  (params (Caller :type Spirit%20Object%20Reference))
  (|CallParentFunction Caller)
  (Utilities|FlowControl|Sequence
    (:then_0
      (Components|Activation|Deactivate (Variables|Default|GetNiagaraReviving)))
    (:then_1
      (if (< (Variables|Default|GetCurrentWaterValue) (Variables|Default|GetMaxWaterValue))
        (Components|Timeline|SetPlayRate (Variables|Default|GetFlowerMesh) 0.0)
        (Class|FMODBlueprintStatics|EventInstanceSetParameter (Variables|Default|GetfmodSpringPlant) "Status" 0.0)))))

(fn ConstructionScript)