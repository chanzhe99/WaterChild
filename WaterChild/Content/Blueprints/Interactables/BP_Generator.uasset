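; BP_Generator is an interactable generator that fills with water and, once full, powers a linked Fountain or, failing that, a BathPump.
; Each OnInteract call adds frame delta time to CurrentWater and drives the water material's Blending parameter by fill ratio.
; An interaction at capacity fires the PoweredBurst effect and transfers power only once.
; The construction script contains disconnected spline-mesh pipe-building logic that never runs.
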(event EventBeginPlay
  (bind _water (Variables|Default|GetWater))
  (Rendering|Material|SetScalarParameterValueonMaterials _water "Blending" 0.0)
  (Rendering|Material|SetScalarParameterValueonMaterials _water "MinWaterHeight" -1e+01))

(event Collision|EventActorBeginOverlap
  (params (OtherActor :type Actor%20Object%20Reference)))

(event EventTick
  (params (DeltaSeconds :type Float%20%28single-precision%29)))

(event EventOnInteract
  (params (Caller :type Spirit%20Object%20Reference))
  (bind _bathpump (Variables|Default|GetBathPump))
  (bind _fountain (Variables|Default|GetFountain))
  (if (>= (Variables|Default|GetCurrentWater) (Variables|Default|GetMaxWater))
    (if (not (Variables|Default|GetGeneratorPowerTransferred))
      (Variables|Default|SetGeneratorPowerTransferred true)
      (Components|Activation|Activate (Variables|Default|GetPoweredBurst) false)
      (Utilities|IsValid _fountain
        (:Is%20Valid
          (Default|Powered _fountain))
        (:Is%20Not%20Valid
          (Utilities|IsValid _bathpump
            (:Is%20Valid
              (Default|Powered _bathpump))))))
    (else
      (Variables|Default|SetCurrentWater (+ (Variables|Default|GetCurrentWater) (Utilities|Time|GetWorldDeltaSeconds)))
      (Rendering|Material|SetScalarParameterValueonMaterials (Variables|Default|GetWater) "Blending" (/ (Variables|Default|GetCurrentWater) (Variables|Default|GetMaxWater))))))

(fn ConstructionScript)