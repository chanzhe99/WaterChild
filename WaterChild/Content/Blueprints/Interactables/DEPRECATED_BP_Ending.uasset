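; Deprecated ending interactable: a revivable plant that plays a closing cutscene, then opens Level_01.
; Interacting while the plant is Growing activates a reviving Niagara effect, which stops when interaction ends.
; PlayPlantAnimation fires a burst effect, disables tick and player input, and blends to a cutscene camera.
; It then plays a Level Sequence and waits out its duration before changing level.
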(event EventBeginPlay)

(event Collision|EventActorBeginOverlap
  (params (OtherActor :type Actor%20Object%20Reference)))

(event EventTick
  (params (DeltaSeconds :type Float%20%28single-precision%29)))

(event EventPlayPlantAnimation
  (bind _returnvalue (Game|GetPlayerController 0))
  (Components|Activation|Activate (Variables|Default|GetNiagaraReviveBurst) false)
  (Components|Activation|Deactivate (Variables|Default|GetNiagaraReviving))
  (Actor|Tick|SetActorTickEnabled false)
  (Utilities|FlowControl|Sequence
    (:then_0
      (bind _returnvalue_2 (Sequencer|Player|CreateLevelSequencePlayer (Variables|Default|GetLevel%20Sequence)))
      (Variables|Default|SetSequencePlayer _returnvalue_2))
    (:then_1
      (Input|DisableInput (Game|GetPlayerCharacter 0) _returnvalue)
      (Game|Player|SetViewTargetwithBlend _returnvalue (Variables|Default|GetCutsceneCamera) (Variables|Default|GetTransitionTime) "VTBlend_Cubic" 0.0 false)
      (Utilities|FlowControl|Delay (Variables|Default|GetTransitionTime))
      (Sequencer|Player|Play (Variables|Default|GetSequencePlayer) :!class /Script/MovieScene.MovieSceneSequencePlayer)
      (Utilities|FlowControl|Delay (Class|TimeManagementBlueprintLibrary|ToSeconds(QualifiedFrameTime) (Media|MediaPlayer|GetDuration (Variables|Default|GetSequencePlayer))))
      (Game|OpenLevel(byName) "Level_01"))))

(event EventOnInteract
  (params (Caller :type Spirit%20Object%20Reference))
  (|CallParentFunction Caller)
  (switch Utilities|FlowControl|Switch|SwitchonEPlantState (Variables|Default|GetPlantState)
    (:Growing
      (Components|Activation|Activate (Variables|Default|GetNiagaraReviving) false))))

(event EventOnInteractEnd
  (params (Caller :type Spirit%20Object%20Reference))
  (|CallParentFunction Caller)
  (Components|Activation|Deactivate (Variables|Default|GetNiagaraReviving)))

(fn ConstructionScript)