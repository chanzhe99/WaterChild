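; BP_KidPool is an interactable kiddie pool that fills with water as it is interacted with.
; BeginPlay sets the Water material to empty and disables UnderwaterVolume.
; Each OnInteract call adds delta-time-scaled water, implying per-frame calls, and drives the material's Blending parameter with the fill ratio.
; Interactions after it reaches MaxWater activate PoweringParticles without resetting them and enable UnderwaterVolume.
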(event EventBeginPlay
  (bind _water (Variables|Default|GetWater))
  (Rendering|Material|SetScalarParameterValueonMaterials _water "Blending" 0.0)
  (Rendering|Material|SetScalarParameterValueonMaterials _water "MinWaterHeight" -55.0)
  (Variables|/Script/Engine.PostProcessVolume|SetbEnabled (Variables|Default|GetUnderwaterVolume) false))

(event Collision|EventActorBeginOverlap
  (params (OtherActor :type Actor%20Object%20Reference)))

(event EventTick
  (params (DeltaSeconds :type Float%20%28single-precision%29)))

(event EventOnInteract
  (params (Caller :type Spirit%20Object%20Reference))
  (if (>= (Variables|Default|GetCurrentWater) (Variables|Default|GetMaxWater))
    (Components|Activation|Activate (Variables|Default|GetPoweringParticles) false)
    (Variables|/Script/Engine.PostProcessVolume|SetbEnabled (Variables|Default|GetUnderwaterVolume) true)
    (else
      (Variables|Default|SetCurrentWater (+ (Variables|Default|GetCurrentWater) (* (Utilities|Time|GetWorldDeltaSeconds) (Variables|Default|GetWaterIncreaseRate))))
      (Rendering|Material|SetScalarParameterValueonMaterials (Variables|Default|GetWater) "Blending" (/ (Variables|Default|GetCurrentWater) (Variables|Default|GetMaxWater))))))

(fn ConstructionScript)