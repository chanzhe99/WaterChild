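; BP_ClimbableFlower is an interactable flower that starts hidden and is revived into the level through its OnSpawn event.
; OnSpawn runs once, revealing the actor, playing the flower mesh's opening animation, then enabling query collision on the collider after a delay matching that animation's length.
; It then increments and prints the game mode's PlantsRevived count.
; Once spawned, any actor overlap plays a bounce animation on the mesh.
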(event Custom|OnSpawn
  (if (not (Variables|Default|GetHasSpawned))
    (Variables|Default|SetHasSpawned true)
    (Rendering|SetActorHiddenInGame false)
    (Audio|Components|Audio|Play (Variables|Default|GetFlowerMesh) false)
    (Utilities|FlowControl|Delay (Variables|/Script/Engine.AnimSequenceBase|GetSequenceLength (Variables|Default|GetFlowerOpenAnimation)))
    (Collision|SetCollisionEnabled (Variables|Default|GetFlowerCollider) "QueryOnly")
    (bind _result (Math|Integer|IncrementInt (Variables|/Game/Blueprints/BP_GameMode.BP_GameMode_C|GetPlantsRevived (Variables|Default|GetGMRef)))
      (:%20%20
        (Development|PrintString (Utilities|String|ToString(Integer) _result))))))

(event EventBeginPlay
  (bind _asbp_game_mode (Utilities|Casting|CastToBP_GameMode (Game|GetGameMode)))
  (Variables|Default|SetGMRef _asbp_game_mode)
  (Variables|Default|SetHasSpawned false)
  (Rendering|SetActorHiddenInGame true))

(event Collision|EventActorBeginOverlap
  (params (OtherActor :type Actor%20Object%20Reference))
  (if (Variables|Default|GetHasSpawned)
    (Components|Animation|PlayAnimation (Variables|Default|GetFlowerMesh) "/Game/Art/Interactables/WallCrawler/Anim_Plant_WallCrawler_Flower_Bounce.Anim_Plant_WallCrawler_Flower_Bounce" false)))

(fn ConstructionScript)