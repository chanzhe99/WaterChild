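; Interactable mural that records brush strokes in a render target, which its material reads alongside the clean mural texture.
; The Construction Script creates the render target and dynamic mural and brush materials; a duplicate setup in EventGraph never runs.
; DrawBrush stamps a brush material at a normalized position with randomized orientation.
; Repeated hits on one spot call IncreaseBrushSize up to a maximum, though its increment math is unconnected; moving resets the size.
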(event EventBeginPlay
  (Variables|Default|SetBrushSize (Variables|Default|GetDefaultBrushSize)))

(fn ConstructionScript
  (Utilities|FlowControl|Sequence
    (:then_0
      (bind _returnvalue (Rendering|CreateRenderTarget2D 1024 512 "RTF_RGBA16f"))
      (Variables|Default|SetRenderTarget _returnvalue))
    (:then_1
      (bind _returnvalue_2 (Rendering|Material|CreateDynamicMaterialInstance "/Game/Murals/MI_Mural.MI_Mural" "None" :!class /Script/Engine.KismetMaterialLibrary))
      (Rendering|Material|SetTextureParameterValue _returnvalue_2 "RenderTarget" (Variables|Default|GetRenderTarget))
      (Rendering|Material|SetMaterial (Variables|Default|GetMuralSurface) 0 _returnvalue_2)
      (Rendering|Material|SetTextureParameterValue _returnvalue_2 "T_Clean" (Variables|Default|GetMuralTexture)))
    (:then_2
      ;[1 1 1] Used to create a material which texture can be changed
      (bind _returnvalue_3 (Rendering|Material|CreateDynamicMaterialInstance "/Game/Murals/M_Brush.M_Brush" "None" :!class /Script/Engine.KismetMaterialLibrary))
      (Variables|Default|SetDynamicBrushMaterial _returnvalue_3))))

(fn DrawBrush
  (params (BrushTexture :type Texture%202D%20Object%20Reference) (DrawLocation :type Vector%202D%20Structure) (BrushMaterial :type Material%20Instance%20Object%20Reference))
  (Utilities|FlowControl|Sequence
    (:then_0
      ;[1 1 1] Used when we want to switch the texture of the brush, otherwise unnecessary
      (Rendering|Material|SetTextureParameterValue (Variables|Default|GetDynamicBrushMaterial) "BrushTexture" BrushTexture)
      (Rendering|Material|SetScalarParameterValue "/Game/Murals/MPC_TestBrush.MPC_TestBrush" "BrushOrientation" (Math|Conversions|ToFloat(Integer) (Math|Random|RandomInteger 4)) :!class /Script/Engine.KismetMaterialLibrary))
    (:then_1
      (bind (_canvas _size _context) (Rendering|BeginDrawCanvastoRenderTarget (Variables|Default|GetRenderTarget)))
      (if (Math|Vector|Equal(Vector) DrawLocation (Variables|Default|GetPreviousDrawLocation) 0.1)
        (if (< (Variables|Default|GetBrushSize) (Variables|Default|GetMaxBrushSize))
          (Variables|Default|SetBrushSize (Utilities|IncreaseBrushSize))
          (else
            (Variables|Default|SetBrushSize (Variables|Default|GetMaxBrushSize))))
        (else
          (Variables|Default|SetPreviousDrawLocation DrawLocation)
          (Variables|Default|SetBrushSize (Variables|Default|GetDefaultBrushSize))))
      (Canvas|DrawMaterial :self _canvas :RenderMaterial BrushMaterial :ScreenPosition (- (* _size DrawLocation) (/ (Variables|Default|GetBrushSize) 2.0)) :ScreenSize (Math|Vector2D|MakeVector2D (Variables|Default|GetBrushSize) (Variables|Default|GetBrushSize)) :CoordinateSize "(X=1.000000,Y=1.000000)" :PivotPoint "(X=0.500000,Y=0.500000)")
      (Rendering|EndDrawCanvastoRenderTarget _context)
      (Development|PrintString (Utilities|String|ToString(Float) (Variables|Default|GetBrushSize))))))

(fn SetBrushSettings
  (params (IncrementRate :type Float%20%28single-precision%29) (MaxSize :type Float%20%28single-precision%29))
  (Variables|Default|SetBrushIncrementRate IncrementRate)
  (Variables|Default|SetMaxBrushSize MaxSize))