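; BP_Door is a sliding double door that opens once it holds three charges and its energy color has changed.
; AddCharge raises a material water level on the right door one step per charge, while LerpEnergyColor blends its color.
; Whichever timeline finishes last triggers a delayed opening that slides both panels apart with Niagara effects and FMOD gate audio.
; A function that counts powered generators to set the charge exists but is never run.
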(event Custom|AddCharge
  (bind _currentchargelevel (Variables|Default|GetCurrentChargeLevel))
  (bind _waterlevel (Timeline|WaterLevelTimeline PlayFromStart)
    (:Update
      (switch int _currentchargelevel
        (:0
          (CallFunction|SetDoorMatBlend _waterlevel 0.0 (Variables|WaterLevel|GetWaterLevel1)))
        (:1
          (CallFunction|SetDoorMatBlend _waterlevel (Variables|WaterLevel|GetWaterLevel1) (Variables|WaterLevel|GetWaterLevel2)))
        (:2
          (CallFunction|SetDoorMatBlend _waterlevel (Variables|WaterLevel|GetWaterLevel2) (Variables|WaterLevel|GetWaterLevel3)))))
    (:Finished
      (bind _result (Math|Integer|IncrementInt _currentchargelevel)
        (:%20%20
          (if (and (== _result 3) (Variables|Default|GetEnergyColorChanged))
            (Utilities|FlowControl|Delay (Variables|Default|GetDelayDoorOpenTime))
            (CallFunction|OpenDoors)))))))

(event Custom|OpenDoors
  (bind _dooropendistance (Variables|Default|GetDoorOpenDistance))
  (Components|Activation|Activate (Variables|Default|GetNS_DoorLeft) true)
  (Components|Activation|Activate (Variables|Default|GetNS_DoorRight) true)
  (bind _returnvalue (Class|FMODBlueprintStatics|PlayEvent2D "/Game/FMOD/Events/SFX/Environment/Gate.Gate"))
  (Variables|Default|SetGateFMODEvent _returnvalue)
  (bind _dooropencurve (Timeline|OpenDoorTimeline PlayFromStart)
    (:Update
      (Transformation|SetRelativeLocation (Variables|Default|GetDoorRight) (Math|Vector|MakeVector (* _dooropencurve _dooropendistance 1.0) 0.0 0.0) false false)
      (Transformation|SetRelativeLocation (Variables|Default|GetDoorLeft) (Math|Vector|MakeVector (* _dooropencurve _dooropendistance -1.0) 0.0 0.0) false false))
    (:Finished
      (Components|Activation|Deactivate (Variables|Default|GetNS_DoorLeft))
      (Components|Activation|Deactivate (Variables|Default|GetNS_DoorRight))
      (Class|FMODBlueprintStatics|EventInstanceSetParameter (Variables|Default|GetGateFMODEvent) "FullyOpen" 1.0))))

(event Custom|LerpEnergyColor
  (bind _watercolor (Timeline|LerpColorTimeline PlayFromStart)
    (:Update
      (Rendering|Material|SetScalarParameterValueonMaterials (Variables|Default|GetDoorRight) "WaterColorBlend" _watercolor))
    (:Finished
      (Variables|Default|SetEnergyColorChanged true)
      (if (== (Variables|Default|GetCurrentChargeLevel) 3)
        (Utilities|FlowControl|Delay (Variables|Default|GetDelayDoorOpenTime))
        (CallFunction|OpenDoors)))))

(event EventBeginPlay
  (Rendering|Material|SetScalarParameterValueonMaterials (Variables|Default|GetDoorRight) "Blend" 0.0))

(fn ConstructionScript)

(fn SetDoorMatBlend
  (params (TimelineValue :type Float%20%28single-precision%29) (StartingValue :type Float%20%28single-precision%29) (TargetValue :type Float%20%28single-precision%29))
  (Rendering|Material|SetScalarParameterValueonMaterials (Variables|Default|GetDoorRight) "Blend" (+ StartingValue (- (* TimelineValue TargetValue) (* TimelineValue StartingValue)))))

(fn SetDoortoGeneratorLevel
  (LocalVariables|SetTempLevel 0)
  (for _array_element (Variables|Default|GetGeneratorsList)
    (if (Variables|/Game/Blueprints/Interactables/BP_Generator.BP_Generator_C|GetGeneratorPowerTransferred _array_element)
      (Math|Integer|IncrementInt (LocalVariables|GetTempLevel))))
  (Variables|Default|SetCurrentChargeLevel (LocalVariables|GetTempLevel)))