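; BP_SmallDoor is an interactable double sliding door that opens after receiving three charges.
; Each AddCharge plays a timeline that raises the right door material's Blend parameter to the next water level through a manual lerp.
; After the third charge and a delay, a second timeline slides both halves apart while their NS effects run.
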(event Custom|AddCharge
  (bind _currentchargelevel (Variables|Default|GetCurrentChargeLevel))
  (bind _waterlevel (Timeline|WaterLevelTimeline PlayFromStart)
    (:Update
      (switch int _currentchargelevel
        (:0
          (CallFunction|SetDoorMatBlend _waterlevel 0.0 (Variables|WaterLevel|GetWaterLevel1)))
        (:1
          (CallFunction|SetDoorMatBlend _waterlevel (Variables|WaterLevel|GetWaterLevel1) (Variables|WaterLevel|GetWaterLevel2)))
        (:2
          (CallFunction|SetDoorMatBlend _waterlevel (Variables|WaterLevel|GetWaterLevel2) (Variables|WaterLevel|GetWaterLevel3)))))
    (:Finished
      (bind _result (Math|Integer|IncrementInt _currentchargelevel)
        (:%20%20
          (if (== _result 3)
            (Utilities|FlowControl|Delay (Variables|Default|GetDelayDoorOpenTime))
            (CallFunction|OpenDoors)))))))

(event Custom|OpenDoors
  (bind _dooropendistance (Variables|Default|GetDoorOpenDistance))
  (Components|Activation|Activate (Variables|Default|GetNS_DoorLeft) true)
  (Components|Activation|Activate (Variables|Default|GetNS_DoorRight) true)
  (bind _waterlevel (Timeline|OpenDoorTimeline PlayFromStart)
    (:Update
      (Transformation|SetRelativeLocation (Variables|Default|GetDoorRight) (Math|Vector|MakeVector (* _waterlevel _dooropendistance 1.0) 0.0 0.0) false false)
      (Transformation|SetRelativeLocation (Variables|Default|GetDoorLeft) (Math|Vector|MakeVector (* _waterlevel _dooropendistance -1.0) 0.0 0.0) false false))
    (:Finished
      (Components|Activation|Deactivate (Variables|Default|GetNS_DoorLeft))
      (Components|Activation|Deactivate (Variables|Default|GetNS_DoorRight)))))

(event EventBeginPlay
  (Rendering|Material|SetScalarParameterValueonMaterials (Variables|Default|GetDoorRight) "Blend" 0.0))

(fn ConstructionScript)

(fn SetDoorMatBlend
  (params (TimelineValue :type Float%20%28single-precision%29) (StartingValue :type Float%20%28single-precision%29) (TargetValue :type Float%20%28single-precision%29))
  (Rendering|Material|SetScalarParameterValueonMaterials (Variables|Default|GetDoorRight) "Blend" (+ StartingValue (- (* TimelineValue TargetValue) (* TimelineValue StartingValue)))))