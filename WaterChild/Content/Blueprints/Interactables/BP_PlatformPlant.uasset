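; Interactable platform plant that the player revives with water, making its petal collider solid once fully watered.
; Each interaction below full water eases a morph target on three petal meshes in proportion to the water value.
; At full water it plays the stem animation, burst VFX and weed-raising timeline once, then disables tick after a hand-synced delay.
; An FMOD Status parameter tracks idle, reviving and revived; BeginPlay setup is skipped in Level_New.
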(event EventPlayReviveDoneEffects
  (bind _petalcollider (Variables|Default|GetPetalCollider))
  (if (not (Variables|Default|GetbReviveAnimPlayed))
    (Collision|SetCollisionProfileName _petalcollider "BlockAllDynamic" true :!class /Script/Engine.PrimitiveComponent)
    (Collision|SetCollisionResponsetoChannel _petalcollider "ECC_Visibility" "ECR_Ignore")
    (Collision|SetCollisionResponsetoChannel _petalcollider "ECC_Camera" "ECR_Ignore")
    (Components|Animation|PlayAnimation (Variables|Default|GetStemMesh) "/Game/Art/Interactables/PlatformPlant/AnimatedSmallStem/Plant_PlatformStem_Anim.Plant_PlatformStem_Anim" false)
    (Variables|Default|SetbReviveAnimPlayed true)
    (Utilities|FlowControl|Sequence
      (:then_0
        (Components|Activation|Activate (Variables|Default|GetNiagaraReviveBurst) false)
        (Class|FMODBlueprintStatics|EventInstanceSetParameter (Variables|Default|GetfmodPlatformPlant) "Status" 2.0)
        (Utilities|FlowControl|Delay 1.83) ; Must follow GrowDuration
        (Actor|Tick|SetActorTickEnabled false))
      (:then_1
        (bind _weed_grow_alpha (Timeline|Weed%20Grower PlayFromStart)
          (:Update
            (Transformation|SetRelativeLocation (Variables|Default|GetWeedsComp) (Math|Vector|Lerp(Vector) (Variables|Default|GetWeedStartPosition) (Variables|Default|GetWeedEndPosition) _weed_grow_alpha) false false)))))))

(event Collision|EventActorBeginOverlap
  (params (OtherActor :type Actor%20Object%20Reference)))

(event EventTick
  (params (DeltaSeconds :type Float%20%28single-precision%29))
  (|CallParentFunction DeltaSeconds))

(event EventActivateRevivingEffects
  (params (IsActivateEffects :type Boolean))
  (bind _niagararevivingtemp (Variables|Default|GetNiagaraRevivingTemp))
  (bind _fmodplatformplant (Variables|Default|GetfmodPlatformPlant))
  (if IsActivateEffects
    (Components|Activation|Activate _niagararevivingtemp false)
    (Class|FMODBlueprintStatics|EventInstanceSetParameter _fmodplatformplant "Status" 1.0)
    (else
      (Components|Activation|Deactivate _niagararevivingtemp)
      (Class|FMODBlueprintStatics|EventInstanceSetParameter _fmodplatformplant "Status" 0.0))))

(event EventBeginPlay
  (bind _returnvalue (Game|GetCurrentLevelName true))
  (if (Utilities|Enum|NotEqual(Enum) _returnvalue "Level_New")
    (|CallParentFunction)
    (for _array_element (Variables|Default|GetMeshArray)
      (Components|SkeletalMesh|SetMorphTarget _array_element "Plane004" 1.25 true)
      (bind _returnvalue_2 (Class|FMODBlueprintStatics|PlayEventatLocation "/Game/FMOD/Events/SFX/Plants/PlatformPlant.PlatformPlant" (Transformation|GetActorTransform)))
      (Variables|Default|SetfmodPlatformPlant _returnvalue_2))))

(event EventOnInteract
  (params (Caller :type Spirit%20Object%20Reference))
  (|CallParentFunction Caller)
  (if (>= (Variables|Default|GetCurrentWaterValue) (Variables|Default|GetMaxWaterValue))
    (Class|Plant|PlayReviveDoneEffects)
    (else
      (CallFunction|SetPetalMorphTargetValues))))

(fn ConstructionScript
  (Variables|Default|SetMeshArray (Utilities|Array|MakeArray (Variables|Default|GetPetalMesh1) (Variables|Default|GetPetalMesh2) (Variables|Default|GetPetalMesh3)))
  (bind _output_get (Variables|Default|SetWeedStartPosition (Variables|/Script/Engine.SceneComponent|GetRelativeLocation (Variables|Default|GetWeedsComp))))
  (Variables|Default|SetWeedEndPosition (+ _output_get (* (Math|Vector|VectorUp) 5e+01))))

(fn SetPetalMorphTargetValues
  (for _array_element (Variables|Default|GetMeshArray)
    (Components|SkeletalMesh|SetMorphTarget _array_element "Plane004" (Math|Float|Clamp(Float) (- 1.25 (/ (Variables|Default|GetCurrentWaterValue) (Variables|Default|GetMaxWaterValue))) 0.0 5.0) true)))