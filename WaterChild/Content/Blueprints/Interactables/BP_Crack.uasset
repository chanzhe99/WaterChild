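; Two-hole crack interactable that lets the player's spirit squeeze through, teleporting it from whichever hole it hits to the other.
; On hit, it snaps the spirit to the entrance, disables input, starts the squeeze and blends to that hole's camera.
; Timed delays sequence a fade to black that masks the move, restoring the spirit's view with exit-facing rotation, then fade in and trigger the squeeze-out transition.
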(event OnComponentHit(Hole1Mesh)
  (params (HitComponent :type Primitive%20Component%20Object%20Reference) (OtherActor :type Actor%20Object%20Reference) (OtherComp :type Primitive%20Component%20Object%20Reference) (NormalImpulse :type Vector :default "0, 0, 0") (Hit :type Hit%20Result%20Structure%20%28by%20ref%29))
  (bind _blend_time (Variables|Default|GetBlend%20Time))
  ;[1 1 1] Detect spirit and start enter crack process
  (bind _asbp_spirit (Utilities|Casting|CastToBP_Spirit OtherActor))
  (CallFunction|SetStartTransformandAnimation _asbp_spirit (Variables|Default|GetHole1Transform) (Variables|Default|GetHole1Camera) (Variables|Default|GetHole2Camera))
  ;[1 1 1] Wait for camera to reach entrance camera rot and fade to black
  (Utilities|FlowControl|Delay (Variables|Default|GetBlend%20Time))
  (CameraFades|StartCameraFade :self (Game|GetPlayerCameraManager 0) :ToAlpha 1.0 :Duration _blend_time :bHoldWhenFinished true)
  ;[1 1 1] Wait for fade and set exit transform
  (Utilities|FlowControl|Delay _blend_time)
  (CallFunction|SetEndTransform _asbp_spirit (Variables|Default|GetHole2Transform) (Variables|Default|GetHole2Camera) (Variables|Default|GetHole1Camera) (Variables|Default|GetHole2CameraRot))
  ;[1 1 1] Teleport external camera
  (Default|TeleportCameraTrackertoSpirit (Variables|/Game/Blueprints/BP_Spirit.BP_Spirit_C|GetExternalCamera _asbp_spirit))
  ;[1 1 1] Wait for set exit transform and fade from black
  (Utilities|FlowControl|Delay (Variables|Default|GetBlend%20Time))
  (CameraFades|StartCameraFade :self (Game|GetPlayerCameraManager 0) :FromAlpha 1.0 :Duration (Variables|Default|GetBlend%20Time))
  ;[1 1 1] Start exit crack animation
  (Class|Spirit|TransitiontoStopSqueeze _asbp_spirit))

(event OnComponentHit(Hole2Mesh)
  (params (HitComponent :type Primitive%20Component%20Object%20Reference) (OtherActor :type Actor%20Object%20Reference) (OtherComp :type Primitive%20Component%20Object%20Reference) (NormalImpulse :type Vector :default "0, 0, 0") (Hit :type Hit%20Result%20Structure%20%28by%20ref%29))
  (bind _blend_time (Variables|Default|GetBlend%20Time))
  ;[1 1 1] Detect spirit and start enter crack process
  (bind _asbp_spirit (Utilities|Casting|CastToBP_Spirit OtherActor))
  (CallFunction|SetStartTransformandAnimation _asbp_spirit (Variables|Default|GetHole2Transform) (Variables|Default|GetHole2Camera) (Variables|Default|GetHole1Camera))
  ;[1 1 1] Wait for camera to reach entrance camera rot and fade to black
  (Utilities|FlowControl|Delay (Variables|Default|GetBlend%20Time))
  (CameraFades|StartCameraFade :self (Game|GetPlayerCameraManager 0) :ToAlpha 1.0 :Duration _blend_time :bHoldWhenFinished true)
  ;[1 1 1] Wait for fade and set exit transform
  (Utilities|FlowControl|Delay _blend_time)
  (CallFunction|SetEndTransform _asbp_spirit (Variables|Default|GetHole1Transform) (Variables|Default|GetHole1Camera) (Variables|Default|GetHole2Camera) (Variables|Default|GetHole1CameraRot))
  ;[1 1 1] Teleport external camera
  (Default|TeleportCameraTrackertoSpirit (Variables|/Game/Blueprints/BP_Spirit.BP_Spirit_C|GetExternalCamera _asbp_spirit))
  ;[1 1 1] Wait for set exit transform and fade from black
  (Utilities|FlowControl|Delay (Variables|Default|GetBlend%20Time))
  (CameraFades|StartCameraFade :self (Game|GetPlayerCameraManager 0) :FromAlpha 1.0 :Duration (Variables|Default|GetBlend%20Time))
  ;[1 1 1] Start exit crack animation
  (Class|Spirit|TransitiontoStopSqueeze _asbp_spirit))

(event EventBeginPlay
  ;[1 1 1] Setup
  (bind _asbp_spirit (Utilities|Casting|CastToBP_Spirit (Game|GetPlayerCharacter 0)))
  (Variables|Default|SetSpiritHalfHeight (Math|Vector|MakeVector 0.0 0.0 (Components|Capsule|GetScaledCapsuleHalfHeight (Variables|/Script/Engine.Character|GetCapsuleComponent _asbp_spirit))))
  (Components|Activation|SetActive (Variables|Default|GetHole1Camera) false false)
  (Components|Activation|SetActive (Variables|Default|GetHole2Camera) false false))

(fn ConstructionScript)

(fn SetStartTransformandAnimation
  (params (SpiritObject :type BP%20Spirit%20Object%20Reference) (EntranceTransform :type Scene%20Component%20Object%20Reference) (EntranceCamera :type Camera%20Component%20Object%20Reference) (ExitCamera :type Camera%20Component%20Object%20Reference))
  (bind _returnvalue (Game|GetPlayerController 0))
  (bind _returnvalue_2 (Transformation|GetWorldTransform EntranceTransform))
  ;[1 1 1] Set spirit location and rotation to prepare for entering crack
  (Transformation|SetActorLocationAndRotation SpiritObject (+ (Variables|Default|GetSpiritHalfHeight) (.location _returnvalue_2)) (.rotation _returnvalue_2))
  (Utilities|FlowControl|Sequence
    (:then_0
      ;[1 1 1] Set active view target to the hole that spirit entered from
      (Components|Activation|SetActive ExitCamera false false)
      (Components|Activation|SetActive EntranceCamera true false))
    (:then_1
      ;[1 1 1] Disable player input and start spirit entering crack animation
      (Input|DisableInput SpiritObject _returnvalue)
      (Class|Spirit|SetState SpiritObject "Squeezing")
      (Class|Spirit|TransitiontoSqueeze SpiritObject)
      ;[1 1 1] Blend spirit view target to entrance
      (Game|Player|SetViewTargetwithBlend _returnvalue self (Variables|Default|GetBlend%20Time) "VTBlend_EaseInOut" 1.0 false))))

(fn SetEndTransform
  (params (SpiritObject :type BP%20Spirit%20Object%20Reference) (ExitTransform :type Scene%20Component%20Object%20Reference) (ExitCamera :type Camera%20Component%20Object%20Reference) (EntranceCamera :type Camera%20Component%20Object%20Reference) (ExitCameraRot :type Spring%20Arm%20Component%20Object%20Reference))
  (bind _returnvalue (Game|GetPlayerController 0))
  (bind _returnvalue_2 (Transformation|GetWorldTransform ExitTransform))
  (Transformation|SetActorLocationAndRotation SpiritObject (+ (Variables|Default|GetSpiritHalfHeight) (.location _returnvalue_2)) (Math|Rotator|CombineRotators (.rotation _returnvalue_2) "0.0,180.0,0.0"))
  (Components|Activation|SetActive EntranceCamera false false)
  (Components|Activation|SetActive ExitCamera true false)
  (Game|Player|SetViewTargetwithBlend _returnvalue (Game|GetPlayerCharacter 0) 0.0 "VTBlend_EaseInOut" 1.0 false)
  (Pawn|SetControlRotation _returnvalue (Transformation|GetWorldRotation ExitCameraRot)))