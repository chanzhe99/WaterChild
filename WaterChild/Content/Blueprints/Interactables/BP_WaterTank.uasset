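; Interactable bathhouse water tank that fills while the player interacts, raising the water material and playing the spinner animation.
; Once full, further interaction activates powering particles and notifies the referenced bath pump.
; Tick sums the fill ratios of three generators and the tank to drive the tank mesh's Blend parameter up to half, then ramps it over time to full once the maximum is reached.
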(event Custom|Powering
  (params (IndentBarLevel :type Float%20%28single-precision%29))
  (Variables|Default|SetCurrentIndentBarLevel IndentBarLevel))

(event EventBeginPlay
  (bind _water (Variables|Default|GetWater))
  (bind _watertankspinner (Variables|Default|GetWaterTankSpinner))
  (Rendering|Material|SetScalarParameterValueonMaterials _water "Blending" 0.0)
  (Rendering|Material|SetScalarParameterValueonMaterials _water "MinWaterHeight" -79.0)
  (Components|Animation|PlayAnimation _watertankspinner "/Game/Art/Meshes/Modular_Assets/HousingArea_Modular_2/SM_Bathhouse/SM_Bathhouse_BIG/SK_WaterTank/SM_Bathhouse_WaterTank_Spin_Anim.SM_Bathhouse_WaterTank_Spin_Anim" true)
  (Components|Timeline|SetPlayRate _watertankspinner 0.0))

(event Collision|EventActorBeginOverlap
  (params (OtherActor :type Actor%20Object%20Reference)))

(event EventTick
  (params (DeltaSeconds :type Float%20%28single-precision%29))
  (bind _generatorlevels (Variables|Default|GetGeneratorLevels))
  (bind _maxindentbarlevel (Variables|Default|GetMaxIndentBarLevel))
  (for (_array_element _array_index) (Variables|Default|GetGenerators)
    (Utilities|Array|SetArrayElem _generatorlevels _array_index (/ (Variables|/Game/Blueprints/Interactables/BP_Generator.BP_Generator_C|GetCurrentWater _array_element) (Variables|/Game/Blueprints/Interactables/BP_Generator.BP_Generator_C|GetMaxWater _array_element)))
    (Variables|Default|SetCurrentIndentBarLevel (+ (Utilities|Array|Get(acopy) _generatorlevels) (Utilities|Array|Get(acopy) _generatorlevels 1) (Utilities|Array|Get(acopy) _generatorlevels 2) (/ (Variables|Default|GetCurrentWater) (Variables|Default|GetMaxWater))))
    (if (< (Variables|Default|GetCurrentIndentBarLevel) _maxindentbarlevel)
      (bind _output_get (Variables|Default|SetMatParamValue (* (/ (Variables|Default|GetCurrentIndentBarLevel) _maxindentbarlevel) 0.5)))
      (Rendering|Material|SetScalarParameterValueonMaterials (Variables|Default|GetWaterTankMesh) "Blend" _output_get)
      (elif (< (Variables|Default|GetMatParamValue) 1.0)
        (Development|PrintString (Utilities|String|ToString(Float) (+ (Variables|Default|GetMatParamValue) (* (Utilities|Time|GetWorldDeltaSeconds) 0.05))))
        (bind _output_get_2 (Variables|Default|SetMatParamValue (+ (Variables|Default|GetMatParamValue) (* (Utilities|Time|GetWorldDeltaSeconds) 0.05))))
        (Rendering|Material|SetScalarParameterValueonMaterials (Variables|Default|GetWaterTankMesh) "Blend" _output_get_2)))))

(event EventOnInteract
  (params (Caller :type Spirit%20Object%20Reference))
  (if (>= (Variables|Default|GetCurrentWater) (Variables|Default|GetMaxWater))
    (Components|Activation|Activate (Variables|Default|GetPoweringParticles) false)
    (Default|WaterTankFilled (Variables|Default|GetBathPumpRef))
    (else
      (Variables|Default|SetCurrentWater (+ (Variables|Default|GetCurrentWater) (Utilities|Time|GetWorldDeltaSeconds)))
      (Rendering|Material|SetScalarParameterValueonMaterials (Variables|Default|GetWater) "Blending" (/ (Variables|Default|GetCurrentWater) (Variables|Default|GetMaxWater)))
      (Components|Timeline|SetPlayRate (Variables|Default|GetWaterTankSpinner) 1.0))))

(event EventOnInteractEnd
  (params (Caller :type Spirit%20Object%20Reference))
  (Components|Timeline|SetPlayRate (Variables|Default|GetWaterTankSpinner) 0.0))

(fn ConstructionScript)