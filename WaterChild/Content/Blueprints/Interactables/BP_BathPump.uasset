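; Bath pump that drives two three-tier fountains and fills the bath water in response to power and a filled water tank.
; Each Powered call advances Stage, and SetFountainStates updates the falls' material state, switching from sand with dust particles to water once the tank is full.
; At stage three with a full tank, Tick raises CurrentWater and drives the water material's Blending parameter.
; OnInteract also increments CurrentWater and prints it.
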(event Custom|Powered
  (bind _result (Math|Integer|IncrementInt (Variables|Default|GetStage))
    (:%20%20
      (Variables|Default|SetStage _result)
      (CallFunction|SetFountainStates))))

(event Custom|WaterTankFilled
  (Variables|Default|SetWaterTankFull true)
  (Variables|Default|SetActivateSandFallParticles false)
  (CallFunction|SetFountainStates))

(event EventBeginPlay
  (bind _water (Variables|Default|GetWater))
  (Rendering|Material|SetScalarParameterValueonMaterials _water "Blending" 0.0)
  (Rendering|Material|SetScalarParameterValueonMaterials _water "MinWaterHeight" -135.0))

(event EventTick
  (params (DeltaSeconds :type Float%20%28single-precision%29))
  (if (Math|Boolean|ANDBoolean (Variables|Default|GetWaterTankFull) (== (Variables|Default|GetStage) 3) (< (Variables|Default|GetCurrentWater) (Variables|Default|GetMaxWater)))
    (Variables|Default|SetCurrentWater (+ (Variables|Default|GetCurrentWater) (Utilities|Time|GetWorldDeltaSeconds)))
    (Rendering|Material|SetScalarParameterValueonMaterials (Variables|Default|GetWater) "Blending" (/ (Variables|Default|GetCurrentWater) (Variables|Default|GetMaxWater)))))

(event EventOnInteract
  (params (Caller :type Spirit%20Object%20Reference))
  (if (not (>= (Variables|Default|GetCurrentWater) (Variables|Default|GetMaxWater)))
    (bind _output_get (Variables|Default|SetCurrentWater (+ (Variables|Default|GetCurrentWater) (Utilities|Time|GetWorldDeltaSeconds))))
    (Development|PrintString (Utilities|String|ToString(Float) _output_get))))

(fn ConstructionScript
  (Rendering|Material|SetScalarParameterValueonMaterials (Variables|Default|GetFountain1Fall1) "Stage" 0.0)
  (Components|Activation|SetAutoActivate (Variables|Default|GetFall1Dust1) false))

(fn SetFountainStates
  (bind _fall3dust1 (Variables|Default|GetFall3Dust1))
  (bind _fall1dust2 (Variables|Default|GetFall1Dust2))
  (if (Variables|Default|GetWaterTankFull)
    (Variables|Default|SetFountainState 2.0)
    (else
      (Variables|Default|SetFountainState 1.0)))
  (switch int (Variables|Default|GetStage)
    (:1
      (Rendering|Material|SetScalarParameterValueonMaterials (Variables|Default|GetFountain1Fall1) "Stage" (Variables|Default|GetFountainState))
      (if (Variables|Default|GetActivateSandFallParticles)
        (Components|Activation|Activate _fall1dust2 false)
        (else
          (Components|Activation|Deactivate _fall1dust2))))
    (:2
      (Rendering|Material|SetScalarParameterValueonMaterials (Variables|Default|GetFountain1Fall2) "Stage" (Variables|Default|GetFountainState))
      (if (Variables|Default|GetActivateSandFallParticles)
        (Components|Activation|Activate (Variables|Default|GetFall2Dust2) false)
        (else
          (Components|Activation|Deactivate (Variables|Default|Get2Fall2Dust2)))))
    (:3
      (Rendering|Material|SetScalarParameterValueonMaterials (Variables|Default|GetFountain1Fall3) "Stage" (Variables|Default|GetFountainState))
      (if (Variables|Default|GetActivateSandFallParticles)
        (Components|Activation|Activate _fall3dust1 false)
        (else
          (Components|Activation|Deactivate _fall3dust1))))))