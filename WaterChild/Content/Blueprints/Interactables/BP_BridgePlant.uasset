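; Interactable bridge plant that grows from a pre-growing pose into an idle bridge as it is watered.
; While interacted with, it advances the pre-grow animation at a rate scaled to the max water value and pauses it if interaction ends early.
; A reviving Niagara effect runs during interaction in the Growing state.
; PlayPlantAnimation plays the growing animation with a burst effect, then loops idle after a fixed delay.
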(event Collision|EventActorBeginOverlap
  (params (OtherActor :type Actor%20Object%20Reference)))

(event EventOnInteract
  (params (Caller :type Spirit%20Object%20Reference))
  (bind _maxwatervalue (Variables|Default|GetMaxWaterValue))
  (bind _bridgemesh (Variables|Default|GetBridgeMesh))
  (bind _returnvalue (/ 1.3 _maxwatervalue))
  (|CallParentFunction Caller)
  (Utilities|FlowControl|Sequence
    (:then_0
      (switch Utilities|FlowControl|Switch|SwitchonEPlantState (Variables|Default|GetPlantState)
        (:Growing
          (Components|Activation|Activate (Variables|Default|GetNiagaraReviving) false))))
    (:then_1
      (if (not (>= (Variables|Default|GetCurrentWaterValue) (Variables|Default|GetMaxWaterValue)))
        (if (Variables|Default|GetbSetPreGrow)
          (Components|Timeline|SetPlayRate _bridgemesh _returnvalue)
          (else
            (Components|Timeline|SetPlayRate _bridgemesh _returnvalue)
            (Components|Animation|PlayAnimation _bridgemesh "/Game/Art/Interactables/BridgePlant/Animations/Anim_Plant_Bridge_PreGrowing.Anim_Plant_Bridge_PreGrowing" false)
            (Variables|Default|SetbSetPreGrow true)))))))

(event EventOnInteractEnd
  (params (Caller :type Spirit%20Object%20Reference))
  (|CallParentFunction Caller)
  (Utilities|FlowControl|Sequence
    (:then_0
      (Components|Activation|Deactivate (Variables|Default|GetNiagaraReviving)))
    (:then_1
      (if (< (Variables|Default|GetCurrentWaterValue) (Variables|Default|GetMaxWaterValue))
        (Components|Timeline|SetPlayRate (Variables|Default|GetBridgeMesh) 0.0)))))

(event EventPlayPlantAnimation
  (bind _bridgemesh (Variables|Default|GetBridgeMesh))
  (Components|Timeline|SetPlayRate _bridgemesh 1.0)
  (Components|Activation|Activate (Variables|Default|GetNiagaraReviveBurst) false)
  (Components|Animation|PlayAnimation _bridgemesh "/Game/Art/Interactables/BridgePlant/Animations/Anim_Plant_Bridge_Growing.Anim_Plant_Bridge_Growing" false)
  (Utilities|FlowControl|Delay 3.0)
  (Components|Activation|Deactivate (Variables|Default|GetNiagaraReviveBurst))
  (Components|Animation|PlayAnimation _bridgemesh "/Game/Art/Interactables/BridgePlant/Animations/Anim_Plant_Bridge_Idle.Anim_Plant_Bridge_Idle" true))

(event EventBeginPlay
  (bind _bridgemesh (Variables|Default|GetBridgeMesh))
  (Variables|Default|SetMaxWaterValue 3.0)
  (Components|Animation|PlayAnimation _bridgemesh "/Game/Art/Interactables/BridgePlant/Animations/Anim_Plant_Bridge_PreGrowing.Anim_Plant_Bridge_PreGrowing" false)
  (Components|Timeline|SetPlayRate _bridgemesh 0.0))

(event EventTick
  (params (DeltaSeconds :type Float%20%28single-precision%29)))

(fn ConstructionScript)