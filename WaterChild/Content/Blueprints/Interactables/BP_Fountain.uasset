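; Interactable fountain puzzle that the player fills with water and powers through three stages to bring to life.
; Interacting raises a water material blend until full, then enables the underwater volume and caustics decal.
; Each Powered call advances a stage and adjusts gear audio parameters; full water at stage three starts staggered particle layers and fountain sound.
; Overlap triggers handle a one-time blown animation and set FMOD music stems by completion state.
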(event OnComponentBeginOverlap(InitialBlownTrigger)
  (params (OverlappedComponent :type Primitive%20Component%20Object%20Reference) (OtherActor :type Actor%20Object%20Reference) (OtherComp :type Primitive%20Component%20Object%20Reference) (OtherBodyIndex :type Integer) (bFromSweep :type Boolean) (SweepResult :type Hit%20Result%20Structure%20%28by%20ref%29))
  (bind _fountainanimbp (Variables|Default|GetFountainAnimBP))
  (if (== OtherActor (Game|GetPlayerCharacter 0))
    (if (not (Variables|/Game/Art/Interactables/Fountain/Animations/AnimBP_Fountain.AnimBP_Fountain_C|GetIsBlown _fountainanimbp))
      (Variables|/Game/Art/Interactables/Fountain/Animations/AnimBP_Fountain.AnimBP_Fountain_C|SetIsBlown _fountainanimbp true)
      (Class|FMODAudioComponent|Play (Variables|Default|GetGearsCreak)))))

(event OnComponentBeginOverlap(MusicArea)
  (params (OverlappedComponent :type Primitive%20Component%20Object%20Reference) (OtherActor :type Actor%20Object%20Reference) (OtherComp :type Primitive%20Component%20Object%20Reference) (OtherBodyIndex :type Integer) (bFromSweep :type Boolean) (SweepResult :type Hit%20Result%20Structure%20%28by%20ref%29))
  (if (== (Game|GetPlayerCharacter 0) OtherActor)
    (if (and (== (Variables|Default|GetCurrentStage) 3) (>= (Variables|Default|GetCurrentWater) (Variables|Default|GetMaxWater)))
      (CallFunction|MusicActivated)
      (else
        (CallFunction|MusicInactive)))))

(event Custom|Powered
  (bind _gears (Variables|Default|GetGears))
  (bind _gears_2 (Variables|Default|GetGears))
  (bind _result (Math|Integer|IncrementInt (Variables|Default|GetCurrentStage))
    (:%20%20
      (bind _output_get (Variables|Default|SetCurrentStage _result))
      (CallFunction|GearsVolPowered)
      (Utilities|FlowControl|Sequence
        (:then_0
          (if (and (== _output_get 3) (>= (Variables|Default|GetCurrentWater) (Variables|Default|GetMaxWater)))
            (Class|FMODAudioComponent|SetParameter _gears_2 "BigGearVol" 0.0)
            (Class|FMODAudioComponent|SetParameter _gears_2 "Running" 0.0)
            (Class|FMODAudioComponent|Play _gears_2)
            (Utilities|FlowControl|Delay 1.0)
            (Class|FMODAudioComponent|Play (Variables|Default|GetFountainSound))
            (CallFunction|ActivateLayer (Variables|Default|GetLayer1Particles))
            (Utilities|FlowControl|Delay 1.0)
            (CallFunction|ActivateLayer (Variables|Default|GetLayer2Particles))
            (Utilities|FlowControl|Delay 1.0)
            (CallFunction|ActivateLayer (Variables|Default|GetLayer3Particles))
            (Utilities|FlowControl|Delay 1.0)
            (CallFunction|ActivateLayer (Variables|Default|GetTopLayerParticles))))
        (:then_1
          (if (== (Variables|Default|GetCurrentStage) 1)
            (Class|FMODAudioComponent|SetParameter _gears "MediumGearVol" 0.0)
            (Class|FMODAudioComponent|Play _gears :!label _label)))
        (:then_2
          (if (== (Variables|Default|GetCurrentStage) 2)
            (Class|FMODAudioComponent|SetParameter _gears "SmallGearVol" 0.0)
            (goto _label)))))))

(event EventBeginPlay
  (bind _water (Variables|Default|GetWater))
  (bind _asanim_bp_fountain (Utilities|Casting|CastToAnimBP_Fountain (Components|SkeletalMesh|GetAnimInstance (Variables|Default|GetFountainSpinMesh))))
  (Variables|Default|SetFountainAnimBP _asanim_bp_fountain)
  (Variables|Default|SetLayer1Particles (Utilities|Array|MakeArray (Variables|Default|GetLayer1Stream1) (Variables|Default|GetLayer1Stream2) (Variables|Default|GetLayer1Stream3) (Variables|Default|GetLayer1Stream4) (Variables|Default|GetLayer1Stream5)))
  (Variables|Default|SetLayer2Particles (Utilities|Array|MakeArray (Variables|Default|GetLayer2Stream1) (Variables|Default|GetLayer2Stream2) (Variables|Default|GetLayer2Stream3) (Variables|Default|GetLayer2Stream4) (Variables|Default|GetLayer2Stream5)))
  (Variables|Default|SetLayer3Particles (Utilities|Array|MakeArray (Variables|Default|GetLayer3Stream1) (Variables|Default|GetLayer3Stream2) (Variables|Default|GetLayer3Stream3) (Variables|Default|GetLayer3Stream4) (Variables|Default|GetLayer3Stream5)))
  (Variables|Default|SetTopLayerParticles (Utilities|Array|MakeArray (Variables|Default|GetTopStream1) (Variables|Default|GetTopStream2) (Variables|Default|GetTopStream3)))
  (Rendering|Material|SetScalarParameterValueonMaterials _water "Blending" 0.0)
  (Rendering|Material|SetScalarParameterValueonMaterials _water "MinWaterHeight" -3e+01)
  (Variables|/Script/Engine.PostProcessVolume|SetbEnabled (Variables|Default|GetUnderwaterVolume) false)
  (Rendering|SetVisibility (Variables|/Script/Engine.DecalActor|GetDecal (Variables|Default|GetWaterCausticsDecal)) false false))

(event EventOnInteractEnd
  (params (Caller :type Spirit%20Object%20Reference))
  (Variables|/Game/Art/Interactables/Fountain/Animations/AnimBP_Fountain.AnimBP_Fountain_C|SetIsFilling (Variables|Default|GetFountainAnimBP) false)
  (if (and (< (Variables|Default|GetCurrentWater) (Variables|Default|GetMaxWater)) (<= (Variables|Default|GetCurrentStage) 0))
    (Class|FMODAudioComponent|SetParameter (Variables|Default|GetGears) "Running" 1.0)
    (Variables|Default|SetbGearsPlaying false)
    (else
      (CallFunction|GearsVolonInteractEnd))))

(event EventOnInteract
  (params (Caller :type Spirit%20Object%20Reference))
  (bind _gears (Variables|Default|GetGears))
  (Variables|/Game/Art/Interactables/Fountain/Animations/AnimBP_Fountain.AnimBP_Fountain_C|SetIsFilling (Variables|Default|GetFountainAnimBP) true)
  (if (>= (Variables|Default|GetCurrentWater) (Variables|Default|GetMaxWater))
    (Components|Activation|Activate (Variables|Default|GetPoweredBurst) false)
    (CallFunction|GearsVolonInteract)
    (Variables|/Script/Engine.PostProcessVolume|SetbEnabled (Variables|Default|GetUnderwaterVolume) true)
    (Rendering|SetVisibility (Variables|/Script/Engine.DecalActor|GetDecal (Variables|Default|GetWaterCausticsDecal)) true false)
    (if (== (Variables|Default|GetCurrentStage) 3)
      (Class|FMODAudioComponent|Play (Variables|Default|GetFountainSound))
      (Utilities|FlowControl|Delay 1.0)
      (CallFunction|ActivateLayer (Variables|Default|GetLayer1Particles))
      (Utilities|FlowControl|Delay 1.0)
      (CallFunction|ActivateLayer (Variables|Default|GetLayer2Particles))
      (Utilities|FlowControl|Delay 1.0)
      (CallFunction|ActivateLayer (Variables|Default|GetLayer3Particles))
      (Utilities|FlowControl|Delay 1.0)
      (CallFunction|ActivateLayer (Variables|Default|GetTopLayerParticles)))
    (else
      (Variables|Default|SetCurrentWater (+ (Variables|Default|GetCurrentWater) (* (Utilities|Time|GetWorldDeltaSeconds) (Variables|Default|GetWaterIncreaseRate))))
      (Rendering|Material|SetScalarParameterValueonMaterials (Variables|Default|GetWater) "Blending" (/ (Variables|Default|GetCurrentWater) (Variables|Default|GetMaxWater)))
      (if (not (Variables|Default|GetbGearsPlaying))
        (Variables|Default|SetbGearsPlaying true)
        (Class|FMODAudioComponent|SetParameter _gears "Running" 0.0)
        (Class|FMODAudioComponent|Play _gears)))))

(fn ConstructionScript
  (Variables|Default|SetEmptyWaterMeshLevel (.z (Variables|/Script/Engine.SceneComponent|GetRelativeLocation (Variables|Default|GetWater)))))

(fn ActivateLayer
  (params (Layer :type Array%20of%20Niagara%20Component%20Object%20References))
  (for _array_element Layer
    (Components|Activation|Activate _array_element false)))

(fn GearsVolPowered
  (bind _gears (Variables|Default|GetGears))
  (Utilities|FlowControl|Sequence
    (:then_0
      (if (== (Variables|Default|GetCurrentStage) 1)
        (Class|FMODAudioComponent|SetParameter _gears "BigGearVol" 0.0)))
    (:then_1
      (if (== (Variables|Default|GetCurrentStage) 2)
        (Class|FMODAudioComponent|SetParameter _gears "MediumGearVol" 0.0)))
    (:then_2
      (if (== (Variables|Default|GetCurrentStage) 3)
        (Class|FMODAudioComponent|SetParameter _gears "SmallGearVol" 0.0)))))

(fn GearsVolonInteract
  (bind _gears (Variables|Default|GetGears))
  (Utilities|FlowControl|Sequence
    (:then_0
      (if (== (Variables|Default|GetCurrentStage) 0)
        (Class|FMODAudioComponent|SetParameter _gears "SmallGearVol" 0.0)
        (Class|FMODAudioComponent|SetParameter _gears "MediumGearVol" 0.0)
        (Class|FMODAudioComponent|SetParameter _gears "BigGearVol" 0.0)))
    (:then_1
      (if (== (Variables|Default|GetCurrentStage) 1)
        (Class|FMODAudioComponent|SetParameter _gears "SmallGearVol" 0.0)
        (Class|FMODAudioComponent|SetParameter _gears "MediumGearVol" 0.0)))
    (:then_2
      (if (== (Variables|Default|GetCurrentStage) 2)
        (Class|FMODAudioComponent|SetParameter _gears "SmallGearVol" 0.0)))))

(fn GearsVolonInteractEnd
  (bind _gears (Variables|Default|GetGears))
  (Utilities|FlowControl|Sequence
    (:then_0
      (if (== (Variables|Default|GetCurrentStage) 0)
        (Class|FMODAudioComponent|SetParameter _gears "SmallGearVol" 1.0)
        (Class|FMODAudioComponent|SetParameter _gears "MediumGearVol" 1.0)
        (Class|FMODAudioComponent|SetParameter _gears "BigGearVol" 1.0)))
    (:then_1
      (if (== (Variables|Default|GetCurrentStage) 1)
        (Class|FMODAudioComponent|SetParameter _gears "SmallGearVol" 1.0)
        (Class|FMODAudioComponent|SetParameter _gears "MediumGearVol" 1.0)))
    (:then_2
      (if (== (Variables|Default|GetCurrentStage) 2)
        (Class|FMODAudioComponent|SetParameter (Variables|Default|GetGears) "SmallGearVol" 1.0)))))

(fn MusicActivated
  (bind _asbp_game_mode (Utilities|Casting|CastToBP_GameMode (Game|GetGameMode)))
  (Utilities|FlowControl|Sequence
    (:then_0
      ;[0.1515 1 0] Main Track
      (Class|FMODBlueprintStatics|EventInstanceSetParameter (Variables|/Game/Blueprints/BP_GameMode.BP_GameMode_C|GetfmodMusicLoop _asbp_game_mode) "MainTrack" 1.0))
    (:then_1
      (Class|FMODBlueprintStatics|EventInstanceSetParameter (Variables|/Game/Blueprints/BP_GameMode.BP_GameMode_C|GetfmodMusicLoop _asbp_game_mode) "TrackA" 0.0))
    (:then_2
      (Class|FMODBlueprintStatics|EventInstanceSetParameter (Variables|/Game/Blueprints/BP_GameMode.BP_GameMode_C|GetfmodMusicLoop _asbp_game_mode) "TrackB" 1.0))
    (:then_3
      ;[1 0.9557 0] "Percussion"
      (Class|FMODBlueprintStatics|EventInstanceSetParameter (Variables|/Game/Blueprints/BP_GameMode.BP_GameMode_C|GetfmodMusicLoop _asbp_game_mode) "PianoMelody" 1.0))
    (:then_4
      (Class|FMODBlueprintStatics|EventInstanceSetParameter (Variables|/Game/Blueprints/BP_GameMode.BP_GameMode_C|GetfmodMusicLoop _asbp_game_mode) "PianoAccomp1" 1.0))
    (:then_5
      (Class|FMODBlueprintStatics|EventInstanceSetParameter (Variables|/Game/Blueprints/BP_GameMode.BP_GameMode_C|GetfmodMusicLoop _asbp_game_mode) "PianoAccomp2" 0.0))
    (:then_6
      (Class|FMODBlueprintStatics|EventInstanceSetParameter (Variables|/Game/Blueprints/BP_GameMode.BP_GameMode_C|GetfmodMusicLoop _asbp_game_mode) "Glockenspiel" 0.0))
    (:then_7
      ;[0.05353 0.01776 1] Strings
      (Class|FMODBlueprintStatics|EventInstanceSetParameter (Variables|/Game/Blueprints/BP_GameMode.BP_GameMode_C|GetfmodMusicLoop _asbp_game_mode) "Violin" 1.0))
    (:then_8
      (Class|FMODBlueprintStatics|EventInstanceSetParameter (Variables|/Game/Blueprints/BP_GameMode.BP_GameMode_C|GetfmodMusicLoop _asbp_game_mode) "Viola" 0.0))
    (:then_9
      (Class|FMODBlueprintStatics|EventInstanceSetParameter (Variables|/Game/Blueprints/BP_GameMode.BP_GameMode_C|GetfmodMusicLoop _asbp_game_mode) "Cello" 0.0))))

(fn MusicInactive
  (bind _asbp_game_mode (Utilities|Casting|CastToBP_GameMode (Game|GetGameMode)))
  (Utilities|FlowControl|Sequence
    (:then_0
      ;[0.1515 1 0] Main Track
      (Class|FMODBlueprintStatics|EventInstanceSetParameter (Variables|/Game/Blueprints/BP_GameMode.BP_GameMode_C|GetfmodMusicLoop _asbp_game_mode) "MainTrack" 1.0))
    (:then_1
      (Class|FMODBlueprintStatics|EventInstanceSetParameter (Variables|/Game/Blueprints/BP_GameMode.BP_GameMode_C|GetfmodMusicLoop _asbp_game_mode) "TrackA" 0.0))
    (:then_2
      (Class|FMODBlueprintStatics|EventInstanceSetParameter (Variables|/Game/Blueprints/BP_GameMode.BP_GameMode_C|GetfmodMusicLoop _asbp_game_mode) "TrackB" 1.0))
    (:then_3
      ;[1 0.9557 0] "Percussion"
      (Class|FMODBlueprintStatics|EventInstanceSetParameter (Variables|/Game/Blueprints/BP_GameMode.BP_GameMode_C|GetfmodMusicLoop _asbp_game_mode) "PianoMelody" 1.0))
    (:then_4
      (Class|FMODBlueprintStatics|EventInstanceSetParameter (Variables|/Game/Blueprints/BP_GameMode.BP_GameMode_C|GetfmodMusicLoop _asbp_game_mode) "PianoAccomp1" 0.0))
    (:then_5
      (Class|FMODBlueprintStatics|EventInstanceSetParameter (Variables|/Game/Blueprints/BP_GameMode.BP_GameMode_C|GetfmodMusicLoop _asbp_game_mode) "PianoAccomp2" 0.0))
    (:then_6
      (Class|FMODBlueprintStatics|EventInstanceSetParameter (Variables|/Game/Blueprints/BP_GameMode.BP_GameMode_C|GetfmodMusicLoop _asbp_game_mode) "Glockenspiel" 0.0))
    (:then_7
      ;[0.05353 0.01776 1] Strings
      (Class|FMODBlueprintStatics|EventInstanceSetParameter (Variables|/Game/Blueprints/BP_GameMode.BP_GameMode_C|GetfmodMusicLoop _asbp_game_mode) "Violin" 0.0))
    (:then_8
      (Class|FMODBlueprintStatics|EventInstanceSetParameter (Variables|/Game/Blueprints/BP_GameMode.BP_GameMode_C|GetfmodMusicLoop _asbp_game_mode) "Viola" 0.0))
    (:then_9
      (Class|FMODBlueprintStatics|EventInstanceSetParameter (Variables|/Game/Blueprints/BP_GameMode.BP_GameMode_C|GetfmodMusicLoop _asbp_game_mode) "Cello" 0.0))))