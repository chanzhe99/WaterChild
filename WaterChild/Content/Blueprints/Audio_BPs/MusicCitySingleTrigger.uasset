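; Music trigger actor that starts and stops the City audio as the player's controlled pawn crosses its overlap volumes.
; City1Enter plays the audio, while City1Exit and TempOff stop it, with an IsPlaying flag preventing repeat calls.
; Each change prints a debug string.
; TempOff's end overlap is empty and its "TEMP PLAY" resume logic is disconnected, so leaving that volume does not restart the music.
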(event OnComponentBeginOverlap(City1Enter)
  (params (OverlappedComponent :type Primitive%20Component%20Object%20Reference) (OtherActor :type Actor%20Object%20Reference) (OtherComp :type Primitive%20Component%20Object%20Reference) (OtherBodyIndex :type Integer) (bFromSweep :type Boolean) (SweepResult :type Hit%20Result%20Structure%20%28by%20ref%29))
  (if (== (Pawn|GetControlledPawn (Game|GetPlayerController 0)) OtherActor)
    (if (not (Variables|Default|GetbIsPlaying))
      (Development|PrintString "PLAY")
      (Class|FMODAudioComponent|Play (Variables|Default|GetCity))
      (Variables|Default|SetbIsPlaying true))))

(event OnComponentBeginOverlap(TempOff)
  (params (OverlappedComponent :type Primitive%20Component%20Object%20Reference) (OtherActor :type Actor%20Object%20Reference) (OtherComp :type Primitive%20Component%20Object%20Reference) (OtherBodyIndex :type Integer) (bFromSweep :type Boolean) (SweepResult :type Hit%20Result%20Structure%20%28by%20ref%29))
  (if (== OtherActor (Pawn|GetControlledPawn (Game|GetPlayerController 0)))
    (if (Variables|Default|GetbIsPlaying)
      (Development|PrintString "TEMP STOP")
      (Class|FMODAudioComponent|Stop (Variables|Default|GetCity))
      (Variables|Default|SetbIsPlaying false))))

(event OnComponentEndOverlap(TempOff)
  (params (OverlappedComponent :type Primitive%20Component%20Object%20Reference) (OtherActor :type Actor%20Object%20Reference) (OtherComp :type Primitive%20Component%20Object%20Reference) (OtherBodyIndex :type Integer)))

(event OnComponentBeginOverlap(City1Exit)
  (params (OverlappedComponent :type Primitive%20Component%20Object%20Reference) (OtherActor :type Actor%20Object%20Reference) (OtherComp :type Primitive%20Component%20Object%20Reference) (OtherBodyIndex :type Integer) (bFromSweep :type Boolean) (SweepResult :type Hit%20Result%20Structure%20%28by%20ref%29))
  (if (== OtherActor (Pawn|GetControlledPawn (Game|GetPlayerController 0)))
    (if (Variables|Default|GetbIsPlaying)
      (Development|PrintString "STOP")
      (Class|FMODAudioComponent|Stop (Variables|Default|GetCity))
      (Variables|Default|SetbIsPlaying false))))

(event EventBeginPlay)

(event Collision|EventActorBeginOverlap
  (params (OtherActor :type Actor%20Object%20Reference)))

(event EventTick
  (params (DeltaSeconds :type Float%20%28single-precision%29)))

(fn ConstructionScript)