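; CrackSpirit is a test actor that travels along the spline of a referenced Path, starting at BeginPlay when IsActive is set.
; The CrackMove timeline's play rate is scaled by Duration, and its track value sets the distance along the spline.
; Each update sets both location and rotation from that world-space spline point.
; Tick only prints the MoveForward input value for debugging, with an empty branch.
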(event Custom|Move
  (bind _path (Variables|Default|GetPath))
  (bind _spline (Variables|/Game/Blueprints/Tests/CrackPath.CrackPath_C|GetSpline _path))
  (Components|Timeline|SetPlayRate (Variables|Default|GetCrackMove) (/ 1.0 (Variables|Default|GetDuration)))
  (bind _newtrack_0 (Timeline|CrackMove Play)
    (:Update
      (Variables|Default|SetAlpha _newtrack_0)
      (Transformation|SetActorLocationAndRotation (Spline|GetLocationatDistanceAlongSpline _spline (Math|Float|Lerp 0.0 (Spline|GetSplineLength _spline) (Variables|Default|GetAlpha)) "World") (Spline|GetRotationatDistanceAlongSpline _spline (Math|Float|Lerp 0.0 (Spline|GetSplineLength _spline) (Variables|Default|GetAlpha)) "World")))))

(event EventBeginPlay
  (if (Variables|Default|GetIsActive)
    (CallFunction|Move)))

(event Collision|EventActorBeginOverlap
  (params (OtherActor :type Actor%20Object%20Reference)))

(event EventTick
  (params (DeltaSeconds :type Float%20%28single-precision%29))
  (bind _returnvalue (Input|AxisValues|GetMoveForward))
  (if (> _returnvalue 0.0)
    _
    (else
      _))
  (Development|PrintString (Utilities|String|ToString(Float) _returnvalue)))

(fn ConstructionScript)