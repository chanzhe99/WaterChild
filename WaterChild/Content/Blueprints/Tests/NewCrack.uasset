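; Test crack passage actor that lets the player travel in either direction between an Entrance and an Exit as a spirit pawn.
; On BeginPlay it hands its child CrackPath to its child spirit pawn.
; Hitting either end triggers that pawn forward or reverse, teleports the player's pawn to the opposite end, then possesses the spirit pawn.
; The teleport offset follows the endpoint's world-position vector, not its facing.
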(event OnComponentHit(Entrance)
  (params (HitComponent :type Primitive%20Component%20Object%20Reference) (OtherActor :type Actor%20Object%20Reference) (OtherComp :type Primitive%20Component%20Object%20Reference) (NormalImpulse :type Vector :default "0, 0, 0") (Hit :type Hit%20Result%20Structure%20%28by%20ref%29))
  (bind _returnvalue (Game|GetPlayerController 0))
  (bind _returnvalue_2 (Game|GetPlayerController 0))
  (bind _exit (Variables|Default|GetExit))
  (bind _returnvalue_3 (Pawn|GetControlledPawn _returnvalue))
  (bind _returnvalue_4 (Transformation|GetWorldLocation _exit))
  ;[1 1 1] Forward direction
  (if (== OtherActor _returnvalue_3)
    (Default|Triggered (Variables|Default|GetCrackPawn))
    (Transformation|SetActorLocation _returnvalue_3 (+ _returnvalue_4 (* (Math|Vector|GetForwardVector (Math|Conversions|RotationFromXVector _returnvalue_4)) (Variables|Default|GetExitOffset%28Exit%29))) false false)
    (Pawn|UnPossess _returnvalue_2)
    (Pawn|Possess _returnvalue_2 (Variables|Default|GetCrackPawn))))

(event OnComponentHit(Exit)
  (params (HitComponent :type Primitive%20Component%20Object%20Reference) (OtherActor :type Actor%20Object%20Reference) (OtherComp :type Primitive%20Component%20Object%20Reference) (NormalImpulse :type Vector :default "0, 0, 0") (Hit :type Hit%20Result%20Structure%20%28by%20ref%29))
  (bind _returnvalue (Game|GetPlayerController 0))
  (bind _returnvalue_2 (Game|GetPlayerController 0))
  (bind _entrance (Variables|Default|GetEntrance))
  (bind _returnvalue_3 (Transformation|GetWorldLocation _entrance))
  (bind _returnvalue_4 (Pawn|GetControlledPawn _returnvalue))
  ;[1 1 1] Reverse Direction
  (if (== OtherActor _returnvalue_4)
    (Default|TriggeredReverse (Variables|Default|GetCrackPawn))
    (Transformation|SetActorLocation _returnvalue_4 (+ _returnvalue_3 (* (Math|Vector|GetForwardVector (Math|Conversions|RotationFromXVector _returnvalue_3)) (Variables|Default|GetExitOffset%28Entrance%29))) false false)
    (Pawn|UnPossess _returnvalue_2)
    (Pawn|Possess _returnvalue_2 (Variables|Default|GetCrackPawn))))

(event EventBeginPlay
  ;[1 1 1] Setup
  (bind _ascrack_spirit_pawn (Utilities|Casting|CastToCrack_Spirit_Pawn (Variables|/Script/Engine.ChildActorComponent|GetChildActor (Variables|Default|GetCrack_Spirit_Pawn1))))
  (bind _ascrack_path (Utilities|Casting|CastToCrackPath (Variables|/Script/Engine.ChildActorComponent|GetChildActor (Variables|Default|GetCrackPath))))
  (Variables|/Game/Blueprints/Tests/Crack_Spirit_Pawn.Crack_Spirit_Pawn_C|SetPath _ascrack_spirit_pawn _ascrack_path)
  (Variables|Default|SetCrackPawn _ascrack_spirit_pawn))

(event EventTick
  (params (DeltaSeconds :type Float%20%28single-precision%29))
  ;[1 1 1] Forward direction
)

(fn ConstructionScript)