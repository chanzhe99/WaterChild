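; CutsceneTrigger is a trigger-box Blueprint that plays an end cutscene and then shows the UI_End screen.
; When the controlled pawn overlaps, it creates a sequence player, disables input, blends to CutsceneCamera, plays the sequence and, after a fixed delay, opens the widget with UI-only mouse input.
; Any overlap first moves the trigger actor to a hard-coded transform.
; The IsTriggered guard is only set in unconnected nodes, alongside input re-enabling.
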(event OnComponentBeginOverlap(TriggerBox)
  (params (OverlappedComponent :type Primitive%20Component%20Object%20Reference) (OtherActor :type Actor%20Object%20Reference) (OtherComp :type Primitive%20Component%20Object%20Reference) (OtherBodyIndex :type Integer) (bFromSweep :type Boolean) (SweepResult :type Hit%20Result%20Structure%20%28by%20ref%29))
  (bind _returnvalue (Game|GetPlayerController 0))
  (bind _returnvalue_2 (Game|GetPlayerController 0))
  (Transformation|SetActorLocationAndRotation "-4350.085938,14002.815430,3069.000000" "0,-115.000000, 0")
  (if (== OtherActor (Pawn|GetControlledPawn (Game|GetPlayerController 0)))
    (if (not (Variables|Default|GetIsTriggered))
      (Utilities|FlowControl|Sequence
        (:then_0
          (bind _returnvalue_3 (Sequencer|Player|CreateLevelSequencePlayer (Variables|Default|GetLevel_Sequence)))
          (Variables|Default|SetSequencePlayer _returnvalue_3))
        (:then_1
          (Input|DisableInput (Game|GetPlayerCharacter 0) _returnvalue)
          (Game|Player|SetViewTargetwithBlend _returnvalue (Variables|Default|GetCutsceneCamera) 3.0 "VTBlend_Cubic" 0.0 false)
          (Utilities|FlowControl|Delay 2.5)
          (Sequencer|Player|Play (Variables|Default|GetSequencePlayer) :!class /Script/MovieScene.MovieSceneSequencePlayer)
          (Utilities|FlowControl|Delay 15.0)
          (bind _returnvalue_4 (UserInterface|CreateWidget "/Game/Blueprints/UI/UI_End.UI_End_C"))
          (UserInterface|Viewport|AddtoViewport _returnvalue_4 0)
          (Input|SetInputModeUIOnly _returnvalue_2 0 "DoNotLock")
          (Variables|/Script/Engine.PlayerController|SetbShowMouseCursor _returnvalue_2 true))))))

(fn ConstructionScript)