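; Camera trigger volume that blends the player's view to another camera when the player enters its box, disabling input.
; It returns to the saved original view after a timer, which restores input, or on exit when not time-based.
; Tick is enabled only during swaps and repeatedly calls SetViewTargetWithBlend according to swap/return flags.
; End overlap re-arms the trigger unless it is one-use.
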(event OnComponentBeginOverlap(Box)
  (params (OverlappedComponent :type Primitive%20Component%20Object%20Reference) (OtherActor :type Actor%20Object%20Reference) (OtherComp :type Primitive%20Component%20Object%20Reference) (OtherBodyIndex :type Integer) (bFromSweep :type Boolean) (SweepResult :type Hit%20Result%20Structure%20%28by%20ref%29))
  (bind _returnvalue (Game|GetPlayerController 0))
  ;[1 1 1] Check if actor is player
  (if (== _returnvalue (Components|GetOwner OtherActor))
    ;[1 1 1] Mark as used
    (if (stale _output_get)
      (bind _output_get (Variables|Default|SetNotTriggered false))
      ;[1 1 1] don't run if already running
      (if (not (stale _output_get_2))
        (bind _output_get_2 (Variables|Default|SetIsRunning true))
        ;[1 1 1] Remember Original Camera
        (Variables|Default|SetOriginalCam (Pawn|GetViewTarget _returnvalue))
        (Input|DisableInput _returnvalue _returnvalue)
        ;[1 1 1] Tick related
        (Actor|Tick|SetActorTickEnabled true)
        ;[1 1 1] Start swap
        (Variables|Default|SetSwapCam true)
        ;[1 1 1] Timer based swap
        (if (Variables|Default|GetTimeBased)
          (Utilities|FlowControl|Delay (Variables|Default|GetTimer))
          (Input|EnableInput _returnvalue _returnvalue)
          ;[1 1 1] Return to player cam
          (Variables|Default|SetSwapCam false)
          (Variables|Default|SetReturnCam true)
          ;[1 1 1] Tick related
          (Utilities|FlowControl|Delay (Variables|Default|GetCameraSwapTime))
          (Actor|Tick|SetActorTickEnabled false)
          (Variables|Default|SetIsRunning false))))))

(event OnComponentEndOverlap(Box)
  (params (OverlappedComponent :type Primitive%20Component%20Object%20Reference) (OtherActor :type Actor%20Object%20Reference) (OtherComp :type Primitive%20Component%20Object%20Reference) (OtherBodyIndex :type Integer))
  ;[1 1 1] Check if system is one shot or repeatable
  (if (Variables|Default|GetOneUse)
    _
    (else
      (Variables|Default|SetNotTriggered true)))
  ;[1 1 1] check if its not time based
  (if (and (not (Variables|Default|GetTimeBased)) (== (Game|GetPlayerController 0) (Components|GetOwner OtherActor)))
    ;[1 1 1] Return to player cam
    (Variables|Default|SetSwapCam false)
    (Variables|Default|SetReturnCam true)
    ;[1 1 1] Tick related
    (Utilities|FlowControl|Delay (Variables|Default|GetCameraSwapTime))
    (Actor|Tick|SetActorTickEnabled false)
    (Variables|Default|SetIsRunning false)))

(event EventBeginPlay
  ;[1 1 1] Disable tick for optimization
  (Actor|Tick|SetActorTickEnabled false))

(event EventTick
  (params (DeltaSeconds :type Float%20%28single-precision%29))
  (if (Variables|Default|GetSwapCam)
    (Game|Player|SetViewTargetwithBlend (Game|GetPlayerController 0) (Components|GetOwner (Variables|Default|GetCamera)) (Variables|Default|GetCameraSwapTime) (Variables|Default|GetBlending%20type) (Variables|Default|GetCameraSwapCurve) false)
    (elif (Variables|Default|GetReturnCam)
      (Game|Player|SetViewTargetwithBlend (Game|GetPlayerController 0) (Variables|Default|GetOriginalCam) (Variables|Default|GetCameraSwapTime) (Variables|Default|GetBlending%20type) (Variables|Default|GetCameraSwapCurve) false))))

(fn ConstructionScript)