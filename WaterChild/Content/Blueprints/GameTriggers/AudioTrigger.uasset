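; AudioTrigger is a trigger Blueprint that changes the music when the player enters it.
; On actor overlap it checks that the other actor is player 0's controlled pawn, then casts the game mode to BP_GameMode.
; It sets the TrackA parameter to zero on the FMOD music loop event instance held by that game mode.
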(event EventBeginPlay)

(event Collision|EventActorBeginOverlap
  (params (OtherActor :type Actor%20Object%20Reference))
  (if (== OtherActor (Pawn|GetControlledPawn (Game|GetPlayerController 0)))
    (bind _asbp_game_mode (Utilities|Casting|CastToBP_GameMode (Game|GetGameMode)))
    (Class|FMODBlueprintStatics|EventInstanceSetParameter (Variables|/Game/Blueprints/BP_GameMode.BP_GameMode_C|GetfmodMusicLoop _asbp_game_mode) "TrackA" 0.0)))

(event EventTick
  (params (DeltaSeconds :type Float%20%28single-precision%29)))

(fn ConstructionScript)