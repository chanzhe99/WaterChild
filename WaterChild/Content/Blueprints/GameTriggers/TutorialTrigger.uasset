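; Trigger volume that shows a tutorial button prompt on BP_Spirit's UI on overlap, hiding it on exit and optionally firing only once.
; Gamepad and keyboard textures are configurable and preview on billboards via the construction script.
; With a linked TutorialPlant, Tick watches for it becoming Alive, then swaps the player's prompt to the X button/Space prompt, which later overlaps also show.
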(event EventBeginPlay)

(event Collision|EventActorBeginOverlap
  (params (OtherActor :type Actor%20Object%20Reference))
  (if (not (Variables|Default|GetTriggered))
    (bind _asbp_spirit (Utilities|Casting|CastToBP_Spirit OtherActor))
    (Default|FadeinTutorialUI _asbp_spirit (Variables|Default|GetGamepadTexture) (Variables|Default|GetKeyboardTexture))
    (Utilities|IsValid (Variables|Default|GetTutorialPlant)
      (:Is%20Valid
        (if (Variables|Default|GetTutorialSwitched)
          (Default|FadeinTutorialUI _asbp_spirit "/Game/Blueprints/UI/MatUI/tutorial/Controller_Xbutton.Controller_Xbutton" "/Game/Blueprints/UI/MatUI/tutorial/keyboard_SPACE.keyboard_SPACE"))))))

(event EventTick
  (params (DeltaSeconds :type Float%20%28single-precision%29))
  (bind _tutorialplant (Variables|Default|GetTutorialPlant))
  (Utilities|IsValid _tutorialplant
    (:Is%20Valid
      (if (not (Variables|Default|GetTutorialSwitched))
        (if (Utilities|Enum|Equal(Enum) "Alive" (Variables|/Script/WaterChild.Plant|GetPlantState _tutorialplant))
          (Variables|Default|SetTutorialSwitched true)
          (bind _asbp_spirit (Utilities|Casting|CastToBP_Spirit (Game|GetPlayerCharacter 0)))
          (Default|FadeOutTutorialUI _asbp_spirit)
          (Utilities|FlowControl|Delay 0.5)
          (Default|FadeinTutorialUI _asbp_spirit "/Game/Blueprints/UI/MatUI/tutorial/Controller_Xbutton.Controller_Xbutton" "/Game/Blueprints/UI/MatUI/tutorial/keyboard_SPACE.keyboard_SPACE"))))))

(event Collision|EventActorEndOverlap
  (params (OtherActor :type Actor%20Object%20Reference))
  (if (not (Variables|Default|GetTriggered))
    (bind _asbp_spirit (Utilities|Casting|CastToBP_Spirit OtherActor))
    (Default|FadeOutTutorialUI _asbp_spirit)
    (if (Variables|Default|GetTriggersOnce)
      (Variables|Default|SetTriggered true))))

(fn ConstructionScript
  (bind _keyboardtexture (Variables|Default|GetKeyboardTexture))
  (bind _gamepadtexture (Variables|Default|GetGamepadTexture))
  (Utilities|FlowControl|Sequence
    (:then_0
      (Utilities|IsValid _gamepadtexture
        (:Is%20Valid
          (Variables|/Script/Engine.BillboardComponent|SetSprite (Variables|Default|GetGamepadBillboard) _gamepadtexture))))
    (:then_1
      (Utilities|IsValid _keyboardtexture
        (:Is%20Valid
          (Variables|/Script/Engine.BillboardComponent|SetSprite (Variables|Default|GetKeyboardBillboard) _keyboardtexture))))))