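; Trigger actor that changes which layers of the adaptive FMOD music loop play when the player's pawn overlaps it.
; On overlap, it gets the FmodMusicLoop event instance from BP_GameMode.
; A sequence then sets each main, piano, glockenspiel and string track parameter to 1 or 0 from the trigger's matching booleans.
; A PianoAccomp2 branch exists but is unconnected, so it never runs.
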(event EventBeginPlay)

(event Collision|EventActorBeginOverlap
  (params (OtherActor :type Actor%20Object%20Reference))
  (if (== OtherActor (Pawn|GetControlledPawn (Game|GetPlayerController 0)))
    (bind _asbp_game_mode (Utilities|Casting|CastToBP_GameMode (Game|GetGameMode)))
    (Utilities|FlowControl|Sequence
      (:then_0
        ;[0.1515 1 0] Main Track
        (if (Variables|Default|GetbMainTrack)
          (Class|FMODBlueprintStatics|EventInstanceSetParameter (Variables|/Game/Blueprints/BP_GameMode.BP_GameMode_C|GetfmodMusicLoop _asbp_game_mode) "MainTrack" 1.0)
          (else
            (Class|FMODBlueprintStatics|EventInstanceSetParameter (Variables|/Game/Blueprints/BP_GameMode.BP_GameMode_C|GetfmodMusicLoop _asbp_game_mode) "MainTrack" 0.0))))
      (:then_1
        (if (Variables|Default|GetbTrackA)
          (Class|FMODBlueprintStatics|EventInstanceSetParameter (Variables|/Game/Blueprints/BP_GameMode.BP_GameMode_C|GetfmodMusicLoop _asbp_game_mode) "TrackA" 1.0)
          (else
            (Class|FMODBlueprintStatics|EventInstanceSetParameter (Variables|/Game/Blueprints/BP_GameMode.BP_GameMode_C|GetfmodMusicLoop _asbp_game_mode) "TrackA" 0.0))))
      (:then_2
        (if (Variables|Default|GetbTrackB)
          (Class|FMODBlueprintStatics|EventInstanceSetParameter (Variables|/Game/Blueprints/BP_GameMode.BP_GameMode_C|GetfmodMusicLoop _asbp_game_mode) "TrackB" 1.0)
          (else
            (Class|FMODBlueprintStatics|EventInstanceSetParameter (Variables|/Game/Blueprints/BP_GameMode.BP_GameMode_C|GetfmodMusicLoop _asbp_game_mode) "TrackB" 0.0))))
      (:then_3
        ;[1 0.9557 0] "Percussion"
        (if (Variables|Default|GetbPianoMelody)
          (Class|FMODBlueprintStatics|EventInstanceSetParameter (Variables|/Game/Blueprints/BP_GameMode.BP_GameMode_C|GetfmodMusicLoop _asbp_game_mode) "PianoMelody" 1.0)
          (else
            (Class|FMODBlueprintStatics|EventInstanceSetParameter (Variables|/Game/Blueprints/BP_GameMode.BP_GameMode_C|GetfmodMusicLoop _asbp_game_mode) "PianoMelody" 0.0))))
      (:then_4
        (if (Variables|Default|GetbPianoAccomp1)
          (Class|FMODBlueprintStatics|EventInstanceSetParameter (Variables|/Game/Blueprints/BP_GameMode.BP_GameMode_C|GetfmodMusicLoop _asbp_game_mode) "PianoAccomp1" 1.0)
          (else
            (Class|FMODBlueprintStatics|EventInstanceSetParameter (Variables|/Game/Blueprints/BP_GameMode.BP_GameMode_C|GetfmodMusicLoop _asbp_game_mode) "PianoAccomp1" 0.0))))
      (:then_5
        (if (Variables|Default|GetbGlockenspiel)
          (Class|FMODBlueprintStatics|EventInstanceSetParameter (Variables|/Game/Blueprints/BP_GameMode.BP_GameMode_C|GetfmodMusicLoop _asbp_game_mode) "Glockenspiel" 1.0)
          (else
            (Class|FMODBlueprintStatics|EventInstanceSetParameter (Variables|/Game/Blueprints/BP_GameMode.BP_GameMode_C|GetfmodMusicLoop _asbp_game_mode) "Glockenspiel" 0.0))))
      (:then_6
        ;[0.05353 0.01776 1] Strings
        (if (Variables|Default|GetbViolin)
          (Class|FMODBlueprintStatics|EventInstanceSetParameter (Variables|/Game/Blueprints/BP_GameMode.BP_GameMode_C|GetfmodMusicLoop _asbp_game_mode) "Violin" 1.0)
          (else
            (Class|FMODBlueprintStatics|EventInstanceSetParameter (Variables|/Game/Blueprints/BP_GameMode.BP_GameMode_C|GetfmodMusicLoop _asbp_game_mode) "Violin" 0.0))))
      (:then_7
        (if (Variables|Default|GetbViola)
          (Class|FMODBlueprintStatics|EventInstanceSetParameter (Variables|/Game/Blueprints/BP_GameMode.BP_GameMode_C|GetfmodMusicLoop _asbp_game_mode) "Viola" 1.0)
          (else
            (Class|FMODBlueprintStatics|EventInstanceSetParameter (Variables|/Game/Blueprints/BP_GameMode.BP_GameMode_C|GetfmodMusicLoop _asbp_game_mode) "Viola" 0.0))))
      (:then_8
        (if (Variables|Default|GetbCello)
          (Class|FMODBlueprintStatics|EventInstanceSetParameter (Variables|/Game/Blueprints/BP_GameMode.BP_GameMode_C|GetfmodMusicLoop _asbp_game_mode) "Cello" 1.0)
          (else
            (Class|FMODBlueprintStatics|EventInstanceSetParameter (Variables|/Game/Blueprints/BP_GameMode.BP_GameMode_C|GetfmodMusicLoop _asbp_game_mode) "Cello" 0.0)))))))

(event EventTick
  (params (DeltaSeconds :type Float%20%28single-precision%29)))

(fn ConstructionScript)