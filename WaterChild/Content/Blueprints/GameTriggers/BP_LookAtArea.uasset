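; One-shot trigger area that offers the Spirit player a "look at" tutorial prompt while inside it.
; Tick box-traces the AreaVisualiser extent for the player, then registers the area as the ExternalCamera's CurrentLookAtBP and fades in the TutorialUI prompt.
; Leaving fades the prompt out, clearing that reference when the animation finishes.
; PressedLookAtPrompt plays the press animation, clears the reference and permanently disables the area.
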(event Custom|PressedLookAtPrompt
  (if (not (Variables|Default|GetHasBeenTriggered))
    (Utilities|PressLookatPromptAnim
      (:then
        (Variables|Default|SetHasBeenTriggered true)
        (Variables|/Game/Blueprints/ExternalCamera.ExternalCamera_C|SetCurrentLookAtBP (Variables|/Game/Blueprints/BP_Spirit.BP_Spirit_C|GetExternalCamera (Variables|Default|GetSpiritRef)) 0)))))

(event EventBeginPlay)

(event Collision|EventActorBeginOverlap
  (params (OtherActor :type Actor%20Object%20Reference)))

(event EventTick
  (params (DeltaSeconds :type Float%20%28single-precision%29))
  (bind _returnvalue (Transformation|GetActorLocation))
  (bind (_outhit _returnvalue_2) (Class|KismetSystemLibrary|BoxTraceSingleforObjects _returnvalue _returnvalue (Components|Box|GetScaledBoxExtent (Variables|Default|GetAreaVisualiser)) "0, 0, 0" (Variables|Default|GetPlayerObjType) false 0 "ForOneFrame" true))
  (if _returnvalue_2
    (if (not (Variables|Default|GetHasBeenTriggered))
      (Variables|Default|SetHitResult _outhit)
      (Utilities|IsValid (Variables|Default|GetSpiritRef)
        (:Is%20Valid
          _)
        (:Is%20Not%20Valid
          (bind _asbp_spirit (Utilities|Casting|CastToBP_Spirit (.HitActor (Collision|BreakHitResult (Variables|Default|GetHitResult)))))
          (bind _output_get (Variables|Default|SetSpiritRef _asbp_spirit))))
      (Utilities|IsValid (Variables|/Game/Blueprints/BP_Spirit.BP_Spirit_C|GetExternalCamera _output_get)
        (:Is%20Valid
          (Variables|/Game/Blueprints/ExternalCamera.ExternalCamera_C|SetCurrentLookAtBP (Variables|/Game/Blueprints/BP_Spirit.BP_Spirit_C|GetExternalCamera _output_get) self)
          (Utilities|FadeinLookatPrompt))))
    (elif (not (Variables|Default|GetHasBeenTriggered))
      (Utilities|FadeOutLookatPrompt
        (:Finished
          (Variables|/Game/Blueprints/ExternalCamera.ExternalCamera_C|SetCurrentLookAtBP (Variables|/Game/Blueprints/BP_Spirit.BP_Spirit_C|GetExternalCamera (Variables|Default|GetSpiritRef)) 0))))))

(fn ConstructionScript)