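; Trigger actor that starts the end-of-game warning when the player's pawn overlaps it.
; On overlap it shows the UI_EndWarning widget, switches to UI-only input and reveals the mouse cursor.
; It also passes its Arrow component's rotation to BP_Spirit as WalkBackRotation and sets the GlobalMusic parameter to a lower value.
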(event EventBeginPlay)

(event Collision|EventActorBeginOverlap
  (params (OtherActor :type Actor%20Object%20Reference))
  (bind _returnvalue (Game|GetPlayerController 0))
  (if (== OtherActor (Pawn|GetControlledPawn (Game|GetPlayerController 0)))
    (bind _returnvalue_2 (UserInterface|CreateWidget "/Game/Blueprints/UI/UI_EndWarning.UI_EndWarning_C"))
    (UserInterface|Viewport|AddtoViewport _returnvalue_2 0)
    (Input|SetInputModeUIOnly _returnvalue 0 "DoNotLock")
    (Variables|/Script/Engine.PlayerController|SetbShowMouseCursor _returnvalue true)
    (bind _asbp_spirit (Utilities|Casting|CastToBP_Spirit (Game|GetPlayerCharacter 0)))
    (Variables|/Game/Blueprints/BP_Spirit.BP_Spirit_C|SetWalkBackRotation _asbp_spirit (Transformation|GetWorldRotation (Variables|Default|GetArrow)))
    (Class|FMODBlueprintStatics|SetGlobalParameterbyName "GlobalMusic" 0.2)))

(event EventTick
  (params (DeltaSeconds :type Float%20%28single-precision%29)))

(fn ConstructionScript)