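; Start-screen camera actor that holds the opening view, then hands it back to the player's camera when the game starts.
; CallStart saves the original view target and switches to this camera.
; GameStart locks Spirit input and enables Tick to drive a timed blend back, which is instant when the GameMode is debugging.
; After the blend delay, Tick stops, the movement tutorial UI fades in, and input and pausing are enabled.
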(event OnClicked(StartButton)
  ;[1 1 1] Button Input
)

(event Custom|GameStart
  (params (SpiritControllerRef :type BP%20Spirit%20Controller%20Object%20Reference))
  (bind _returnvalue (Game|GetPlayerController 0))
  ;[1 1 1] Button Input
  (bind _asbp_spirit (Utilities|Casting|CastToBP_Spirit (Pawn|GetControlledPawn _returnvalue)))
  (Class|Spirit|SetCanTakeInput _asbp_spirit false)
  (Actor|Tick|SetActorTickEnabled true)
  (Variables|Default|SetPlayPressed true)
  (Input|SetInputModeGameOnly _returnvalue)
  (Variables|/Script/Engine.PlayerController|SetbShowMouseCursor _returnvalue false)
  (Utilities|FlowControl|Delay (select (Variables|Default|GetGM_IsDebugging) 0.0 (Variables|Default|GetCameraSwapTime)))
  (Actor|Tick|SetActorTickEnabled false)
  (bind _asbp_spirit_2 (Utilities|FadeinTutorialUI "/Game/Blueprints/UI/MatUI/tutorial/Controller_RightAnalog.Controller_RightAnalog" "/Game/Blueprints/UI/MatUI/tutorial/Mouse_Move.Mouse_Move")
    (:then
      (Class|Spirit|SetCanTakeInput _asbp_spirit_2 true)
      (Variables|/Game/Blueprints/BP_SpiritController.BP_SpiritController_C|SetCanPauseGame SpiritControllerRef true))))

(event Custom|Call%20Start
  (bind _returnvalue (Game|GetPlayerController 0))
  ;[1 1 1] Change Port and remember player cam
  (Variables|Default|SetOriginalCam (Pawn|GetViewTarget _returnvalue))
  (Game|Player|SetViewTargetwithBlend _returnvalue (Components|GetOwner (Variables|Default|GetCamera)) 0.0 "VTBlend_Linear" 0.0 false)
  (Actor|Tick|SetActorTickEnabled false)
  (bind _asbp_game_mode (Utilities|Casting|CastToBP_GameMode (Game|GetGameMode)))
  (Variables|Default|SetGM_IsDebugging (Variables|/Game/Blueprints/BP_GameMode.BP_GameMode_C|GetIsDebugging _asbp_game_mode)))

(event EventTick
  (params (DeltaSeconds :type Float%20%28single-precision%29))
  ;[1 1 1] Change Camera, tick is disabled after
  (if (Variables|Default|GetPlayPressed)
    (Game|Player|SetViewTargetwithBlend (Game|GetPlayerController 0) (Variables|Default|GetOriginalCam) (select (Variables|Default|GetGM_IsDebugging) 0.0 (Variables|Default|GetCameraSwapTime)) (Variables|Default|GetBlendingType) (Variables|Default|GetCameraSwapCurve) false)))

(fn ConstructionScript)