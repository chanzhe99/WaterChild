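; BP_GameEndTrigger is a box trigger that shows a game-end warning when the player reaches it.
; Each Tick it box-traces the BoxTrigger volume for the controlled pawn, with an IsColliding latch so it fires once per entry.
; On entry it opens UI_GameEndWarning with Game-and-UI input, freezes BP_Spirit, passes it the Arrow's rotation as WalkBackRotation and sets the GlobalMusic parameter to zero.
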(event EventBeginPlay)

(event Collision|EventActorBeginOverlap
  (params (OtherActor :type Actor%20Object%20Reference)))

(event EventTick
  (params (DeltaSeconds :type Float%20%28single-precision%29))
  (bind _returnvalue (Game|GetPlayerController 0))
  (bind _boxtrigger (Variables|Default|GetBoxTrigger))
  (bind _returnvalue_2 (Transformation|GetWorldLocation _boxtrigger))
  (bind (_outhit _returnvalue_3) (Class|KismetSystemLibrary|BoxTraceSingleforObjects _returnvalue_2 (+ _returnvalue_2 "0, 0,0.000010") (Components|Box|GetScaledBoxExtent _boxtrigger) (Transformation|GetWorldRotation _boxtrigger) (Variables|Default|GetPlayer%20Object%20Type) false 0 "None" true)) ; City1Enter
  (if (and _returnvalue_3 (== (.HitActor (Collision|BreakHitResult _outhit)) (Pawn|GetControlledPawn _returnvalue)))
    (if (not (Variables|Default|GetIsColliding))
      (Variables|Default|SetIsColliding true)
      (bind _returnvalue_4 (UserInterface|CreateWidget "/Game/Blueprints/UI/UI_GameEndWarning.UI_GameEndWarning_C" _returnvalue))
      (UserInterface|Viewport|AddtoViewport _returnvalue_4 0)
      (Input|SetInputModeGameandUI (Game|GetPlayerController 0) _returnvalue_4 "DoNotLock" true)
      (bind _asbp_spirit (Utilities|Casting|CastToBP_Spirit (Game|GetPlayerCharacter 0)))
      (Class|Spirit|SetState _asbp_spirit "StuckInPlace")
      (Class|Spirit|SetCanTakeInput _asbp_spirit false)
      (Variables|/Game/Blueprints/BP_Spirit.BP_Spirit_C|SetWalkBackRotation _asbp_spirit (Transformation|GetWorldRotation (Variables|Default|GetArrow)))
      (Class|FMODBlueprintStatics|SetGlobalParameterbyName "GlobalMusic" 0.0))
    (elif (Variables|Default|GetIsColliding)
      (Variables|Default|SetIsColliding false))))

(fn ConstructionScript)