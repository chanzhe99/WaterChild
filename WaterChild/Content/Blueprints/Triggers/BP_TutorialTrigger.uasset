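; Tutorial trigger volume that fades gamepad and keyboard control prompts in and out on BP_Spirit's TutorialUI.
; Tick box-traces the visualiser bounds to derive begin, tick and end overlap events, rather than using collision overlaps.
; Prompts can time out or trigger only once, disabling tick afterwards.
; If a linked TutorialPlant is alive during overlap, the prompt switches once to the X button/Space textures, which later entries reuse.
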(event Custom|BeginOverlap
  (if (not (Variables|TriggerConditions|GetIsActive))
    (Variables|TriggerConditions|SetIsActive true)
    (Utilities|IsValid (Variables|TriggerConditions|GetTutorialPlant)
      (:Is%20Valid
        (if (Variables|TriggerConditions|GetTutorialSwitched)
          (Utilities|FadeinTutorialUI "/Game/Blueprints/UI/MatUI/tutorial/Controller_Xbutton.Controller_Xbutton" "/Game/Blueprints/UI/MatUI/tutorial/keyboard_SPACE.keyboard_SPACE")
          (else
            (Utilities|FadeinTutorialUI (Variables|Default|GetGamepadTexture) (Variables|Default|GetKeyboardTexture) :!label _label))))
      (:Is%20Not%20Valid
        (goto _label)))))

(event Custom|TickOverlap
  (Utilities|FlowControl|Sequence
    (:then_0
      (if (and (Variables|TriggerConditions|GetFadesOverTime) (Variables|TriggerConditions|GetIsActive))
        (if (< (Variables|Default|GetFadeOutTime_Tick) (Variables|Default|GetFadeOutTime))
          (Variables|Default|SetFadeOutTime_Tick (+ (Variables|Default|GetFadeOutTime_Tick) (Utilities|Time|GetWorldDeltaSeconds)))
          (else
            (Utilities|FadeOutTutorialUI
              (:Finished
                (Variables|TriggerConditions|SetIsActive false)
                (Actor|Tick|SetActorTickEnabled false)))))))
    (:then_1
      (Utilities|CheckPlantandSwitchUI)
      (Utilities|FadeOutTutorialUI
        (:Finished
          (Utilities|FadeinTutorialUI "/Game/Blueprints/UI/MatUI/tutorial/Controller_Xbutton.Controller_Xbutton" "/Game/Blueprints/UI/MatUI/tutorial/keyboard_SPACE.keyboard_SPACE"))))))

(event Custom|EndOverlap
  (if (Variables|TriggerConditions|GetIsActive)
    (Utilities|FadeOutTutorialUI
      (:then
        (if (Variables|TriggerConditions|GetTriggersOnlyOnce)
          (Actor|Tick|SetActorTickEnabled false)))
      (:Finished
        (Variables|TriggerConditions|SetIsActive false)))))

(event EventTick
  (params (DeltaSeconds :type Float%20%28single-precision%29))
  (bind _triggervisualiser (Variables|Default|GetTriggerVisualiser))
  (bind _returnvalue (Transformation|GetWorldLocation _triggervisualiser))
  (if (Variables|TriggerConditions|GetStartWithOverlapEnabled)
    (bind (_outhit _returnvalue_2) (Class|KismetSystemLibrary|BoxTraceSingleforObjects _returnvalue _returnvalue (Components|Box|GetScaledBoxExtent _triggervisualiser) (Transformation|GetWorldRotation _triggervisualiser) (Variables|CollisionDetection|GetPlayerObj) false 0 "ForOneFrame" true))
    (if _returnvalue_2
      (Utilities|IsValid (Variables|CollisionDetection|GetSpiritRef)
        (:Is%20Valid
          _)
        (:Is%20Not%20Valid
          (bind _asbp_spirit (Utilities|Casting|CastToBP_Spirit (.HitActor (Collision|BreakHitResult _outhit))))
          (Variables|CollisionDetection|SetSpiritRef _asbp_spirit)))
      (if (Variables|CollisionDetection|GetIsOverlapping)
        _
        (else
          (Variables|CollisionDetection|SetIsOverlapping true)
          (CallFunction|BeginOverlap)))
      (CallFunction|TickOverlap)
      (else
        (Utilities|IsValid (Variables|CollisionDetection|GetSpiritRef)
          (:Is%20Valid
            (if (Variables|CollisionDetection|GetIsOverlapping)
              (Variables|CollisionDetection|SetIsOverlapping false)
              (CallFunction|EndOverlap))))))))

(fn ConstructionScript
  (bind _keyboardtexture (Variables|Default|GetKeyboardTexture))
  (bind _gamepadtexture (Variables|Default|GetGamepadTexture))
  (Utilities|FlowControl|Sequence
    (:then_0
      (if (Variables|TriggerConditions|GetFadesOverTime)
        (Variables|TriggerConditions|SetTriggersOnlyOnce true)))
    (:then_1
      (Utilities|IsValid _gamepadtexture
        (:Is%20Valid
          (Variables|/Script/Engine.BillboardComponent|SetSprite (Variables|Default|GetGamepadBillboard) _gamepadtexture))))
    (:then_2
      (Utilities|IsValid _keyboardtexture
        (:Is%20Valid
          (Variables|/Script/Engine.BillboardComponent|SetSprite (Variables|Default|GetKeyboardBillboard) _keyboardtexture))))))