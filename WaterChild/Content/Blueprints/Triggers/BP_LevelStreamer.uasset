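; Level streaming trigger volume that loads and unloads the game's sublevels as the BP_Spirit player enters and leaves.
; Tick box-traces the visualiser's bounds, caching the spirit and firing begin/end overlap events on state changes.
; Those events re-call themselves to step through parallel flag and level-name arrays, asynchronously loading or unloading flagged levels, gated by DoLoad and DoUnload.
; A pass halts early when a flagged level is already in the target state.
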(event Custom|BeginOverlap
  (Utilities|LoopLoadLevels
    (:true
      (CallFunction|BeginOverlap))
    (:finishedLooping
      (Variables|Default|SetCurrentPendingLoad 0))))

(event Custom|TickOverlap)

(event Custom|EndOverlap
  (Utilities|LoopUnloadLevels
    (:true
      (CallFunction|EndOverlap))
    (:finishedLooping
      (Variables|Default|SetCurrentPendingLoad 0))))

(event EventBeginPlay
  (Variables|BoolLoadLevel|SetLoad_LVList (Utilities|MakeBoolLoadArray))
  (Variables|LevelNames|SetLevelNameList (Utilities|MakeLevelNamesArray))
  (Variables|Default|SetTotalPendingLoad (Utilities|Array|Length (Variables|BoolLoadLevel|GetLoad_LVList))))

(event EventTick
  (params (DeltaSeconds :type Float%20%28single-precision%29))
  (bind _triggervisualiser (Variables|Default|GetTriggerVisualiser))
  (bind _returnvalue (Transformation|GetWorldLocation _triggervisualiser))
  (bind (_outhit _returnvalue_2) (Class|KismetSystemLibrary|BoxTraceSingleforObjects _returnvalue (+ _returnvalue "0, 0,0.000010") (Components|Box|GetScaledBoxExtent _triggervisualiser) (Transformation|GetWorldRotation _triggervisualiser) (Variables|CollisionDetection|GetPlayerObj) false 0 "ForOneFrame" true))
  (if _returnvalue_2
    (Utilities|IsValid (Variables|CollisionDetection|GetSpiritRef)
      (:Is%20Valid
        _)
      (:Is%20Not%20Valid
        (bind _asbp_spirit (Utilities|Casting|CastToBP_Spirit (.HitActor (Collision|BreakHitResult _outhit))))
        (Variables|CollisionDetection|SetSpiritRef _asbp_spirit)))
    (if (Variables|CollisionDetection|GetIsOverlapping)
      _
      (else
        (Variables|CollisionDetection|SetIsOverlapping true)
        (CallFunction|BeginOverlap)))
    (CallFunction|TickOverlap)
    (else
      (Utilities|IsValid (Variables|CollisionDetection|GetSpiritRef)
        (:Is%20Valid
          (if (Variables|CollisionDetection|GetIsOverlapping)
            (Variables|CollisionDetection|SetIsOverlapping false)
            (CallFunction|EndOverlap)))))))

(fn ConstructionScript)