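; BP_GraveyardSandstorm is a trigger volume that tells the Spirit's animation Blueprint whether it is in the graveyard area.
; Each Tick, it box-traces for player object types at the AreaVisualiser box's location and scaled extent, rather than using overlap events.
; The first hit that casts to BP_Spirit is cached, and its IsInGraveyard flag switches on while the trace hits and off when it misses.
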(event EventBeginPlay)

(event Collision|EventActorBeginOverlap
  (params (OtherActor :type Actor%20Object%20Reference)))

(event EventTick
  (params (DeltaSeconds :type Float%20%28single-precision%29))
  (bind _areavisualiser (Variables|Default|GetAreaVisualiser))
  (bind _returnvalue (Transformation|GetWorldLocation _areavisualiser))
  (bind (_outhit _returnvalue_2) (Class|KismetSystemLibrary|BoxTraceSingleforObjects _returnvalue _returnvalue (Components|Box|GetScaledBoxExtent _areavisualiser) "0, 0, 0" (Variables|Default|GetPlayerObjType) false 0 "None" true))
  (if _returnvalue_2
    (Utilities|IsValid (Variables|Default|GetSpiritRef)
      (:Is%20Valid
        _)
      (:Is%20Not%20Valid
        (bind _asbp_spirit (Utilities|Casting|CastToBP_Spirit (.HitActor (Collision|BreakHitResult _outhit))))
        (Variables|Default|SetSpiritRef _asbp_spirit)))
    (if (not (Variables|/Game/Art/Spirit/Animations/AnimBP_Spirit.AnimBP_Spirit_C|GetIsInGraveyard (Variables|/Game/Blueprints/BP_Spirit.BP_Spirit_C|GetSpiritAnimBP (Variables|Default|GetSpiritRef))))
      (Variables|/Game/Art/Spirit/Animations/AnimBP_Spirit.AnimBP_Spirit_C|SetIsInGraveyard (Variables|/Game/Blueprints/BP_Spirit.BP_Spirit_C|GetSpiritAnimBP (Variables|Default|GetSpiritRef)) true))
    (else
      (Utilities|IsValid (Variables|Default|GetSpiritRef)
        (:Is%20Valid
          (if (Variables|/Game/Art/Spirit/Animations/AnimBP_Spirit.AnimBP_Spirit_C|GetIsInGraveyard (Variables|/Game/Blueprints/BP_Spirit.BP_Spirit_C|GetSpiritAnimBP (Variables|Default|GetSpiritRef)))
            (Variables|/Game/Art/Spirit/Animations/AnimBP_Spirit.AnimBP_Spirit_C|SetIsInGraveyard (Variables|/Game/Blueprints/BP_Spirit.BP_Spirit_C|GetSpiritAnimBP (Variables|Default|GetSpiritRef)) false)))))))

(fn ConstructionScript)