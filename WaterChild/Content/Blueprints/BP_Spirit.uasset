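; BP_Spirit is the player spirit character, extending parent logic to paint on murals and climbables as it revives and climbs.
; Forward line traces find collision UVs, passed to BP_Mural or BP_Climbable brushes each climbing tick and shortly after a revive hit.
; An FMOD event follows revive start and stop via a parameter.
; It also toggles a pause menu without actually pausing; footprint decal and tutorial UI helpers are left disconnected.
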(event Custom|Event%20LeftFoot)

(event Custom|Event%20RightFoot)

(event EventBeginPlay)

(event EventOnRevive
  (params (PlantHit :type Plant%20Object%20Reference))
  (bind _arrowlinetrace (Variables|Default|GetArrowLineTrace))
  (bind _returnvalue (Transformation|GetWorldLocation _arrowlinetrace))
  (|CallParentFunction PlantHit)
  (Utilities|FlowControl|Delay 0.1)
  (bind _outhit (Collision|LineTraceForObjects _returnvalue (+ _returnvalue (* (Math|Vector|GetForwardVector _arrowlinetrace) (Variables|Default|GetReviveTraceLength))) (Variables|Default|GetMuralObject) true 0 "None"))
  (if (Utilities|ClassIsChildOf (Utilities|GetClass (.HitActor (Collision|BreakHitResult _outhit))) "/Game/Murals/BP_Mural.BP_Mural_C")
    (bind _asbp_mural (Utilities|Casting|CastToBP_Mural (.HitActor (Collision|BreakHitResult _outhit))))
    (Default|DrawBrush _asbp_mural 0 (Variables|Default|GetBrushSize) (.UV (Class|GameplayStatics|FindCollisionUV _outhit)))
    (else
      (bind _asbp_climbable (Utilities|Casting|CastToBP_Climbable (.HitActor (Collision|BreakHitResult _outhit))))
      (Default|ClimbBrush _asbp_climbable 0 (.UV (Class|GameplayStatics|FindCollisionUV _outhit))))))

(event EventTick
  (params (DeltaSeconds :type Float%20%28single-precision%29))
  (bind _arrowlinetrace (Variables|Default|GetArrowLineTrace))
  (bind _returnvalue (Transformation|GetWorldLocation _arrowlinetrace))
  (|CallParentFunction DeltaSeconds)
  (switch Utilities|FlowControl|Switch|SwitchonESpiritState (Variables|Default|GetSpiritState)
    (:Climbing
      (bind _outhit (Collision|LineTraceForObjects _returnvalue (+ _returnvalue (* (Math|Vector|GetForwardVector _arrowlinetrace) (Variables|Default|GetClimbTraceLength))) (Variables|Default|GetMuralObject) true 0 "None"))
      (bind _asbp_climbable (Utilities|Casting|CastToBP_Climbable (.HitActor (Collision|BreakHitResult _outhit))))
      (Default|ClimbBrush _asbp_climbable 0 (.UV (Class|GameplayStatics|FindCollisionUV _outhit))))))

(event EventOnJump
  (|CallParentFunction))

(event EventRevive
  (|CallParentFunction)
  (bind _returnvalue (Class|FMODBlueprintStatics|PlayEventatLocation "/Game/FMOD/Events/SFX/Character/Reviving.Reviving" (Transformation|GetActorTransform))))

(event EventStopRevive
  (|CallParentFunction)
  (Class|FMODBlueprintStatics|EventInstanceSetParameter (stale EventRevive _returnvalue) "Revived" 1.0))

(event Input|ActionEvents|InputActionActionButton
  (params (Key :type Key%20Structure :default "None"))
  ;[1 0.02371 0] Buggy when connected
)

(event Input|ActionEvents|InputActionPauseButton
  (params (Key :type Key%20Structure :default "None"))
  (:Pressed
    (if (Game|IsGamePaused)
      (CallFunction|UnpauseGame)
      (else
        (CallFunction|PauseGame)))))

(fn ConstructionScript)

(fn PauseGame
  (bind _returnvalue (Game|GetPlayerController 0))
  (Utilities|IsValid (LocalVariables|GetPauseMenu)
    (:Is%20Valid
      _)
    (:Is%20Not%20Valid
      (bind _returnvalue_2 (UserInterface|CreateWidget "/Game/Blueprints/UI/UI_Pause.UI_Pause_C" _returnvalue))
      (LocalVariables|SetPauseMenu _returnvalue_2)))
  (UserInterface|Viewport|AddtoViewport (LocalVariables|GetPauseMenu) 0)
  (Input|SetInputModeUIOnly _returnvalue (LocalVariables|GetPauseMenu) "DoNotLock")
  (Variables|/Script/Engine.PlayerController|SetbShowMouseCursor _returnvalue true)
  (Components|Movement|StopMovementImmediately (Variables|Character|GetCharacterMovement)))

(fn UnpauseGame
  (bind _returnvalue (Game|GetPlayerController 0))
  (Viewport|RemoveAllWidgets)
  (Input|SetInputModeGameOnly _returnvalue)
  (Variables|/Script/Engine.PlayerController|SetbShowMouseCursor _returnvalue false))

(fn SpawnFootprint
  (params (ArrowFoot :type Scene%20Component%20Object%20Reference))
  (bind _returnvalue (Transformation|GetWorldLocation ArrowFoot))
  (bind _outhit (Collision|LineTraceByChannel (+ _returnvalue "0, 0,20.000000") (- _returnvalue "0, 0,20.000000") "TraceTypeQuery1" false 0 "None"))
  (Rendering|Decal|SpawnDecalatLocation "/Game/Art/Spirit/Materials/Footprints/M_Footprint.M_Footprint" "10.000000,5.000000,10.000000" (.Location (Collision|BreakHitResult _outhit)) (Math|Rotator|MakeRotator -9e+01 9e+01 (.Yaw (Math|Rotator|BreakRotator (Transformation|GetWorldRotation ArrowFoot)))) 0.0))

(fn SetTutorialUITextures
  (params (GamepadTexture :type Texture%202D%20Object%20Reference) (KeyboardTexture :type Texture%202D%20Object%20Reference))
  (Utilities|IsValid (Variables|Default|GetTutorialUI)
    (:Is%20Valid
      _)
    (:Is%20Not%20Valid
      (bind _returnvalue (UserInterface|CreateWidget "/Game/Blueprints/UI/UI_Tutorial.UI_Tutorial_C" (Game|GetPlayerController 0)))
      (bind _output_get (Variables|Default|SetTutorialUI _returnvalue))))
  (UserInterface|Viewport|AddtoViewport _output_get 0)
  (bind _returnvalue_2 (Appearance|GetDynamicMaterial (Variables|/Game/Blueprints/UI/UI_Tutorial.UI_Tutorial_C|GetImage_Gamepad _output_get) :!class /Script/UMG.Image))
  (Rendering|Material|SetTextureParameterValue _returnvalue_2 "T_Control" GamepadTexture)
  (bind _returnvalue_3 (Appearance|GetDynamicMaterial (Variables|/Game/Blueprints/UI/UI_Tutorial.UI_Tutorial_C|GetImage_Keyboard _output_get) :!class /Script/UMG.Image))
  (Rendering|Material|SetTextureParameterValue _returnvalue_3 "T_Control" KeyboardTexture))