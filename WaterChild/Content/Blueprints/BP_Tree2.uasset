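; Tree of Life actor that sets the glow parameters on its tree mesh's materials.
; Both the construction script and BeginPlay apply the same cyan emissive color and pulse frequency through material parameter setters.
; Each also checks the current level name, turning emissive strength off in Level_01 and setting a soft glow in every other level.
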(event EventBeginPlay
  (bind _sm_treeoflife (Variables|Default|GetSM_TreeOfLife))
  (Rendering|Material|SetVectorParameterValueonMaterials _sm_treeoflife "Emissivecolor" "0.178125,1.000000,0.979881")
  (Rendering|Material|SetScalarParameterValueonMaterials _sm_treeoflife "Frequency" 0.1)
  (bind _returnvalue (Game|GetCurrentLevelName true))
  (if (Utilities|Enum|Equal(Enum) _returnvalue "Level_01")
    (Rendering|Material|SetScalarParameterValueonMaterials _sm_treeoflife "Emissive strength" 0.0)
    (else
      (Rendering|Material|SetScalarParameterValueonMaterials _sm_treeoflife "Emissive strength" 0.5))))

(event Collision|EventActorBeginOverlap
  (params (OtherActor :type Actor%20Object%20Reference)))

(event EventTick
  (params (DeltaSeconds :type Float%20%28single-precision%29)))

(fn ConstructionScript
  (bind _sm_treeoflife (Variables|Default|GetSM_TreeOfLife))
  (Rendering|Material|SetVectorParameterValueonMaterials _sm_treeoflife "Emissivecolor" "0.178125,1.000000,0.979881")
  (Rendering|Material|SetScalarParameterValueonMaterials _sm_treeoflife "Frequency" 0.1)
  (bind _returnvalue (Game|GetCurrentLevelName true))
  (if (Utilities|Enum|Equal(Enum) _returnvalue "Level_01")
    (Rendering|Material|SetScalarParameterValueonMaterials _sm_treeoflife "Emissive strength" 0.0)
    (else
      (Rendering|Material|SetScalarParameterValueonMaterials _sm_treeoflife "Emissive strength" 0.5))))