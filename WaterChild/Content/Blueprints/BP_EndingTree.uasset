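; BP_EndingTree is a tree actor, named for the ending, that animates its growth and then fades in its leaves.
; BeginPlay zeroes material opacity, starts the plant animation at zero play rate, then flows straight into the grow sequence that GrowTree also triggers.
; That sequence restores normal play rate, waits a fixed delay timed to the animation, then runs a timeline driving the Opacity parameter from a curve.
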(event Custom|GrowTree
  (Components|Timeline|SetPlayRate (Variables|Default|GetTreeMesh) 1.0)
  (Utilities|FlowControl|Delay 2.0) ; 2.1s for tree grow to fully finish, 2s + timeline duration is around that time
  (bind _leavesopacitycurve (Timeline|GrowLeavesTimeline PlayFromStart)
    (:Update
      (Rendering|Material|SetScalarParameterValueonMaterials (Variables|Default|GetTreeMesh) "Opacity" _leavesopacitycurve))))

(event EventBeginPlay
  (bind _treemesh (Variables|Default|GetTreeMesh))
  (Rendering|Material|SetScalarParameterValueonMaterials _treemesh "Opacity" 0.0)
  (Components|Animation|PlayAnimation _treemesh "/Game/Art/Cinematics/Props/Foliage/Tree/Plant_Tree_Anim.Plant_Tree_Anim" false)
  (Components|Timeline|SetPlayRate _treemesh 0.0)
  (Components|Timeline|SetPlayRate (Variables|Default|GetTreeMesh) 1.0)
  (Utilities|FlowControl|Delay 2.0) ; 2.1s for tree grow to fully finish, 2s + timeline duration is around that time
  (bind _leavesopacitycurve (Timeline|GrowLeavesTimeline PlayFromStart)
    (:Update
      (Rendering|Material|SetScalarParameterValueonMaterials (Variables|Default|GetTreeMesh) "Opacity" _leavesopacitycurve))))

(fn ConstructionScript)