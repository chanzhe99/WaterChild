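; Trigger volume that sets which layers of the FMOD music loop play when the player's pawn is inside it.
; Tick runs a zero-length box trace over MusicCollision instead of using overlap events, then passes the game mode to MusicDefault.
; MusicDefault sets each instrument parameter on FmodMusicLoop on or off from matching booleans.
; TriggerOnce limits this to the first detection; otherwise it reapplies every tick while the pawn is detected.
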(event EventBeginPlay)

(event Collision|EventActorBeginOverlap
  (params (OtherActor :type Actor%20Object%20Reference)))

(event EventTick
  (params (DeltaSeconds :type Float%20%28single-precision%29))
  (bind _musiccollision (Variables|Default|GetMusicCollision))
  (bind _returnvalue (Transformation|GetWorldLocation _musiccollision))
  (bind (_outhit _returnvalue_2) (Class|KismetSystemLibrary|BoxTraceSingleforObjects _returnvalue (+ _returnvalue "0, 0,0.000010") (Components|Box|GetScaledBoxExtent _musiccollision) (Transformation|GetWorldRotation _musiccollision) (Variables|Default|GetPlayer%20Object%20Type) false 0 "None" true))
  (if _returnvalue_2
    (if (== (.HitActor (Collision|BreakHitResult _outhit)) (Pawn|GetControlledPawn (Game|GetPlayerController 0)))
      (if (Variables|Default|GetbTriggerOnce)
        (if (not (Variables|Default|GetbLock))
          (Variables|Default|SetbLock true)
          (bind _asbp_game_mode (Utilities|Casting|CastToBP_GameMode (Game|GetGameMode) :!label _label))
          (CallFunction|MusicDefault _asbp_game_mode))
        (else
          (goto _label))))))

(fn ConstructionScript)

(fn MusicDefault
  (params (BP_GameMode :type BP%20Game%20Mode%20Object%20Reference))
  (bind _fmodmusicloop (Variables|/Game/Blueprints/BP_GameMode.BP_GameMode_C|GetfmodMusicLoop BP_GameMode))
  (bind _fmodmusicloop_2 (Variables|/Game/Blueprints/BP_GameMode.BP_GameMode_C|GetfmodMusicLoop BP_GameMode))
  (bind _fmodmusicloop_3 (Variables|/Game/Blueprints/BP_GameMode.BP_GameMode_C|GetfmodMusicLoop BP_GameMode))
  (Utilities|FlowControl|Sequence
    (:then_0
      ;[0.1515 1 0] Main Track
      (if (Variables|Default|GetbMainTrack)
        (Class|FMODBlueprintStatics|EventInstanceSetParameter _fmodmusicloop "MainTrack" 1.0)
        (else
          (Class|FMODBlueprintStatics|EventInstanceSetParameter _fmodmusicloop "MainTrack" 0.0))))
    (:then_1
      (if (Variables|Default|GetbTrackA)
        (Class|FMODBlueprintStatics|EventInstanceSetParameter _fmodmusicloop "TrackA" 1.0)
        (else
          (Class|FMODBlueprintStatics|EventInstanceSetParameter _fmodmusicloop "TrackA" 0.0))))
    (:then_2
      (if (Variables|Default|GetbTrackB)
        (Class|FMODBlueprintStatics|EventInstanceSetParameter _fmodmusicloop "TrackB" 1.0)
        (else
          (Class|FMODBlueprintStatics|EventInstanceSetParameter _fmodmusicloop "TrackB" 0.0))))
    (:then_3
      ;[1 0.9557 0] "Percussion"
      (if (Variables|Default|GetbPianoMelody)
        (Class|FMODBlueprintStatics|EventInstanceSetParameter _fmodmusicloop_2 "PianoMelody" 1.0)
        (else
          (Class|FMODBlueprintStatics|EventInstanceSetParameter _fmodmusicloop_2 "PianoMelody" 0.0))))
    (:then_4
      (if (Variables|Default|GetbPianoAccomp1)
        (Class|FMODBlueprintStatics|EventInstanceSetParameter _fmodmusicloop_2 "PianoAccomp1" 1.0)
        (else
          (Class|FMODBlueprintStatics|EventInstanceSetParameter _fmodmusicloop_2 "PianoAccomp1" 0.0))))
    (:then_5
      (if (Variables|Default|GetbPianoAccomp2)
        (Class|FMODBlueprintStatics|EventInstanceSetParameter _fmodmusicloop_2 "PianoAccomp2" 1.0)
        (else
          (Class|FMODBlueprintStatics|EventInstanceSetParameter _fmodmusicloop_2 "PianoAccomp2" 0.0))))
    (:then_6
      (if (Variables|Default|GetbGlockenspiel)
        (Class|FMODBlueprintStatics|EventInstanceSetParameter _fmodmusicloop_2 "Glockenspiel" 1.0)
        (else
          (Class|FMODBlueprintStatics|EventInstanceSetParameter _fmodmusicloop_2 "Glockenspiel" 0.0))))
    (:then_7
      ;[0.05353 0.01776 1] Strings
      (if (Variables|Default|GetbViolin)
        (Class|FMODBlueprintStatics|EventInstanceSetParameter _fmodmusicloop_3 "Violin" 1.0)
        (else
          (Class|FMODBlueprintStatics|EventInstanceSetParameter _fmodmusicloop_3 "Violin" 0.0))))
    (:then_8
      (if (Variables|Default|GetbViola)
        (Class|FMODBlueprintStatics|EventInstanceSetParameter _fmodmusicloop_3 "Viola" 1.0)
        (else
          (Class|FMODBlueprintStatics|EventInstanceSetParameter _fmodmusicloop_3 "Viola" 0.0))))
    (:then_9
      (if (Variables|Default|GetbCello)
        (Class|FMODBlueprintStatics|EventInstanceSetParameter _fmodmusicloop_3 "Cello" 1.0)
        (else
          (Class|FMODBlueprintStatics|EventInstanceSetParameter _fmodmusicloop_3 "Cello" 0.0))))))