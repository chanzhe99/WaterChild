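; Music trigger actor that starts and stops the City audio as the player's controlled pawn enters its box volumes.
; Every Tick, zero-length box traces matching City1Enter and City1Exit play or stop the audio, guarded by IsPlaying checks, instead of using those boxes' empty overlap events.
; A separate TempOff box stops the audio on begin overlap; its play counterpart is disconnected.
; Each transition prints a debug string.
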(event OnComponentBeginOverlap(City1Enter)
  (params (OverlappedComponent :type Primitive%20Component%20Object%20Reference) (OtherActor :type Actor%20Object%20Reference) (OtherComp :type Primitive%20Component%20Object%20Reference) (OtherBodyIndex :type Integer) (bFromSweep :type Boolean) (SweepResult :type Hit%20Result%20Structure%20%28by%20ref%29)))

(event OnComponentBeginOverlap(TempOff)
  (params (OverlappedComponent :type Primitive%20Component%20Object%20Reference) (OtherActor :type Actor%20Object%20Reference) (OtherComp :type Primitive%20Component%20Object%20Reference) (OtherBodyIndex :type Integer) (bFromSweep :type Boolean) (SweepResult :type Hit%20Result%20Structure%20%28by%20ref%29))
  (bind _city (Variables|Default|GetCity))
  (if (== OtherActor (Pawn|GetControlledPawn (Game|GetPlayerController 0)))
    (bind _returnvalue (Class|FMODAudioComponent|IsPlaying _city))
    (if _returnvalue
      (Development|PrintString "TEMP STOP")
      (Class|FMODAudioComponent|Stop _city))))

(event OnComponentEndOverlap(TempOff)
  (params (OverlappedComponent :type Primitive%20Component%20Object%20Reference) (OtherActor :type Actor%20Object%20Reference) (OtherComp :type Primitive%20Component%20Object%20Reference) (OtherBodyIndex :type Integer)))

(event OnComponentBeginOverlap(City1Exit)
  (params (OverlappedComponent :type Primitive%20Component%20Object%20Reference) (OtherActor :type Actor%20Object%20Reference) (OtherComp :type Primitive%20Component%20Object%20Reference) (OtherBodyIndex :type Integer) (bFromSweep :type Boolean) (SweepResult :type Hit%20Result%20Structure%20%28by%20ref%29)))

(event EventBeginPlay)

(event Collision|EventActorBeginOverlap
  (params (OtherActor :type Actor%20Object%20Reference)))

(event EventTick
  (params (DeltaSeconds :type Float%20%28single-precision%29))
  (bind _city (Variables|Default|GetCity))
  (bind _city1enter (Variables|Default|GetCity1Enter))
  (bind _city1exit (Variables|Default|GetCity1Exit))
  (bind _returnvalue (Transformation|GetWorldLocation _city1exit))
  (bind _returnvalue_2 (Transformation|GetWorldLocation _city1enter))
  (Utilities|FlowControl|Sequence
    (:then_0
      (bind (_outhit _returnvalue_3) (Class|KismetSystemLibrary|BoxTraceSingleforObjects _returnvalue_2 _returnvalue_2 (Components|Box|GetScaledBoxExtent _city1enter) (Transformation|GetWorldRotation _city1enter) (Variables|Default|GetPlayer%20Object%20Type) false 0 "None" true)) ; City1Enter
      (if _returnvalue_3
        (if (== (.HitActor (Collision|BreakHitResult _outhit)) (Pawn|GetControlledPawn (Game|GetPlayerController 0)))
          (bind _returnvalue_4 (Class|FMODAudioComponent|IsPlaying _city))
          (if (not _returnvalue_4)
            (Class|FMODAudioComponent|Play _city)
            (Development|PrintString "PLAY")))))
    (:then_1
      (bind (_outhit_2 _returnvalue_5) (Class|KismetSystemLibrary|BoxTraceSingleforObjects _returnvalue _returnvalue (Components|Box|GetScaledBoxExtent _city1exit) (Transformation|GetWorldRotation _city1exit) (Variables|Default|GetPlayer%20Object%20Type) false 0 "None" true)) ; City1Exit
      (if _returnvalue_5
        (if (== (.HitActor (Collision|BreakHitResult _outhit_2)) (Pawn|GetControlledPawn (Game|GetPlayerController 0)))
          (bind _returnvalue_6 (Class|FMODAudioComponent|IsPlaying _city))
          (if _returnvalue_6
            (Class|FMODAudioComponent|Stop _city)
            (Development|PrintString "STOP")))))))

(fn ConstructionScript)