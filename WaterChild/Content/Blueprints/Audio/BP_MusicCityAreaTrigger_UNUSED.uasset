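; Trigger actor that plays city area music while the player is inside it, marked unused by its asset name.
; At BeginPlay it zeroes the strings and violin parameters on the City audio component.
; Begin and end overlap events start and stop that component, responding only to the pawn controlled by player controller 0.
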(event EventBeginPlay
  (bind _city (Variables|Default|GetCity))
  (Class|FMODAudioComponent|SetParameter _city "CityStrings" 0.0)
  (Class|FMODAudioComponent|SetParameter _city "CityViolin" 0.0))

(event Collision|EventActorBeginOverlap
  (params (OtherActor :type Actor%20Object%20Reference))
  (if (== OtherActor (Pawn|GetControlledPawn (Game|GetPlayerController 0)))
    (Class|FMODAudioComponent|Play (Variables|Default|GetCity))))

(event EventTick
  (params (DeltaSeconds :type Float%20%28single-precision%29)))

(event Collision|EventActorEndOverlap
  (params (OtherActor :type Actor%20Object%20Reference))
  (if (== (Pawn|GetControlledPawn (Game|GetPlayerController 0)) OtherActor)
    (Class|FMODAudioComponent|Stop (Variables|Default|GetCity))))

(fn ConstructionScript)