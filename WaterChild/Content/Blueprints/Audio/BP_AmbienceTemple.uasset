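; BP_AmbienceTemple is an audio actor that adjusts wind and temple ambience as overlaps begin and end on two trigger volumes.
; Wind and Temple sounds start on BeginPlay with chimes silenced.
; The main trigger sets wind volume to configurable enter and exit values, optionally toggling chimes through a sound parameter.
; The end trigger sets wind to full on entry and restores the exit value on leaving.
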(event OnComponentBeginOverlap(MainTempleTrigger)
  (params (OverlappedComponent :type Primitive%20Component%20Object%20Reference) (OtherActor :type Actor%20Object%20Reference) (OtherComp :type Primitive%20Component%20Object%20Reference) (OtherBodyIndex :type Integer) (bFromSweep :type Boolean) (SweepResult :type Hit%20Result%20Structure%20%28by%20ref%29))
  (Class|FMODAudioComponent|SetParameter (Variables|Default|GetWind) "WindVolume" (Variables|Default|GetWindVolumeEnter))
  (if (Variables|Default|GetbPlayChimes)
    (Class|FMODAudioComponent|SetParameter (Variables|Default|GetTemple) "PlayChimes" 0.8)))

(event OnComponentEndOverlap(MainTempleTrigger)
  (params (OverlappedComponent :type Primitive%20Component%20Object%20Reference) (OtherActor :type Actor%20Object%20Reference) (OtherComp :type Primitive%20Component%20Object%20Reference) (OtherBodyIndex :type Integer))
  (Class|FMODAudioComponent|SetParameter (Variables|Default|GetWind) "WindVolume" (Variables|Default|GetWindVolumeExit))
  (if (Variables|Default|GetbPlayChimes)
    (Class|FMODAudioComponent|SetParameter (Variables|Default|GetTemple) "PlayChimes" 0.0)))

(event OnComponentBeginOverlap(EndTempleTrigger)
  (params (OverlappedComponent :type Primitive%20Component%20Object%20Reference) (OtherActor :type Actor%20Object%20Reference) (OtherComp :type Primitive%20Component%20Object%20Reference) (OtherBodyIndex :type Integer) (bFromSweep :type Boolean) (SweepResult :type Hit%20Result%20Structure%20%28by%20ref%29))
  (Class|FMODAudioComponent|SetParameter (Variables|Default|GetWind) "WindVolume" 1.0))

(event OnComponentEndOverlap(EndTempleTrigger)
  (params (OverlappedComponent :type Primitive%20Component%20Object%20Reference) (OtherActor :type Actor%20Object%20Reference) (OtherComp :type Primitive%20Component%20Object%20Reference) (OtherBodyIndex :type Integer))
  (Class|FMODAudioComponent|SetParameter (Variables|Default|GetWind) "WindVolume" (Variables|Default|GetWindVolumeExit)))

(event EventBeginPlay
  (bind _temple (Variables|Default|GetTemple))
  (Class|FMODAudioComponent|Play (Variables|Default|GetWind))
  (Class|FMODAudioComponent|Play _temple)
  (Class|FMODAudioComponent|SetParameter _temple "PlayChimes" 0.0))

(event EventTick
  (params (DeltaSeconds :type Float%20%28single-precision%29)))

(event Collision|EventActorBeginOverlap
  (params (OtherActor :type Actor%20Object%20Reference)))

(event Collision|EventActorEndOverlap
  (params (OtherActor :type Actor%20Object%20Reference)))

(fn ConstructionScript)