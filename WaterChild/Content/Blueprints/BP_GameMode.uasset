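; Game mode that starts the looping FMOD background music when play begins.
; BeginPlay sets the master, music and SFX global parameters, plays the music event in 2D and keeps the instance.
; The level name selects the layers: Level_New enables TrackA alone, while any other level enables TrackA and TrackB.
; An unconnected chain for showing a start menu with the mouse cursor and disabled player input never runs.
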(event EventBeginPlay
  (Class|FMODBlueprintStatics|SetGlobalParameterbyName "GlobalMaster" 0.8)
  (Class|FMODBlueprintStatics|SetGlobalParameterbyName "GlobalMusic" 0.8)
  (Class|FMODBlueprintStatics|SetGlobalParameterbyName "GlobalSFX" 0.8)
  (bind _returnvalue (Class|FMODBlueprintStatics|PlayEvent2D "/Game/FMOD/Events/Music/MusicLoop.MusicLoop"))
  (bind _output_get (Variables|Default|SetfmodMusicLoop _returnvalue))
  (bind _returnvalue_2 (Game|GetCurrentLevelName true))
  (if (Utilities|Enum|Equal(Enum) _returnvalue_2 "Level_New")
    (Class|FMODBlueprintStatics|EventInstanceSetParameter _output_get "TrackA" 1.0)
    (else
      (Class|FMODBlueprintStatics|EventInstanceSetParameter _output_get "TrackA" 1.0)
      (Class|FMODBlueprintStatics|EventInstanceSetParameter _output_get "TrackB" 1.0))))

(event EventTick
  (params (DeltaSeconds :type Float%20%28single-precision%29)))

(fn ConstructionScript)