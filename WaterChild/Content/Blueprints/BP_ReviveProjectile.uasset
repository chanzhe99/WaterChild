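; Spirit's revive projectile that detects hits itself by tracing short rays along six axis directions every Tick against interactable object types.
; On the first hit it destroys itself, leaves the spirit's projectile list and spawns a splash effect.
; It then selects and interacts with a hit Interactable, and paints a growing brush at the hit UV on murals or climbables with matching particle effects.
; Older trace and interact-end logic remains disconnected.
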(event EventTick
  (params (DeltaSeconds :type Float%20%28single-precision%29))
  (bind _spiritreference (Variables|Default|GetSpiritReference))
  (bind (_outhitresult _washit) (CallFunction|LineTraceOutfromOrigin))
  (if _washit
    (Variables|Default|SetOutHitRef _outhitresult)
    (Actor|DestroyActor)
    (Utilities|Array|RemoveItem (Variables|/Game/Blueprints/BP_Spirit.BP_Spirit_C|GetProjectileList (Variables|Default|GetSpiritReference)) self)
    (Niagara|SpawnSystematLocation "/Game/Art/Particles/P_SprayWater/P_Splash.P_Splash" (.impactpoint (Variables|Default|GetOutHitRef)) (Math|Conversions|RotationFromXVector (.impactnormal (Variables|Default|GetOutHitRef))))
    (Utilities|FlowControl|Sequence
      (:then_0
        (bind _asinteractable (Utilities|Casting|CastToInteractable (.hitactor (Variables|Default|GetOutHitRef))))
        (bind _output_get (Variables|/Script/WaterChild.Spirit|SetSelectedPlant _spiritreference _asinteractable))
        (Class|Interactable|OnInteract _output_get _spiritreference))
      (:then_1
        (if (Utilities|ClassIsChildOf (Utilities|GetClass (.hitactor (Variables|Default|GetOutHitRef))) "/Game/Blueprints/Interactables/BP_Mural.BP_Mural_C")
          (bind _asbp_mural (Utilities|Casting|CastToBP_Mural (.hitactor (Variables|Default|GetOutHitRef))))
          (Default|SetBrushSettings _asbp_mural 7.5e+02 5e+02)
          (Default|DrawBrush _asbp_mural 0 (.UV (Class|GameplayStatics|FindCollisionUV (Variables|Default|GetOutHitRef))) "/Game/Murals/MI_MuralBrush.MI_MuralBrush")
          (Niagara|SpawnSystematLocation "/Game/Art/Particles/P_DustFalling/P_DustFalling.P_DustFalling" (.impactpoint (Variables|Default|GetOutHitRef)))
          (else
            (bind _asbp_climbable (Utilities|Casting|CastToBP_Climbable (.hitactor (Variables|Default|GetOutHitRef))))
            (Default|SetBrushSettings _asbp_climbable 7.5e+02 5e+02)
            (Default|ClimbBrush _asbp_climbable 0 (.UV (Class|GameplayStatics|FindCollisionUV (Variables|Default|GetOutHitRef))) "/Game/Murals/MI_MuralBrush.MI_MuralBrush")
            (Niagara|SpawnSystematLocation "/Game/Art/Particles/P_PlantREvive/P_WallPlantRevive.P_WallPlantRevive" (.impactpoint (Variables|Default|GetOutHitRef)))))))))

(fn ConstructionScript)

(fn LineTraceinAxis
  (params (LineAxis :type Vector))
  (bind _returnvalue (Transformation|GetActorLocation))
  (bind (_outhit _returnvalue_2) (Collision|LineTraceForObjects (- _returnvalue LineAxis) (+ _returnvalue LineAxis) (Variables|Default|GetInteractableObjectTypes) true 0 "ForOneFrame"))
  (return _outhit _returnvalue_2))

(fn LineTraceOutfromOrigin
  (bind (_outhit _returnvalue) (CallFunction|LineTraceinAxisTest "-10.000000, 0, 0"))
  (if _returnvalue
    (LocalVariables|SettempHitResult _outhit)
    (LocalVariables|SettempHitBool true)
    (else
      (bind (_outhit_2 _returnvalue_2) (CallFunction|LineTraceinAxisTest "10.000000, 0, 0"))
      (if _returnvalue_2
        (LocalVariables|SettempHitResult _outhit_2)
        (LocalVariables|SettempHitBool true)
        (else
          (bind (_outhit_3 _returnvalue_3) (CallFunction|LineTraceinAxisTest "0.000000,-10.000000, 0"))
          (if _returnvalue_3
            (LocalVariables|SettempHitResult _outhit_3)
            (LocalVariables|SettempHitBool true)
            (else
              (bind (_outhit_4 _returnvalue_4) (CallFunction|LineTraceinAxisTest "0.000000,10.000000, 0"))
              (if _returnvalue_4
                (LocalVariables|SettempHitResult _outhit_4)
                (LocalVariables|SettempHitBool true)
                (else
                  (bind (_outhit_5 _returnvalue_5) (CallFunction|LineTraceinAxisTest "0.000000,0.000000,-10.000000"))
                  (if _returnvalue_5
                    (LocalVariables|SettempHitResult _outhit_5)
                    (LocalVariables|SettempHitBool true)
                    (else
                      (bind (_outhit_6 _returnvalue_6) (CallFunction|LineTraceinAxisTest "0.000000,0.000000,10.000000"))
                      (if _returnvalue_6
                        (LocalVariables|SettempHitResult _outhit_6)
                        (LocalVariables|SettempHitBool true)
                        (else
                          (LocalVariables|SettempHitBool false)))))))))))))
  (return (LocalVariables|GettempHitResult) (LocalVariables|GettempHitBool)))

(fn LineTraceinAxisTest
  (params (LineAxis :type Vector))
  (bind _returnvalue (Transformation|GetActorLocation))
  (bind (_outhit _returnvalue_2) (Collision|LineTraceForObjects _returnvalue (+ LineAxis _returnvalue) (Variables|Default|GetInteractableObjectTypes) true 0 "ForOneFrame"))
  (return _outhit _returnvalue_2))