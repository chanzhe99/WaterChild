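; StartCamera is a trigger camera that holds the opening view until the game starts, then blends to the player's camera.
; BeginPlay stores the original view target, switches to the camera's owner and disables tick.
; GameStart or a StartButton click enables tick, which reissues the configurable blend back every frame.
; After a delay matching the blend time, tick stops and game-only input and character input are enabled.
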(event OnClicked(StartButton)
  (bind _returnvalue (Game|GetPlayerController 0))
  ;[1 1 1] Button Input
  (Actor|Tick|SetActorTickEnabled true)
  (Variables|Default|SetGameStarted true)
  (Utilities|FlowControl|Delay (Variables|Default|GetCameraSwapTime))
  (Actor|Tick|SetActorTickEnabled false)
  (Input|SetInputModeGameOnly _returnvalue)
  (Input|EnableInput (Game|GetPlayerCharacter 0) _returnvalue))

(event Custom|GameStart
  (bind _returnvalue (Game|GetPlayerController 0))
  ;[1 1 1] Button Input
  (Actor|Tick|SetActorTickEnabled true)
  (Variables|Default|SetGameStarted true)
  (Utilities|FlowControl|Delay (Variables|Default|GetCameraSwapTime))
  (Actor|Tick|SetActorTickEnabled false)
  (Input|SetInputModeGameOnly _returnvalue)
  (Input|EnableInput (Game|GetPlayerCharacter 0) _returnvalue))

(event EventBeginPlay
  (bind _returnvalue (Game|GetPlayerController 0))
  ;[1 1 1] Change Port and remember player cam
  (Variables|Default|SetOriginalCam (Pawn|GetViewTarget _returnvalue))
  (Game|Player|SetViewTargetwithBlend _returnvalue (Components|GetOwner (Variables|Default|GetCamera)) 0.0 "VTBlend_Linear" 0.0 false)
  (Actor|Tick|SetActorTickEnabled false))

(event EventTick
  (params (DeltaSeconds :type Float%20%28single-precision%29))
  ;[1 1 1] Change Camera, tick is disabled after
  (if (Variables|Default|GetGameStarted)
    (Game|Player|SetViewTargetwithBlend (Game|GetPlayerController 0) (Variables|Default|GetOriginalCam) (Variables|Default|GetCameraSwapTime) (Variables|Default|GetBlendingType) (Variables|Default|GetCameraSwapCurve) false)))

(fn ConstructionScript)