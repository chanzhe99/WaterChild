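; A one-shot cutscene trigger volume that plays a Level Sequence when the player's controlled pawn overlaps its TriggerBox.
; It creates a sequence player, disables player character input, plays the sequence, then waits its duration with a Delay before restoring input.
; IsTriggered blocks replays but is only set after that Delay, so overlaps during playback are not blocked.
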(event OnComponentBeginOverlap(TriggerBox)
  (params (OverlappedComponent :type Primitive%20Component%20Object%20Reference) (OtherActor :type Actor%20Object%20Reference) (OtherComp :type Primitive%20Component%20Object%20Reference) (OtherBodyIndex :type Integer) (bFromSweep :type Boolean) (SweepResult :type Hit%20Result%20Structure%20%28by%20ref%29))
  (if (== OtherActor (Pawn|GetControlledPawn (Game|GetPlayerController 0)))
    (if (not (Variables|Default|GetIsTriggered))
      (Utilities|FlowControl|Sequence
        (:then_0
          (bind _returnvalue (Sequencer|Player|CreateLevelSequencePlayer (Variables|Default|GetLevel_Sequence)))
          (Variables|Default|SetSequencePlayer _returnvalue))
        (:then_1
          (Input|DisableInput (Game|GetPlayerCharacter 0) (Game|GetPlayerController 0))
          (Sequencer|Player|Play (Variables|Default|GetSequencePlayer) :!class /Script/MovieScene.MovieSceneSequencePlayer)
          (Utilities|FlowControl|Delay (Class|TimeManagementBlueprintLibrary|ToSeconds(QualifiedFrameTime) (Media|MediaPlayer|GetDuration (Variables|Default|GetSequencePlayer))))
          (Input|EnableInput (Game|GetPlayerCharacter 0) (Game|GetPlayerController 0))
          (Variables|Default|SetIsTriggered true))))))

(event EventBeginPlay)

(event EventTick
  (params (DeltaSeconds :type Float%20%28single-precision%29)))

(fn ConstructionScript)