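; CameraTrigger is a trigger volume that briefly turns the player's view toward a CameraTarget, guarded by a Triggered flag that it clears on use.
; When the first player's pawn overlaps the Box, it stores the current view target, moves its Camera onto the player camera's transform and takes over the view.
; Tick interpolates the Camera's rotation toward the target, then blends back to the original view once nearly aligned.
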(event OnComponentBeginOverlap(Box)
  (params (OverlappedComponent :type Primitive%20Component%20Object%20Reference) (OtherActor :type Actor%20Object%20Reference) (OtherComp :type Primitive%20Component%20Object%20Reference) (OtherBodyIndex :type Integer) (bFromSweep :type Boolean) (SweepResult :type Hit%20Result%20Structure%20%28by%20ref%29))
  (bind _returnvalue (Game|GetPlayerCameraManager 0))
  (bind _returnvalue_2 (Game|GetPlayerController 0))
  (if (== _returnvalue_2 (Components|GetOwner OtherActor))
    (if (stale _output_get)
      (bind _output_get (Variables|Default|SetTriggered false))
      (Variables|Default|SetOriginalCam (Pawn|GetViewTarget _returnvalue_2))
      (Transformation|SetWorldLocationAndRotation (Variables|Default|GetCamera) (Transformation|GetActorLocation _returnvalue) (Transformation|GetActorRotation _returnvalue) false true)
      (Game|Player|SetViewTargetwithBlend (Game|GetPlayerController 0) (Components|GetOwner (Variables|Default|GetCamera)) 0.0 "VTBlend_EaseIn" 0.0 false)
      (bind _output_get_2 (Variables|Default|SetLookTarget (Math|Rotator|FindLookatRotation (Transformation|GetWorldLocation (Variables|Default|GetCamera)) (Transformation|GetWorldLocation (Variables|Default|GetCameraTarget))))))))

(event EventTick
  (params (DeltaSeconds :type Float%20%28single-precision%29))
  (bind _returnvalue (Utilities|Time|GetWorldDeltaSeconds))
  (bind _cameratarget (Variables|Default|GetCameraTarget))
  (bind _camera (Variables|Default|GetCamera))
  (bind _camera_2 (Variables|Default|GetCamera))
  (bind _returnvalue_2 (Transformation|GetWorldLocation _cameratarget))
  (bind _returnvalue_3 (Transformation|GetWorldLocation _camera))
  (bind _returnvalue_4 (Transformation|GetWorldRotation _camera_2))
  (bind _returnvalue_5 (Math|Rotator|FindLookatRotation _returnvalue_3 _returnvalue_2))
  (bind _returnvalue_6 (Math|Interpolation|RInterpTo _returnvalue_4 _returnvalue_5 _returnvalue 2.0))
  (if (== (Pawn|GetViewTarget (Game|GetPlayerController 0)) (Components|GetOwner (Variables|Default|GetCamera)))
    (if (Math|Rotator|Equal(Rotator) _returnvalue_6 (stale OnComponentBeginOverlap(Box) _output_get_2) 0.5)
      (Game|Player|SetViewTargetwithBlend (Game|GetPlayerController 0) (Variables|Default|GetOriginalCam) 1.0 "VTBlend_EaseInOut" 1.0 false)
      (else
        (Transformation|SetWorldRotation (Variables|Default|GetCamera) _returnvalue_6 false false)))))

(fn ConstructionScript)