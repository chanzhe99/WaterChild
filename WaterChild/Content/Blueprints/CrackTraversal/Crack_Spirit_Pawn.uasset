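; Spirit pawn that carries the player along a crack's spline path in either direction while forward input is held.
; Trigger events set direction and enable tick, which drives a timeline with play rate scaled by spline length for constant speed.
; Reverse travel runs the timeline backwards with rotation flipped 180 degrees.
; At the path's end it repossesses the pawn remembered at BeginPlay, fades the camera, restores input and stops ticking.
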(event Custom|Triggered
  ;[1 1 1] Direction setup
  (Variables|Default|SetStartPoint 0.0)
  (Variables|Default|SetEndPoint 1.0)
  (Variables|Default|SetEffectiveSpeed (Variables|Default|GetSpeed))
  (Variables|Default|SetIsForward true)
  (Components|Timeline|SetNewTime (Variables|Default|GetCrackMove) (Variables|Default|GetStartPoint))
  (Actor|Tick|SetActorTickEnabled true))

(event Custom|Deactivate_Tick
  ;[1 1 1] Deactivate when not in use
  (Actor|Tick|SetActorTickEnabled false))

(event Custom|Triggered_Reverse
  ;[1 1 1] Direction setup
  (Variables|Default|SetStartPoint 1.0)
  (Variables|Default|SetEndPoint 0.0)
  (Variables|Default|SetEffectiveSpeed (* (Variables|Default|GetSpeed) -1.0))
  (Variables|Default|SetIsForward false)
  (Components|Timeline|SetNewTime (Variables|Default|GetCrackMove) (Variables|Default|GetStartPoint))
  (Actor|Tick|SetActorTickEnabled true))

(event EventBeginPlay
  (bind _returnvalue (Game|GetPlayerController 0))
  ;[1 1 1] Remember pawn
  (CallFunction|DeactivateTick)
  (Variables|Default|SetOriginalPawn (Pawn|GetControlledPawn _returnvalue))
  (Variables|Default|SetPlayer%20Controller _returnvalue))

(event Collision|EventActorBeginOverlap
  (params (OtherActor :type Actor%20Object%20Reference)))

(event EventTick
  (params (DeltaSeconds :type Float%20%28single-precision%29))
  (bind _returnvalue (Game|GetPlayerController 0))
  (bind _path (Variables|Default|GetPath))
  (bind _spline (Variables|/Game/Blueprints/CrackTraversal/CrackPath.CrackPath_C|GetSpline _path))
  ;[1 1 1] Check for foward input
  (if (> (Input|AxisValues|GetMoveForward) 0.0)
    ;[1 1 1] Travel along spline
    (Components|Timeline|SetPlayRate (Variables|Default|GetCrackMove) (* (/ 1.0 (Spline|GetSplineLength (Variables|/Game/Blueprints/CrackTraversal/CrackPath.CrackPath_C|GetSpline (Variables|Default|GetPath)))) (Variables|Default|GetEffectiveSpeed)))
    (bind _newtrack_0 (Timeline|CrackMove Play) ; Goes from 0 to 1
      (:Update
        (Variables|Default|SetAlpha _newtrack_0)
        (if (Variables|Default|GetIsForward)
          (Transformation|SetActorLocationAndRotation (Spline|GetLocationatDistanceAlongSpline _spline (Math|Float|Lerp 0.0 (Spline|GetSplineLength _spline) (Variables|Default|GetAlpha)) "World") (Spline|GetRotationatDistanceAlongSpline _spline (Math|Float|Lerp 0.0 (Spline|GetSplineLength _spline) (Variables|Default|GetAlpha)) "World"))
          (else
            (Transformation|SetActorLocationAndRotation (Spline|GetLocationatDistanceAlongSpline _spline (Math|Float|Lerp 0.0 (Spline|GetSplineLength _spline) (Variables|Default|GetAlpha)) "World") (Math|Rotator|CombineRotators (Spline|GetRotationatDistanceAlongSpline _spline (Math|Float|Lerp 0.0 (Spline|GetSplineLength _spline) (Variables|Default|GetAlpha)) "World") "0,180.000000, 0"))))
        ;[1 1 1] Detect End and return
        (if (== (Variables|Default|GetAlpha) (Variables|Default|GetEndPoint))
          (Audio|Components|Audio|Stop (Variables|Default|GetCrackMove))
          (Pawn|UnPossess _returnvalue)
          (Pawn|Possess _returnvalue (Variables|Default|GetOriginalPawn))
          (Utilities|FlowControl|Sequence
            (:then_0
              (CallFunction|DeactivateTick)
              (CameraFades|StartCameraFade (Variables|/Script/Engine.PlayerController|GetPlayerCameraManager (Game|GetPlayerController 0)) 1.0 0.0 (Variables|Default|GetFadeTime) "(R=1.000000,G=1.000000,B=1.000000,A=1.000000)" false false))
            (:then_1
              (Input|EnableInput (Game|GetPlayerCharacter 0) _returnvalue))))))
    (else
      (Timeline|CrackMove Stop))))

(fn ConstructionScript)