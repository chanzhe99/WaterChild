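; Crack traversal actor that lets the player pass between an entrance and an exit by taking control of a spirit pawn.
; On BeginPlay it hands its spline to the child-actor Crack_Spirit_Pawn as the path.
; Hitting either end disables input, blends the view and fades out, then triggers the pawn forward or in reverse.
; It then teleports the player's pawn to the opposite end, possesses the spirit pawn and fades back in.
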(event OnComponentHit(Entrance)
  (params (HitComponent :type Primitive%20Component%20Object%20Reference) (OtherActor :type Actor%20Object%20Reference) (OtherComp :type Primitive%20Component%20Object%20Reference) (NormalImpulse :type Vector :default "0, 0, 0") (Hit :type Hit%20Result%20Structure%20%28by%20ref%29))
  (bind _returnvalue (Game|GetPlayerController 0))
  (bind _returnvalue_2 (Game|GetPlayerController 0))
  (bind _blend_time (Variables|Default|GetBlend%20Time))
  (bind _returnvalue_3 (Pawn|GetControlledPawn _returnvalue))
  ;[1 1 1] Forward direction
  (if (== OtherActor _returnvalue_3)
    (Utilities|FlowControl|Sequence
      (:then_0
        (Input|DisableInput (Game|GetPlayerCharacter 0) _returnvalue))
      (:then_1
        (Components|Activation|SetActive (Variables|Default|GetEntranceCam) false false)
        (Game|Player|SetViewTargetwithBlend _returnvalue 0 _blend_time "VTBlend_EaseInOut" 0.5 false)
        (CameraFades|StartCameraFade :self (Variables|/Script/Engine.PlayerController|GetPlayerCameraManager _returnvalue) :ToAlpha 1.0 :Duration _blend_time)
        (Utilities|FlowControl|Delay _blend_time)
        (Default|Triggered (Variables|Default|GetCrackPawn))
        (Transformation|SetActorLocation _returnvalue_3 (Transformation|GetWorldLocation (Variables|Default|GetExitPoint)) false false)
        (Pawn|UnPossess _returnvalue_2)
        (Pawn|Possess _returnvalue_2 (Variables|Default|GetCrackPawn))
        (CameraFades|StartCameraFade :self (Variables|/Script/Engine.PlayerController|GetPlayerCameraManager _returnvalue_2) :FromAlpha 1.0 :Duration (Variables|Default|GetBlend%20Time))))))

(event OnComponentHit(Exit)
  (params (HitComponent :type Primitive%20Component%20Object%20Reference) (OtherActor :type Actor%20Object%20Reference) (OtherComp :type Primitive%20Component%20Object%20Reference) (NormalImpulse :type Vector :default "0, 0, 0") (Hit :type Hit%20Result%20Structure%20%28by%20ref%29))
  (bind _returnvalue (Game|GetPlayerController 0))
  (bind _returnvalue_2 (Game|GetPlayerController 0))
  (bind _blend_time (Variables|Default|GetBlend%20Time))
  (bind _returnvalue_3 (Pawn|GetControlledPawn _returnvalue))
  ;[1 1 1] Reverse Direction
  (if (== OtherActor _returnvalue_3)
    (Utilities|FlowControl|Sequence
      (:then_0
        (Input|DisableInput (Game|GetPlayerCharacter 0) 0))
      (:then_1
        (Components|Activation|SetActive (Variables|Default|GetExitCam) false false)
        (Game|Player|SetViewTargetwithBlend _returnvalue 0 _blend_time "VTBlend_EaseInOut" 0.5 false)
        (CameraFades|StartCameraFade :self (Variables|/Script/Engine.PlayerController|GetPlayerCameraManager _returnvalue) :ToAlpha 1.0 :Duration _blend_time)
        (Utilities|FlowControl|Delay _blend_time)
        (Default|TriggeredReverse (Variables|Default|GetCrackPawn))
        (Transformation|SetActorLocation _returnvalue_3 (Transformation|GetWorldLocation (Variables|Default|GetEntrancePoint)) false false)
        (Pawn|UnPossess _returnvalue_2)
        (Pawn|Possess _returnvalue_2 (Variables|Default|GetCrackPawn))
        (CameraFades|StartCameraFade :self (Variables|/Script/Engine.PlayerController|GetPlayerCameraManager _returnvalue_2) :FromAlpha 1.0 :Duration (Variables|Default|GetBlend%20Time))))))

(event EventBeginPlay
  ;[1 1 1] Setup
  (bind _ascrack_spirit_pawn (Utilities|Casting|CastToCrack_Spirit_Pawn (Variables|/Script/Engine.ChildActorComponent|GetChildActor (Variables|Default|GetCrack_Spirit_Pawn1))))
  (Variables|/Game/Blueprints/CrackTraversal/Crack_Spirit_Pawn.Crack_Spirit_Pawn_C|SetPath _ascrack_spirit_pawn (Variables|Default|GetCrackSpline))
  (Variables|Default|SetCrackPawn _ascrack_spirit_pawn)
  (Variables|Default|SetOriginal%20Zoom (Variables|/Script/Engine.PlayerCameraManager|GetDefaultFOV (Variables|/Script/Engine.PlayerController|GetPlayerCameraManager (Game|GetPlayerController 0))))
  (Actor|Tick|SetActorTickEnabled false))

(fn ConstructionScript)