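; Butterfly guide actor that appears near the camera and travels along a spline while the player stays close.
; ActivateButterfly, or a test F key, reveals it, flies it to the spline start, then enables two trigger spheres.
; Entering StartSphere plays or resumes the length-scaled travel timeline; leaving StopSphere halts it.
; The fly-in speed calculation sets the travel timeline's rate, leaving the fly-in timeline's rate untouched.
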(event OnComponentBeginOverlap(StartSphere)
  (params (OverlappedComponent :type Primitive%20Component%20Object%20Reference) (OtherActor :type Actor%20Object%20Reference) (OtherComp :type Primitive%20Component%20Object%20Reference) (OtherBodyIndex :type Integer) (bFromSweep :type Boolean) (SweepResult :type Hit%20Result%20Structure%20%28by%20ref%29))
  (bind _butterflypath (Variables|Default|GetButterflyPath))
  ;[1 1 1] Check for ovelap
  (if (== OtherActor (Game|GetPlayerCharacter 0))
    ;[1 1 1] Travel along spline
    (Components|Timeline|SetPlayRate (Variables|Default|GetButterflyTravel) (* (/ 1.0 (Spline|GetSplineLength (Variables|Default|GetButterflyPath))) (Variables|Default|GetSpeed)))
    (bind _newtrack_0 (Timeline|ButterflyTravel Play)
      (:Update
        (Variables|Default|SetAlpha _newtrack_0)
        (Transformation|SetWorldLocationAndRotation (Variables|Default|GetButterfly) (Spline|GetLocationatDistanceAlongSpline _butterflypath (Math|Float|Lerp 0.0 (Spline|GetSplineLength _butterflypath) (Variables|Default|GetAlpha)) "World") (Spline|GetRotationatDistanceAlongSpline _butterflypath (Math|Float|Lerp 0.0 (Spline|GetSplineLength _butterflypath) (Variables|Default|GetAlpha)) "World") false false))
      (:Finished
        (CallFunction|CollisionOff)))))

(event OnComponentEndOverlap(StopSphere)
  (params (OverlappedComponent :type Primitive%20Component%20Object%20Reference) (OtherActor :type Actor%20Object%20Reference) (OtherComp :type Primitive%20Component%20Object%20Reference) (OtherBodyIndex :type Integer))
  ;[1 1 1] Stop movement when out of detection
  (if (== OtherActor (Game|GetPlayerCharacter 0))
    (Audio|Components|Audio|Stop (Variables|Default|GetButterflyTravel))))

(event Custom|ActivateButterfly
  (bind _returnvalue (Game|GetPlayerCameraManager 0))
  (bind _butterflypath (Variables|Default|GetButterflyPath))
  (bind _butterflypath_2 (Variables|Default|GetButterflyPath))
  (bind _returnvalue_2 (Spline|GetLocationatDistanceAlongSpline _butterflypath_2 0.0 "World"))
  (bind _returnvalue_3 (Camera|GetCameraLocation _returnvalue))
  ;[1 1 1] Moves the butterfly near the camera and makes its visible
  (bind _output_get (Variables|Default|SetSpawnRotation (Math|Rotator|FindLookatRotation _returnvalue_3 _returnvalue_2)))
  (bind _output_get_2 (Variables|Default|SetSpawnPos (+ _returnvalue_3 (Variables|Default|GetSpawnOffset))))
  (Transformation|SetWorldLocationAndRotation (Variables|Default|GetButterfly) _output_get_2 _output_get false false)
  (Development|SetHiddeninGame (Variables|Default|GetButterfly) false false)
  ;[1 1 1] Travel towards start of spline
  (Components|Timeline|SetPlayRate (Variables|Default|GetButterflyTravel) (* (/ 1.0 (Math|Vector|Distance(Vector) (Variables|Default|GetSpawnPos) _returnvalue_2)) (Variables|Default|GetSpeed)))
  (bind _newtrack_0 (Timeline|FlyInTimeline Play)
    (:Update
      (Transformation|SetWorldLocationAndRotation (Variables|Default|GetButterfly) (Math|Vector|Lerp(Vector) (Variables|Default|GetSpawnPos) (Spline|GetLocationatDistanceAlongSpline _butterflypath 0.0 "World") _newtrack_0) (Math|Rotator|Lerp(Rotator) (Variables|Default|GetSpawnRotation) (Spline|GetRotationatDistanceAlongSpline _butterflypath 0.0 "World") _newtrack_0 true) false false))
    (:Finished
      (CallFunction|Collisionon))))

(event Custom|CollisionOn
  ;[1 1 1] Turning on the collision spheres
  (Collision|SetCollisionEnabled (Variables|Default|GetStartSphere) "QueryOnly")
  (Collision|SetCollisionEnabled (Variables|Default|GetStopSphere) "QueryOnly"))

(event Custom|CollisionOff
  ;[1 1 1] Turning Off the collision spheres
  (Collision|SetCollisionEnabled (Variables|Default|GetStartSphere) "NoCollision")
  (Collision|SetCollisionEnabled (Variables|Default|GetStopSphere) "NoCollision"))

(event EventBeginPlay
  (Actor|Tick|SetActorTickEnabled false)
  (Development|SetHiddeninGame (Variables|Default|GetButterfly) true false)
  (CallFunction|CollisionOff)
  ;[1 0 0.09455] FOR TESTING, REMOVE LATER
  (Input|EnableInput (Game|GetPlayerController 0)))

(event Collision|EventActorBeginOverlap
  (params (OtherActor :type Actor%20Object%20Reference)))

(event Input|KeyboardEvents|F
  (params (Key :type Key%20Structure :default "None"))
  (bind _returnvalue (Game|GetPlayerCameraManager 0))
  (bind _butterflypath (Variables|Default|GetButterflyPath))
  (bind _butterflypath_2 (Variables|Default|GetButterflyPath))
  (bind _returnvalue_2 (Spline|GetLocationatDistanceAlongSpline _butterflypath_2 0.0 "World"))
  (bind _returnvalue_3 (Camera|GetCameraLocation _returnvalue))
  ;[1 0 0.09455] FOR TESTING, REMOVE LATER
  (:Pressed
    ;[1 1 1] Moves the butterfly near the camera and makes its visible
    (bind _output_get (Variables|Default|SetSpawnRotation (Math|Rotator|FindLookatRotation _returnvalue_3 _returnvalue_2)))
    (bind _output_get_2 (Variables|Default|SetSpawnPos (+ _returnvalue_3 (Variables|Default|GetSpawnOffset))))
    (Transformation|SetWorldLocationAndRotation (Variables|Default|GetButterfly) _output_get_2 _output_get false false)
    (Development|SetHiddeninGame (Variables|Default|GetButterfly) false false)
    ;[1 1 1] Travel towards start of spline
    (Components|Timeline|SetPlayRate (Variables|Default|GetButterflyTravel) (* (/ 1.0 (Math|Vector|Distance(Vector) (Variables|Default|GetSpawnPos) _returnvalue_2)) (Variables|Default|GetSpeed)))
    (bind _newtrack_0 (Timeline|FlyInTimeline Play)
      (:Update
        (Transformation|SetWorldLocationAndRotation (Variables|Default|GetButterfly) (Math|Vector|Lerp(Vector) (Variables|Default|GetSpawnPos) (Spline|GetLocationatDistanceAlongSpline _butterflypath 0.0 "World") _newtrack_0) (Math|Rotator|Lerp(Rotator) (Variables|Default|GetSpawnRotation) (Spline|GetRotationatDistanceAlongSpline _butterflypath 0.0 "World") _newtrack_0 true) false false))
      (:Finished
        (CallFunction|Collisionon)))))

(fn ConstructionScript
  (Components|Sphere|SetSphereRadius (Variables|Default|GetStartSphere) (Variables|Default|GetStartRadius) true)
  (Components|Sphere|SetSphereRadius (Variables|Default|GetStopSphere) (Variables|Default|GetStopRadius) true))