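; Legacy player controller that drives the camera each Tick by adjusting control rotation from Turn and LookUp input.
; Two angled line traces from the pawn nudge yaw momentum away from world obstacles, while proximity between pawn and camera manager adds a pitch pushback.
; Input decelerates through easing, then feeds eased yaw and pitch, with Y negated.
; Vertical avoidance and trace-debug branches are disconnected leftovers.
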(event EventBeginPlay)

(event EventTick
  (params (DeltaSeconds :type Float%20%28single-precision%29))
  (bind _returnvalue (Pawn|GetControlRotation :!class /Script/Engine.Controller))
  (bind _returnvalue_2 (Pawn|GetControlledPawn))
  (bind _returnvalue_3 (Pawn|GetControlRotation :!class /Script/Engine.Controller))
  (bind _returnvalue_4 (Input|AxisValues|GetTurn))
  (bind _returnvalue_5 (Input|AxisValues|GetLookUp))
  (bind _playercameramanager (Variables|Default|GetPlayerCameraManager))
  (bind _avoidanceeasevalue (Variables|Default|GetAvoidanceEaseValue))
  (bind _playercameramanager_2 (Variables|Default|GetPlayerCameraManager))
  (bind _returnvalue_6 (Transformation|GetActorLocation _playercameramanager_2))
  (bind _returnvalue_7 (Transformation|GetActorLocation _returnvalue_2))
  (bind _yaw (Math|Rotator|BreakRotator _returnvalue_3))
  (bind _returnvalue_8 (Camera|GetCameraLocation _playercameramanager))
  (bind (_roll _pitch _yaw_2) (Math|Rotator|BreakRotator _returnvalue))
  (bind _returnvalue_9 (Math|Vector|Distance(Vector) _returnvalue_7 _returnvalue_6))
  (bind _returnvalue_10 (Math|Rotator|MakeRotator 0.0 0.0 _yaw))
  (bind _z (Math|Vector|BreakVector _returnvalue_8))
  (bind _z_2 (Math|Vector|BreakVector _returnvalue_7))
  (bind _returnvalue_11 (+ _returnvalue_7 "0.000000,0,-20.000000"))
  (bind _returnvalue_12 (- _z _z_2))
  (bind _returnvalue_13 (Math|Vector|MakeVector 0.0 0.0 _returnvalue_12))
  (bind _returnvalue_14 (+ _returnvalue_7 _returnvalue_13 "0.000000,0,-20.000000"))
  (Variables|Default|SetDeltaSeconds DeltaSeconds)
  ;[0.9167 0.8333 1] Obstacle Aboidance
  (bind _returnvalue_15 (Collision|LineTraceForObjects _returnvalue_11 (+ (* (Math|Vector|GetForwardVector (Math|Rotator|CombineRotators _returnvalue_10 "0,160.000000, 0")) (Variables|Default|GetAvoidace%20Range)) _returnvalue_14) (Utilities|Array|MakeArray "ObjectTypeQuery1" "ObjectTypeQuery2") false 0 "None"))
  (if _returnvalue_15
    (bind _output_get (Variables|Default|SetXDeceleration (Class|KismetMathLibrary|FInterpEaseinOut (stale _output_get) (+ (stale _output_get) (Variables|Default|GetAvoidanceRate)) (Variables|Default|GetDeltaSeconds) _avoidanceeasevalue))))
  (bind _returnvalue_16 (Collision|LineTraceForObjects _returnvalue_11 (+ (* (Math|Vector|GetForwardVector (Math|Rotator|CombineRotators _returnvalue_10 "0,-160.000000, 0")) (Variables|Default|GetAvoidace%20Range)) _returnvalue_14) (Utilities|Array|MakeArray "ObjectTypeQuery1" "ObjectTypeQuery2") false 0 "None"))
  (if _returnvalue_16
    (bind _output_get_2 (Variables|Default|SetXDeceleration (Class|KismetMathLibrary|FInterpEaseinOut (stale _output_get_2) (+ (stale _output_get_2) (* (Variables|Default|GetAvoidanceRate) -1.0)) (Variables|Default|GetDeltaSeconds) _avoidanceeasevalue))))
  ;[1 1 1] Pushback
  (if (<= _returnvalue_9 (Variables|Default|GetPushbackRadius))
    (Variables|Default|SetPushback (* (Variables|Default|GetPushbackStrength) (- 1.0 (/ _returnvalue_9 (Variables|Default|GetPushbackRadius))) 2.0))
    (else
      (Variables|Default|SetPushback 0.0)))
  ;[1 1 1] Deceleration X
  (if (> (Math|Float|Absolute(Float) (Variables|Default|GetXDeceleration)) (Math|Float|Absolute(Float) _returnvalue_4))
    (Variables|Default|SetXDeceleration (Math|Interpolation|Ease "EaseOut" (Variables|Default|GetDeltaSeconds) (Variables|Default|GetXDeceleration) _returnvalue_4 (Variables|Default|GetX%20Deceleration%20Strength)))
    (else
      (Variables|Default|SetXDeceleration _returnvalue_4)))
  ;[1 1 1] Deceleration Y
  (if (> (Math|Float|Absolute(Float) (Variables|Default|GetYDeceleration)) (Math|Float|Absolute(Float) _returnvalue_5))
    (Variables|Default|SetYDeceleration (Math|Interpolation|Ease "EaseOut" (Variables|Default|GetDeltaSeconds) (Variables|Default|GetYDeceleration) _returnvalue_5 (Variables|Default|GetY%20Deceleration%20Strength)))
    (else
      (Variables|Default|SetYDeceleration _returnvalue_5)))
  (Pawn|SetControlRotation (Math|Rotator|MakeRotator _roll (Math|Interpolation|Ease "EaseInOut" (Variables|Default|GetDeltaSeconds) (+ _pitch (+ (Variables|Default|GetPushback) (* (Variables|Default|GetYDeceleration) -1.0))) (- _pitch (+ (Variables|Default|GetPushback) (* (Variables|Default|GetYDeceleration) -1.0))) (Variables|Default|GetY%20Ease%20amount)) (Math|Interpolation|Ease "EaseInOut" (Variables|Default|GetDeltaSeconds) (+ _yaw_2 (Variables|Default|GetXDeceleration)) (- _yaw_2 (Variables|Default|GetXDeceleration)) (Variables|Default|GetX%20Ease%20Amount)))))

(fn ConstructionScript)